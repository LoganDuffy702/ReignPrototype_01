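; BP_Storyteller displays an array of text lines on screen with a typewriter effect.
; It creates a hidden UMG_Storyteller widget at BeginPlay, and StartStoryteller reveals it and starts the sequence.
; RunStoryTeller steps through lines with delays, while DisplayText re-triggers itself by timer to append one character at a time.
; FinishCurrentLineNow completes the current line, and the AllTextDone dispatcher fires after the last line clears.
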(event Custom|StartStoryteller
  (params (TextToDisplay :type Array%20of%20Texts))
  ;[1 1 1] Call when you want to start the Story Teller
  (Widget|SetVisibility (Variables|Default|GetUMG%20Storyteller%20Widget) "Visible")
  (Variables|Default|SetTextToDisplay TextToDisplay)
  (CallFunction|RunStoryTeller))

(event Custom|RunStoryTeller
  (bind _texttodisplay (Variables|Default|GetTextToDisplay))
  (bind _returnvalue (Utilities|Array|Length _texttodisplay))
  ;[1 1 1] Called to set up and handle displaying the next line of text
  (bind _result (Math|Integer|IncrementInt (Variables|Default|GetArrayIterator))
    (:%20%20
      (Variables|Default|SetArrayIterator _result) ; Increment our current iteractor for the string to display
      (Development|PrintString (Utilities|String|ToString(Integer) _returnvalue))
      (if (>= (Variables|Default|GetArrayIterator) _returnvalue) ; Are we done Displaying all of our text?
        (Utilities|FlowControl|Delay (Variables|Setup|GetDelayBetweenLines)) ; Delay the next line of text
        (Rendering|Components|TextRender|SetText (Variables|Default|GetStorytellerTextBlock) "") ; Clear our Text Block
        (Variables|Default|SetArrayIterator -1)
        (Default|CallAllTextDone) ; Call our Dispatcher now that we are done
        (else
          (Development|PrintString "Hello")
          (if (> (Variables|Default|GetArrayIterator) 0) ; Do we need to delay this line?
            (Utilities|FlowControl|Delay (Variables|Setup|GetDelayBetweenLines)) ; Delay our line
          )
          (Rendering|Components|TextRender|SetText (Variables|Default|GetStorytellerTextBlock) "") ; Clear our Text Block
          (Variables|Default|SetFinishTextNow false) ; Reset our Finish Text now Boolean
          (Variables|Default|SetCurrentStringToDisplay (Utilities|String|ToString(Text) (Utilities|Array|Get(acopy) (Variables|Default|GetTextToDisplay) (Variables|Default|GetArrayIterator)))) ; Set our Current String we want to show
          (CallFunction|DisplayText) ; Display the string on the screen
        )))))

(event Custom|FinishCurrentLineNow
  ;[1 1 1] Call when you want the current line to finish immediately
  (Variables|Default|SetFinishTextNow true))

(event EventBeginPlay
  ;[1 1 1] Create our widget and add it to the screen, get a reference to the text block
  (bind _returnvalue (UserInterface|CreateWidget "/Game/Dialogue/UC/-StorytellerObject/Storyteller/UMG_Storyteller.UMG_Storyteller_C"))
  (Variables|Default|SetUMG%20Storyteller%20Widget _returnvalue)
  (UserInterface|Viewport|AddtoViewport _returnvalue 0)
  (Variables|Default|SetStorytellerTextBlock (Variables|/Game/Dialogue/UC/-StorytellerObject/Storyteller/UMG_Storyteller.UMG_Storyteller_C|GetThisTextBlock _returnvalue))
  (Widget|SetVisibility _returnvalue "Hidden"))

(fn ConstructionScript)

(fn DisplayText
  (bind _storytellertextblock (Variables|Default|GetStorytellerTextBlock))
  (bind _returnvalue (Class|TextBlock|GetText _storytellertextblock))
  (bind _returnvalue_2 (Utilities|String|ToString(Text) _returnvalue))
  (Rendering|Components|TextRender|SetText (Variables|Default|GetStorytellerTextBlock) (Utilities|Text|ToText(String) (Utilities|String|Append _returnvalue_2 (Utilities|String|GetSubstring (Variables|Default|GetCurrentStringToDisplay) (Utilities|String|Len _returnvalue_2))))) ; Set our Text Block to the current position of our text
  (if (Variables|Default|GetFinishTextNow) ; Do we want to finish immediately?
    (Rendering|Components|TextRender|SetText (Variables|Default|GetStorytellerTextBlock) (Utilities|Text|ToText(String) (Variables|Default|GetCurrentStringToDisplay))) ; Set our Text Block to the entire string
    (CallFunction|RunStoryTeller) ; Run our Story Teller to advance the Story
    (elif (Utilities|Enum|Equal(Enum) (Class|TextBlock|GetText (Variables|Default|GetStorytellerTextBlock)) (Utilities|Text|ToText(String) (Variables|Default|GetCurrentStringToDisplay))) ; Is our string finished?
      (CallFunction|RunStoryTeller) ; Run our Story Teller to advance the Story
      (else
        (Utilities|Time|SetTimerbyFunctionName 0 "DisplayText" (Variables|Setup|GetDelayBetweenLetters)) ; Call ourselves after the delay to show the next character
      ))))