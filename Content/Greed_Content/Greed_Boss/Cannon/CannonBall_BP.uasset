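; CannonBall_BP is the cannonball actor for the Greed boss's cannon, built from a collision sphere, static mesh and particle system.
; On any sphere overlap, it spawns a large explosion, deactivates its particles, hides the mesh, disables collision and destroys itself after a short delay.
; A blocking hit only spawns a leap effect at the impact point.
; The graph applies no damage and sets no movement.
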(event OnComponentBeginOverlap(Sphere)
  (params (OverlappedComponent :type Primitive%20Component%20Object%20Reference) (OtherActor :type Actor%20Object%20Reference) (OtherComp :type Primitive%20Component%20Object%20Reference) (OtherBodyIndex :type Integer) (bFromSweep :type Boolean) (SweepResult :type Hit%20Result%20Structure%20%28by%20ref%29))
  (Effects|SpawnEmitteratLocation "/Game/StarterContent/Particles/P_Explosion.P_Explosion" (Transformation|GetWorldLocation (Variables|Default|GetSphere)) "0, 0, 0" "10.000000,10.000000,10.000000")
  (Components|Activation|Deactivate (Variables|Default|GetParticleSystem))
  (Rendering|SetVisibility (Variables|Default|GetStaticMesh) false false)
  (Collision|SetCollisionEnabled (Variables|Default|GetSphere) "NoCollision")
  (Utilities|FlowControl|Delay 2.0)
  (Actor|DestroyActor))

(event OnComponentHit(Sphere)
  (params (HitComponent :type Primitive%20Component%20Object%20Reference) (OtherActor :type Actor%20Object%20Reference) (OtherComp :type Primitive%20Component%20Object%20Reference) (NormalImpulse :type Vector :default "0, 0, 0") (Hit :type Hit%20Result%20Structure%20%28by%20ref%29))
  (Effects|SpawnEmitteratLocation "/Game/Reign_Assets/EnemyObjects/Jump_Enemy/Jump_FX/JumpStart_Enemy_LeapFX1.JumpStart_Enemy_LeapFX1" (.impactpoint Hit) "0, 0, 0" "5.000000,5.000000,5.000000"))

(event EventBeginPlay)

(event Collision|EventActorBeginOverlap
  (params (OtherActor :type Actor%20Object%20Reference)))

(event EventTick
  (params (DeltaSeconds :type Float%20%28single-precision%29)))

(fn ConstructionScript)