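; Greed boss cannon that the player's attacks either fire or turn, gated by a CanFire flag.
; Melee, Special and AIR hits play the fire montage; Grapple and Pull rotate it a step and re-enable CanFire after a delay.
; A separate FireCannonEvent spawns a cannonball at FireSphere.
; PullPlayerEvent, whose call here is unwired, uses a timeline to drag the player toward the cannon while updating the chain beam.
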(event Custom|PullPlayerEvent
  (bind _capsulecomponent (Variables|Default|GetCapsuleComponent))
  (bind _returnvalue (Transformation|GetWorldLocation _capsulecomponent))
  (Variables|Default|SetPlayerLastLoc (Transformation|GetActorLocation (Variables|Default|GetPlayerRef)))
  (bind _newtrack_0 (Timeline|Timeline_0 PlayFromStart)
    (:Update
      (Class|ParticleSystemComponent|SetBeamEndPoint (Variables|/Game/Reign_Assets/Weapon_BP/Master_Weapon_BP.Master_Weapon_BP_C|GetChainParticle (Variables|/Game/Reign_Assets/Player_Character/Blueprints/MC_Prototype_BP.MC_Prototype_BP_C|GetEquippedWeapon (Variables|Default|GetPlayerRef))) 0 (Transformation|GetWorldLocation (Variables|Default|GetChokePoint)))
      (Transformation|SetActorLocation (Variables|Default|GetPlayerRef) (Math|Vector|Lerp(Vector) (Math|Vector|MakeVector (.X (Math|Vector|BreakVector (Variables|Default|GetPlayerLastLoc))) (.Y (Math|Vector|BreakVector (Variables|Default|GetPlayerLastLoc))) (.Z (Math|Vector|BreakVector (Variables|Default|GetPlayerLastLoc)))) (+ (* (Math|Vector|MakeVector (.x _returnvalue) (.y _returnvalue) (+ (.z _returnvalue) 1.5e+02)) (/ 3.0 4.0)) (* (Math|Vector|MakeVector (.X (Math|Vector|BreakVector (Variables|Default|GetPlayerLastLoc))) (.Y (Math|Vector|BreakVector (Variables|Default|GetPlayerLastLoc))) (.Z (Math|Vector|BreakVector (Variables|Default|GetPlayerLastLoc)))) (/ 1.0 4.0))) _newtrack_0) false false))))

(event Custom|FireCannonEvent
  (bind _firesphere (Variables|Default|GetFireSphere))
  (Game|SpawnActorfromClass "/Game/Greed_Content/Greed_Boss/Cannon/CannonBall_BP.CannonBall_BP_C" (Math|Transform|MakeTransform (Transformation|GetWorldLocation _firesphere) (Transformation|GetWorldRotation _firesphere) "0.700000,0.700000,0.700000") "Undefined" 0 0))

(event EventBeginPlay
  (|CallParentFunction) ; This node is disabled and will not be called.\nDrag off pins to build functionality.
)

(event Collision|EventActorBeginOverlap
  (params (OtherActor :type Actor%20Object%20Reference)))

(event EventTick
  (params (DeltaSeconds :type Float%20%28single-precision%29))
  (|CallParentFunction DeltaSeconds) ; This node is disabled and will not be called.\nDrag off pins to build functionality.
)

(event EventDealingDamage
  (params (Sent%20Damage :type Integer) (Sender :type Actor%20Object%20Reference) (DamageType :type Name :default "None"))
  (if (Variables|Default|GetCanFire)
    (Variables|Default|SetCanFire false)
    (switch name DamageType
      (:Melee
        (Animation|PlayAnimMontage "/Game/Greed_Content/Greed_Boss/Cannon/CannonAnimations/FireAnim_Anim_Montage.FireAnim_Anim_Montage" 1.0 "None" :!label _label))
      (:Special
        (goto _label))
      (:AIR
        (goto _label))
      (:Grapple
        (Class|Actor|AddActorWorldRotation "0,45.000000, 0" :!label _label_2)
        (Utilities|FlowControl|Delay 1.0)
        (Variables|Default|SetCanFire true))
      (:PullTo
        (goto _label_2)))))

(fn ConstructionScript
  (|CallParentFunction))