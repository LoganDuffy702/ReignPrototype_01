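; Legs body part of the Greed boss: a character that trails its parent body part and knocks the player away on contact.
; Each tick it aims at the parent's capsule and adds movement input whenever farther than a fixed distance from it.
; Capsule overlap launches the player up and opposite their own facing, scaled by PlayerKnockBack.
; A reset event moves the capsule to a fixed world point; DamagePlayer and LaunchMask are empty stubs.
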(event OnComponentBeginOverlap(CapsuleComponent)
  (params (OverlappedComponent :type Primitive%20Component%20Object%20Reference) (OtherActor :type Actor%20Object%20Reference) (OtherComp :type Primitive%20Component%20Object%20Reference) (OtherBodyIndex :type Integer) (bFromSweep :type Boolean) (SweepResult :type Hit%20Result%20Structure%20%28by%20ref%29))
  (bind _playerknockback (Variables|Default|GetPlayerKnockBack))
  (Development|PrintString "PlayerHit")
  (bind _asmc_prototype_bp (Utilities|Casting|CastToMC_Prototype_BP OtherActor))
  (Character|LaunchCharacter _asmc_prototype_bp (+ (* (Math|Vector|GetForwardVector (Variables|/Script/Engine.Character|GetCapsuleComponent _asmc_prototype_bp)) (* _playerknockback -0.5)) (Math|Vector|MakeVector 0.0 0.0 _playerknockback)) false true))

(event Custom|GoToResetPoint
  (Transformation|SetWorldLocation (Variables|Collision|GetCapsuleComponent) "0, 0,1000.000000" false false))

(event Custom|CheckForMovement
  (if (not (<= (Math|Vector|VectorLength (- (Transformation|GetActorLocation) (Transformation|GetWorldLocation (Variables|/Script/Engine.Character|GetCapsuleComponent (Variables|Default|GetParentBodyPart))))) 7e+02))
    (Pawn|Input|AddMovementInput (Variables|Default|GetForwardVector) 1.0 false)))

(event EventBeginPlay
  (bind _asmc_prototype_bp (Utilities|Casting|CastToMC_Prototype_BP (Game|GetPlayerCharacter 0)))
  (Variables|Default|SetPlayer%20Ref _asmc_prototype_bp))

(event EventTick
  (params (DeltaSeconds :type Float%20%28single-precision%29))
  (Variables|Default|SetForwardVector (Math|Vector|GetForwardVector (Math|Rotator|FindLookatRotation (Transformation|GetActorLocation) (Transformation|GetWorldLocation (Variables|/Script/Engine.Character|GetCapsuleComponent (Variables|Default|GetParentBodyPart))))))
  (CallFunction|CheckforMovement))

(fn ConstructionScript)

(fn LaunchMask)

(fn DamagePlayer)