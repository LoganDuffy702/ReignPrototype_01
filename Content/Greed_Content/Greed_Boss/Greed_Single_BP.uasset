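; Greed_Single_BP is a body segment of the Greed boss that trails its parent body part.
; Each tick it computes the direction to the parent's capsule and adds movement input toward it whenever it is more than a set distance away, giving a follow-the-leader chain.
; A reset event moves the capsule to a fixed point and shows the placeholder body.
; It caches the player character on BeginPlay; rotation and force-based movement nodes are left disconnected.
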(event Custom|GoToResetPoint
  (Transformation|SetWorldLocation (Variables|Collision|GetCapsuleComponent) "0, 0,1000.000000" false false)
  (Rendering|SetVisibility (Variables|Default|GetBodyPlaceholder) true false))

(event Custom|CheckForMovement
  (if (not (<= (Math|Vector|VectorLength (- (Transformation|GetActorLocation) (Transformation|GetWorldLocation (Variables|/Script/Engine.Character|GetCapsuleComponent (Variables|Default|GetParentBodyPart))))) 7e+02))
    (Pawn|Input|AddMovementInput (Variables|Default|GetForwardVector) 1.0 false)))

(event EventBeginPlay
  (bind _asmc_prototype_bp (Utilities|Casting|CastToMC_Prototype_BP (Game|GetPlayerCharacter 0)))
  (Variables|Default|SetPlayer%20Ref _asmc_prototype_bp))

(event EventTick
  (params (DeltaSeconds :type Float%20%28single-precision%29))
  (Variables|Default|SetForwardVector (Math|Vector|GetForwardVector (Math|Rotator|FindLookatRotation (Transformation|GetActorLocation) (Transformation|GetWorldLocation (Variables|/Script/Engine.Character|GetCapsuleComponent (Variables|Default|GetParentBodyPart))))))
  (CallFunction|CheckforMovement))

(fn ConstructionScript)