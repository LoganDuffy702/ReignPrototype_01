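; Booth_Destroy_BP is a destructible booth environment prop that breaks apart when it takes damage.
; A damage event passes the damage type and skeletal mesh to LogansDestroyDecorComponent's DestroySolver and spawns a decor damage effect at the capsule.
; If the mesh is then playing an animation, the capsule loses collision and the actor destroys itself five seconds later.
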(event EventDealingDamage
  (params (Sent%20Damage :type Integer) (Sender :type Actor%20Object%20Reference) (DamageType :type Name :default "None"))
  (bind _capsule (Variables|Default|GetCapsule))
  (Default|DestroySolver (Variables|Default|GetLogans_DestroyDecor_Component) DamageType (Variables|Default|GetSkeletalMesh))
  (Effects|SpawnEmitteratLocation "/Game/Greed_Content/Greed_env_assets/DecorDMG_FX.DecorDMG_FX" (Transformation|GetWorldLocation (Variables|Default|GetCapsule)))
  (if (Audio|Components|Audio|IsPlaying (Variables|Default|GetSkeletalMesh))
    (Collision|SetCollisionObjectType _capsule "ECC_WorldStatic")
    (Collision|SetCollisionEnabled _capsule "NoCollision")
    (Utilities|FlowControl|Delay 5.0)
    (Actor|DestroyActor)))

(fn ConstructionScript)