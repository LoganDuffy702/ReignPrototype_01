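; Destructible urn for the Limbo boss fight that damages the boss when broken and relocates each time it is repaired.
; On battle start or repair it shuffles its platforms and teleports above the first with a random yaw, with repair also raising all platforms.
; A DoOnce gates hits, while one timeline scrubs the break animation and material dissolve, reversing on repair to restore effects and re-arm damage.
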(event Custom|RepairUrn
  (bind _skeletalmesh1 (Variables|Default|GetSkeletalMesh1))
  (for _array_element (Variables|Default|GetPlatforms)
    (Default|RiseUp _array_element))
  (Utilities|FlowControl|Delay 1.0)
  (CallFunction|FindNewPlatform)
  (Variables|Default|SetBroken? false)
  (Rendering|SetVisibility (Variables|Default|GetSkeletalMesh1) true false)
  (bind (_direction _animationtrack _dissolvetrack) (Timeline|Timeline_0 ReverseFromEnd)
    (:Update
      (Components|Animation|SetPosition _skeletalmesh1 _animationtrack true)
      (Rendering|Material|SetScalarParameterValueonMaterials _skeletalmesh1 "Falloff" _dissolvetrack))
    (:Finished
      (if (Variables|Default|GetBroken?)
        (Rendering|SetVisibility (Variables|Default|GetSkeletalMesh1) false false)
        (else
          (Rendering|SetVisibility (Variables|Default|GetParticleSystem) true false)
          (CallFunction|EnableCollision))))))

(event Custom|FindNewPlatform
  (bind _platforms (Variables|Default|GetPlatforms))
  (Utilities|Array|Shuffle _platforms)
  (Transformation|SetActorLocation (+ (Transformation|GetWorldLocation (Variables|/Game/Limbo_Content/Limbo_Boss/BPs/LB_Urn/Urn_Location_Actor_BP.Urn_Location_Actor_BP_C|GetPlacementPoint (Utilities|Array|Get(acopy) _platforms))) "0, 0,200.000000") false false)
  (Transformation|SetActorRotation (Math|Rotator|MakeRotator 0.0 0.0 (Math|Random|RandomFloatinRange -3.6e+02 3.6e+02))))

(event Custom|StartBattle
  (CallFunction|FindNewPlatform))

(event Custom|EnableCollision
  (bind _skeletalmesh1 (Variables|Default|GetSkeletalMesh1))
  (Utilities|FlowControl|DoOnce false) ; enters at Reset
)

(event EventDealingDamage
  (params (Sent%20Damage :type Integer) (Sender :type Actor%20Object%20Reference) (DamageType :type Name :default "None"))
  (bind _skeletalmesh1 (Variables|Default|GetSkeletalMesh1))
  (Utilities|FlowControl|DoOnce false
    (:Completed
      (CallFunction|PlayImpactSound)
      (Variables|Default|SetBroken? true)
      (Rendering|SetVisibility (Variables|Default|GetParticleSystem) false false)
      (Utilities|IsValid (Variables|Default|GetLimboBossRef)
        (:Is%20Valid
          (Default|DealingDamage (Variables|Default|GetLimboBossRef) 100 self "URN")
          (bind (_direction _animationtrack _dissolvetrack) (Timeline|Timeline_0 PlayFromStart)
            (:Update
              (Components|Animation|SetPosition _skeletalmesh1 _animationtrack true)
              (Rendering|Material|SetScalarParameterValueonMaterials _skeletalmesh1 "Falloff" _dissolvetrack))
            (:Finished
              (if (Variables|Default|GetBroken?)
                (Rendering|SetVisibility (Variables|Default|GetSkeletalMesh1) false false)
                (else
                  (Rendering|SetVisibility (Variables|Default|GetParticleSystem) true false)
                  (CallFunction|EnableCollision))))))
        (:Is%20Not%20Valid
          (Timeline|Timeline_0 PlayFromStart))))))

(fn ConstructionScript)