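; Limbo boss character that constantly moves toward the player and picks attacks by distance.
; A fast looping timer re-aims the forward vector at the player, and Tick feeds it into movement input.
; A slower looping timer runs PlayerDistance, which triggers a random close, mid or long-range montage unless IsAttacking is set, clearing that flag after the montage's duration.
; The AI MoveTo and random-direction movement events are not called here.
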(event Custom|GoToPlayer
  ;[1 1 1] Find Player
  (AI|AIMoveTo self "0, 0, 0" (Game|GetPlayerCharacter 0) 2e+02 false
    (:then
      _)
    (:OnSuccess
      _)
    (:OnFail
      _))
  (Utilities|FlowControl|Delay 1.0)
  (CallFunction|FindPlayer))

(event Custom|FindPlayer
  ;[1 1 1] Run to Player
  (Variables|Default|SetForwardVector (Math|Vector|GetForwardVector (Math|Rotator|FindLookatRotation (Transformation|GetActorLocation) (Transformation|GetActorLocation (Game|GetPlayerCharacter 0)))))
  (Utilities|Time|SetTimerbyEvent (delegate Custom|FindPlayer) 0.01 true))

(event Custom|Follow%20Player
  ;[1 1 1] Soon to be run in random directions
  (Variables|Default|SetForwardVector (Math|Vector|GetForwardVector (Math|Rotator|FindLookatRotation (Transformation|GetActorLocation) (+ "0, 0, 0" (Math|Vector|MakeVector (Math|Random|RandomFloatinRange -4.5e+03 4.5e+03) (Math|Random|RandomFloatinRange -4.5e+03 4.5e+03) (.z (Transformation|GetActorLocation)))))))
  (Utilities|Time|SetTimerbyEvent (delegate Custom|Follow%20Player) 1.0 true))

(event Custom|DistanceToPlayer
  ;[1 1 1] Distance to player
  (Utilities|Time|SetTimerbyFunctionName 0 "PlayerDistance" 1.0 true))

(event Custom|Long%20Range
  (Variables|Default|SetisAttacking true)
  (switch int (Math|Random|RandomIntegerinRange 0 1)
    (:0
      (Variables|Default|SetAttackMontage "/Game/Limbo_Content/Limbo_Boss/Mesh/Animations/Montage/Long_01.Long_01"))
    (:1
      (Variables|Default|SetAttackMontage "/Game/Limbo_Content/Limbo_Boss/Mesh/Animations/Montage/Long_02.Long_02")))
  (bind _returnvalue (Animation|PlayAnimMontage (Variables|Default|GetAttackMontage) 1.0 "None"))
  (Utilities|FlowControl|Delay _returnvalue)
  (Variables|Default|SetisAttacking false))

(event Custom|Close%20Range
  (Variables|Default|SetisAttacking true)
  (switch int (Math|Random|RandomIntegerinRange 0 3)
    (:0
      (Variables|Default|SetAttackMontage "/Game/Limbo_Content/Limbo_Boss/Mesh/Animations/Montage/Close_01.Close_01"))
    (:1
      (Variables|Default|SetAttackMontage "/Game/Limbo_Content/Limbo_Boss/Mesh/Animations/Montage/Close_02.Close_02"))
    (:2
      (Variables|Default|SetAttackMontage "/Game/Limbo_Content/Limbo_Boss/Mesh/Animations/Montage/Close_03.Close_03"))
    (:3
      (Variables|Default|SetAttackMontage "/Game/Limbo_Content/Limbo_Boss/Mesh/Animations/Montage/Close_04.Close_04")))
  (bind _returnvalue (Animation|PlayAnimMontage (Variables|Default|GetAttackMontage) 1.0 "None"))
  (Utilities|FlowControl|Delay _returnvalue)
  (Variables|Default|SetisAttacking false))

(event Custom|Mid%20Range
  (Variables|Default|SetisAttacking true)
  (switch int (Math|Random|RandomIntegerinRange 0 3)
    (:0
      (Variables|Default|SetAttackMontage "/Game/Limbo_Content/Limbo_Boss/Mesh/Animations/Montage/Mid_01.Mid_01"))
    (:1
      (Variables|Default|SetAttackMontage "/Game/Limbo_Content/Limbo_Boss/Mesh/Animations/Montage/Mid_02.Mid_02"))
    (:2
      (Variables|Default|SetAttackMontage "/Game/Limbo_Content/Limbo_Boss/Mesh/Animations/Montage/Mid_03.Mid_03"))
    (:3
      (Variables|Default|SetAttackMontage "/Game/Limbo_Content/Limbo_Boss/Mesh/Animations/Montage/Mid_04.Mid_04")))
  (bind _returnvalue (Animation|PlayAnimMontage (Variables|Default|GetAttackMontage) 1.0 "None"))
  (Utilities|FlowControl|Delay _returnvalue)
  (Variables|Default|SetisAttacking false))

(event EventTick
  (params (DeltaSeconds :type Float%20%28single-precision%29))
  ;[1 1 1] Forward Vector tick and input
  (Pawn|Input|AddMovementInput (Variables|Default|GetForwardVector) 1.0 false))

(event Collision|EventActorBeginOverlap
  (params (OtherActor :type Actor%20Object%20Reference)))

(event EventBeginPlay
  ;[1 1 1] Initialize Boss
  (Variables|Default|SetisAttacking false)
  (Variables|Default|SetAlive true)
  (CallFunction|FindPlayer)
  (CallFunction|DistancetoPlayer))

(fn ConstructionScript)

(fn PlayerDistance
  (bind _returnvalue (Transformation|GetActorLocation))
  (bind _returnvalue_2 (Game|GetPlayerCharacter 0))
  (bind _returnvalue_3 (Transformation|GetActorLocation _returnvalue_2))
  (bind _returnvalue_4 (- _returnvalue _returnvalue_3))
  (bind _returnvalue_5 (Math|Vector|VectorLength _returnvalue_4))
  ;[1 1 1] Check if Attacking / Don't if so
  (if (not (Variables|Default|GetisAttacking))
    ;[1 1 1] Detect Player Distance
    (bind _output_get (Variables|Default|SetDistance _returnvalue_5))
    ;[1 1 1] Mid Range
    (if (and (>= _output_get 1e+03) (<= _output_get 1.5e+03))
      (CallFunction|MidRange)
      (else
        ;[1 1 1] Long Range
        (if (>= _returnvalue_5 1501.0)
          (CallFunction|LongRange)
          (else
            ;[1 1 1] Close Range
            (if (<= _returnvalue_5 999.0)
              _
              (else
                _))
            (CallFunction|CloseRange)))))))