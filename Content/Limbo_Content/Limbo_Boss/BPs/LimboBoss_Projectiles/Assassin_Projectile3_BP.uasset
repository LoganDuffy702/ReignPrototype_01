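; Assassin projectile for the Limbo boss that damages the player and leaves fading decals on the ground beneath it.
; Two capsule overlaps spawn an impact effect, apply damage if the player is hit, and destroy the actor on any overlap.
; A looping timer traces down along the actor's up axis to stamp the decals.
; If nothing is hit, the projectile bursts and destroys itself after a fixed delay.
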(event OnComponentBeginOverlap(Capsule)
  (params (OverlappedComponent :type Primitive%20Component%20Object%20Reference) (OtherActor :type Actor%20Object%20Reference) (OtherComp :type Primitive%20Component%20Object%20Reference) (OtherBodyIndex :type Integer) (bFromSweep :type Boolean) (SweepResult :type Hit%20Result%20Structure%20%28by%20ref%29))
  (Effects|SpawnEmitteratLocation "/Game/Reign_Assets/FX/Impacts/Impact1/Impact_1_FX.Impact_1_FX" (.ImpactPoint (Collision|BreakHitResult SweepResult)))
  (if (== OtherActor (Variables|Default|GetPlayerRef))
    (Default|DealingDamage (Variables|Default|GetPlayerRef) (Variables|Default|GetDamage) 0 "None")
    (Actor|DestroyActor)
    (else
      (Actor|DestroyActor))))

(event OnComponentBeginOverlap(Capsule1)
  (params (OverlappedComponent :type Primitive%20Component%20Object%20Reference) (OtherActor :type Actor%20Object%20Reference) (OtherComp :type Primitive%20Component%20Object%20Reference) (OtherBodyIndex :type Integer) (bFromSweep :type Boolean) (SweepResult :type Hit%20Result%20Structure%20%28by%20ref%29))
  (Effects|SpawnEmitteratLocation "/Game/Reign_Assets/FX/Impacts/Impact1/Impact_1_FX.Impact_1_FX" "0, 0, 0")
  (if (== OtherActor (Variables|Default|GetPlayerRef))
    (Default|DealingDamage (Variables|Default|GetPlayerRef) (Variables|Default|GetDamage) 0 "None")
    (Actor|DestroyActor)
    (else
      (Actor|DestroyActor))))

(event Custom|killme
  (Effects|SpawnEmitteratLocation "/Game/Reign_Assets/FX/Impacts/Impact1/Impact_1_FX.Impact_1_FX" (Transformation|GetWorldLocation (Variables|Default|GetCylinder1)))
  (Actor|DestroyActor))

(event Custom|DecalSpawn
  (bind _returnvalue (Transformation|GetActorLocation))
  (bind _outhit (Collision|LineTraceByChannel _returnvalue (- _returnvalue (* (Math|Vector|GetUpVector (Transformation|GetActorRotation)) 1e+03)) "TraceTypeQuery1" false (Utilities|Array|MakeArray self) "None"))
  (bind _returnvalue_2 (Rendering|Decal|SpawnDecalatLocation "/Game/Greed_Content/Greed_Boss/GB_Ground_Decal_Inst.GB_Ground_Decal_Inst" "100.000000,100.000000,100.000000" (.ImpactPoint (Collision|BreakHitResult _outhit)) "90.000000,0.000000,0.000000" 1.0))
  (Rendering|Components|Decal|SetFadeOut _returnvalue_2 0.0 1.0 true)
  (Utilities|Time|SetTimerbyEvent (delegate Custom|DecalSpawn) 0.1 true))

(event EventBeginPlay
  (CallFunction|DecalSpawn)
  (bind _asmc_prototype_bp (Utilities|Casting|CastToMC_Prototype_BP (Game|GetPlayerCharacter 0)))
  (Variables|Default|SetPlayerRef _asmc_prototype_bp)
  (Utilities|FlowControl|Delay 5.0)
  (CallFunction|Killme))

(fn ConstructionScript)