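; Limbo boss character that teleports between platforms, fires projectile fans and chases the player for melee, with a health bar.
; CombatCheck sets speed and attack rates by health, then chases if the urns are broken or plays a ranged montage.
; The boss takes damage only while chasing; a capped melee series ends by repairing the urns and vanishing.
; DoN counters limit teleport hops and swings, and box traces deal melee damage.
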(event Custom|FireRangedAtk
  ;[1 1 1] Projectile
  (CallFunction|ProjectilePicker))

(event Custom|ResetMelee
  ;[1 1 1] CheckAttackRange
  (Variables|Default|SetisAttacking false)
  (Utilities|FlowControl|DoOnce false) ; enters at Reset
)

(event Custom|CheckForAttack
  ;[1 1 1] CheckAttackRange
  (if (<= (Math|Vector|VectorLength (- (Transformation|GetActorLocation (Variables|Default|GetPlayerRef)) (Transformation|GetActorLocation))) 7e+02)
    (Utilities|FlowControl|DoOnce false
      (:Completed
        (CallFunction|CloseRangeCombat)))))

(event Custom|StartBossFight
  ;[1 1 1] Teleporting Events  (Step 1)
  (Utilities|FlowControl|Delay 3.0)
  (Animation|PlayAnimMontage "/Game/Limbo_Content/Limbo_Boss/ShadowAss_Mesh/SA_Animations/SA_Vanish_V1_Montage.SA_Vanish_V1_Montage" 1.0 "None"))

(event Custom|GoToRandLoc
  (bind _numofteleports (Variables|Default|GetNumOfTeleports))
  ;[1 1 1] Teleporting Events  (Step 1)
  (bind _counter (Utilities|FlowControl|DoN _numofteleports)
    (:Exit
      (if (>= _counter _numofteleports)
        (CallFunction|FindNewPlatform)
        (CallFunction|LookatPlayer)
        (Animation|PlayAnimMontage "/Game/Limbo_Content/Limbo_Boss/ShadowAss_Mesh/SA_Animations/SA_Reappear_Montage.SA_Reappear_Montage" 1.0 "None")
        (else
          (bind _location (CallFunction|FindNewPlatform))
          (Effects|SpawnEmitteratLocation "/Game/Reign_Assets/World_Objects/Tunnel_Object/Tunnel_Spawn_FX.Tunnel_Spawn_FX" _location "0, 0, 0" "6.000000,6.000000,6.000000")
          (Utilities|FlowControl|Delay 0.5)
          (CallFunction|GotoRandLoc))))))

(event Custom|Combat
  ;[1 1 1] Damage Solver
  (CallFunction|LongRangeCombat))

(event Custom|Long%20Range%20Combat
  ;[1 1 1] Combat Types (Step 3)
  (CallFunction|LookatPlayer)
  (Rendering|SetVisibility (Variables|Character|GetMesh) true false)
  (Variables|Default|SetisAttacking true)
  (Animation|PlayAnimMontage (Variables|Default|GetLongAtkMontage) 1.0 "None"))

(event Custom|Close%20Range%20Combat
  (bind _maxmeleeatks (Variables|Default|GetMaxMeleeAtks))
  ;[1 1 1] Combat Types (Step 3)
  (bind _counter (Utilities|FlowControl|DoN _maxmeleeatks :!label _label)
    (:Exit
      (if (>= _counter _maxmeleeatks)
        (CallFunction|LookatPlayer)
        (Variables|Default|SetisAttacking true)
        (Animation|Montage|PlayMontage (Variables|Character|GetMesh) (Variables|Default|GetCloseAtkMontage) (Variables|Default|GetMeleePlayRate)
          (:OnCompleted
            (Variables|Default|SetisAttacking false)
            (Variables|Default|SetChasing? false)
            (CallFunction|ResetTeleportCount)
            (Animation|PlayAnimMontage "/Game/Limbo_Content/Limbo_Boss/ShadowAss_Mesh/SA_Animations/SA_Vanish_V1_Montage.SA_Vanish_V1_Montage" 1.0 "None")
            (CallFunction|ResetMelee)
            (Default|RepairUrn (Variables|Default|GetUrns))
            (goto _label Reset)))
        (else
          (CallFunction|LookatPlayer)
          (Variables|Default|SetisAttacking true)
          (Animation|PlayAnimMontage (Variables|Default|GetCloseAtkMontage) (Variables|Default|GetMeleePlayRate) "None"))))))

(event Custom|ResetTeleportCount
  (bind _numofteleports (Variables|Default|GetNumOfTeleports))
  ;[1 1 1] Teleporting Events  (Step 1)
  (Utilities|FlowControl|DoN _numofteleports) ; enters at Reset
)

(event Custom|AttackTraceEvent
  (bind _attackpoint (Variables|Default|GetAttackPoint))
  (bind _returnvalue (Transformation|GetWorldLocation _attackpoint))
  ;[1 1 1] Attack Trace
  (bind _returnvalue_2 (Class|KismetSystemLibrary|BoxTraceSingleforObjects _returnvalue _returnvalue "350.000000,150.000000,500.000000" (Math|Rotator|MakeRotator 0.0 0.0 (.yaw (Transformation|GetWorldRotation (Variables|Collision|GetCapsuleComponent)))) (Utilities|Array|MakeArray "ObjectTypeQuery3") false (Utilities|Array|MakeArray self) "ForDuration" true))
  (if _returnvalue_2
    (Default|DealingDamage (Variables|Default|GetPlayerRef) 10 0 "None")))

(event EventDealingDamage
  (params (Sent%20Damage :type Integer) (Sender :type Actor%20Object%20Reference) (DamageType :type Name :default "None"))
  ;[1 1 1] Damage Solver
  (if (Variables|Default|GetChasing?)
    (Variables|Default|SetCurrentHealth (- (Variables|Default|GetCurrentHealth) 2.0))
    (if (<= (Variables|Default|GetCurrentHealth) 0.0)
      (CallFunction|UpdateBossHealth)
      (Variables|Default|SetAlive false)
      (else
        (CallFunction|UpdateBossHealth)))))

(event EventTick
  (params (DeltaSeconds :type Float%20%28single-precision%29))
  (bind _returnvalue (Game|GetPlayerCharacter 0))
  (bind _returnvalue_2 (Transformation|GetActorLocation))
  (bind _returnvalue_3 (Transformation|GetActorLocation _returnvalue))
  (bind _returnvalue_4 (Math|Rotator|FindLookatRotation _returnvalue_2 _returnvalue_3))
  (bind _returnvalue_5 (Math|Vector|GetForwardVector _returnvalue_4))
  ;[1 1 1] Forward Vector tick and input
  (if (Variables|Default|GetChasing?)
    (CallFunction|CheckforAttack)
    (if (not (Variables|Default|GetisAttacking))
      (Pawn|Input|AddMovementInput (Math|Vector|MakeVector (.x _returnvalue_5) (.y _returnvalue_5) 0.0) 1.0 false))))

(event EventBeginPlay
  ;[1 1 1] Initialize Boss
  (Variables|Default|SetAlive true)
  (bind _asmc_prototype_bp (Utilities|Casting|CastToMC_Prototype_BP (Game|GetPlayerCharacter 0)))
  (Variables|Default|SetPlayerRef _asmc_prototype_bp)
  (|UINode
    (:Out%20execute
      (Variables|Default|SetStartingPoint (Transformation|GetWorldLocation (Variables|Collision|GetCapsuleComponent))))))

(fn ConstructionScript)

(fn CombatCheck
  (Math|Float|CompareFloat (Variables|Default|GetCurrentHealth) 9e+01
    (:>
      (Variables|Default|SetMeleePlayRate 0.5 :!label _label)
      (Variables|Default|SetRangePlayRate 1.0)
      (Variables|Default|SetNumOfTeleports 1)
      (Variables|/Script/Engine.CharacterMovementComponent|SetMaxWalkSpeed (Variables|Character|GetCharacterMovement) 8e+02)
      (Variables|Default|SetMaxMeleeAtks 3))
    (:==
      (goto _label))
    (:<
      (Variables|Default|SetMeleePlayRate 1.0)
      (Variables|Default|SetNumOfTeleports 1)
      (Variables|Default|SetRangePlayRate 1.5)
      (Variables|/Script/Engine.CharacterMovementComponent|SetMaxWalkSpeed (Variables|Character|GetCharacterMovement) 1.6e+03)
      (Variables|Default|SetMaxMeleeAtks 6)))
  (Variables|Default|SetProjectileCount 30)
  (Variables|Default|SetAttackArc 3.6e+02)
  (if (Variables|/Game/Limbo_Content/Limbo_Boss/BPs/Limbo_Boss_Urn_BP.Limbo_Boss_Urn_BP_C|GetBroken? (Variables|Default|GetUrns))
    (Variables|Default|SetChasing? true)
    (else
      (Animation|PlayAnimMontage "/Game/Limbo_Content/Limbo_Boss/ShadowAss_Mesh/SA_Animations/SA_Kiss_Montage.SA_Kiss_Montage" (Variables|Default|GetRangePlayRate) "None"))))

(fn UpdateBossHealth
  (Progress|SetPercent (Variables|/Game/Limbo_Content/Limbo_Boss/Wigits/Limbo_Boss_HealthBar.Limbo_Boss_HealthBar_C|GetBossHealthBar (Variables|Default|GetLimboBoss_HealthWidget)) (/ (Variables|Default|GetCurrentHealth) (Variables|Default|GetMaxHealth))))

(fn LookatPlayer
  (bind _capsulecomponent (Variables|Collision|GetCapsuleComponent))
  (bind _returnvalue (Transformation|GetWorldRotation _capsulecomponent))
  (Transformation|SetWorldRotation (Variables|Collision|GetCapsuleComponent) (Math|Rotator|MakeRotator (.roll _returnvalue) (.pitch _returnvalue) (.yaw (Math|Rotator|FindLookatRotation (Transformation|GetWorldLocation _capsulecomponent) (Transformation|GetWorldLocation (Variables|/Script/Engine.Character|GetCapsuleComponent (Variables|Default|GetPlayerRef)))))) false false))

(fn FindNewPlatform
  (bind _platform_actors (Variables|Default|GetPlatform%20Actors))
  (bind _output (Utilities|Array|Get(acopy) _platform_actors))
  (bind _box (Variables|/Game/Limbo_Content/Limbo_Boss/BPs/LimboBossPlatforms_BP.LimboBossPlatforms_BP_C|GetBox _output))
  (bind _returnvalue (Transformation|GetWorldLocation _box))
  (bind _returnvalue_2 (+ _returnvalue "0, 0,500.000000"))
  (Utilities|Array|Shuffle _platform_actors)
  (Transformation|SetWorldLocation (Variables|Collision|GetCapsuleComponent) _returnvalue_2 false false)
  (Default|LightUP _output)
  (return _returnvalue_2))

(fn ProjectilePicker
  (bind _capsulecomponent (Variables|Collision|GetCapsuleComponent))
  (bind _returnvalue (Transformation|GetWorldRotation _capsulecomponent))
  (bind (_roll _pitch _yaw) (Math|Rotator|BreakRotator _returnvalue))
  (Variables|Default|SetSpacingValue (/ (Variables|Default|GetAttackArc) (Math|Conversions|ToFloat(Integer) (Variables|Default|GetProjectileCount))))
  (for _index (range 0 (- (Variables|Default|GetProjectileCount) 1))
    (Game|SpawnActorfromClass (Utilities|Array|Get(acopy) (Variables|Default|GetProjectileList)) (Math|Transform|MakeTransform (.location (Transformation|GetWorldTransform (Variables|Default|GetAttackPoint))) (Math|Rotator|MakeRotator _roll _pitch (+ (- _yaw (Variables|Default|GetAttackArc)) (* _index (* (Variables|Default|GetSpacingValue) 2.0)))) "1.000000,1.000000,1.000000") "Undefined" 0 0)))