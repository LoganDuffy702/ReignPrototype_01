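; Limbo boss urn actor that sits on a random platform during the boss fight and can be broken and repaired.
; Starting battle shuffles the Platforms array and teleports the urn just above the first platform's PlacementPoint.
; Taking damage flags it Broken and hides its cube mesh.
; Repairing raises every platform, waits briefly, then relocates the urn, clears the flag and shows it again.
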(event Custom|RepairUrn
  (for _array_element (Variables|Default|GetPlatforms)
    (Default|RiseUp _array_element))
  (Utilities|FlowControl|Delay 1.0)
  (CallFunction|FindNewPlatform)
  (Variables|Default|SetBroken? false)
  (Rendering|SetVisibility (Variables|Default|GetCube) true false))

(event Custom|FindNewPlatform
  (bind _platforms (Variables|Default|GetPlatforms))
  (Utilities|Array|Shuffle _platforms)
  (Transformation|SetActorLocation (+ (Transformation|GetWorldLocation (Variables|/Game/Limbo_Content/Limbo_Boss/BPs/Urn_Location_Actor_BP.Urn_Location_Actor_BP_C|GetPlacementPoint (Utilities|Array|Get(acopy) _platforms))) "0, 0,100.000000") false false))

(event Custom|StartBattle
  (CallFunction|FindNewPlatform))

(event EventBeginPlay)

(event EventDealingDamage
  (params (Sent%20Damage :type Integer) (Sender :type Actor%20Object%20Reference) (DamageType :type Name :default "None"))
  (Development|PrintString "Broken Urn")
  (Variables|Default|SetBroken? true)
  (Rendering|SetVisibility (Variables|Default|GetCube) false false))

(fn ConstructionScript)