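; MasterIslandToMap_BP, by its name a master island-to-map Blueprint, tells the player's map widget which island is currently occupied.
; BeginPlay caches the MC_Prototype_BP player character.
; Any MapCollision begin overlap flags IsOnIsland and sets IslandNumber and the widget's CurrentIslandNum to hardcoded values, without checking the overlapping actor.
; End overlap clears the flag and IslandNumber but leaves the widget value unchanged.
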(event OnComponentEndOverlap(MapCollision)
  (params (OverlappedComponent :type Primitive%20Component%20Object%20Reference) (OtherActor :type Actor%20Object%20Reference) (OtherComp :type Primitive%20Component%20Object%20Reference) (OtherBodyIndex :type Integer))
  ;[1 1 1] Set Var for in/out of Col box
  (Variables|Default|SetIsOnIsland? false)
  (if (Variables|Default|GetIsOnIsland?)
    (Variables|Default|SetIsland%20Number 1)
    (Variables|/Game/Limbo_Content/Map_Widget/Map_Widget.Map_Widget_C|SetCurrentIslandNum (Variables|/Game/Reign_Assets/Player_Character/Blueprints/MC_Prototype_BP.MC_Prototype_BP_C|GetMapWidget (Variables|Default|GetPlayerRef)) 0)
    (else
      (Variables|Default|SetIsland%20Number 0))))

(event OnComponentBeginOverlap(MapCollision)
  (params (OverlappedComponent :type Primitive%20Component%20Object%20Reference) (OtherActor :type Actor%20Object%20Reference) (OtherComp :type Primitive%20Component%20Object%20Reference) (OtherBodyIndex :type Integer) (bFromSweep :type Boolean) (SweepResult :type Hit%20Result%20Structure%20%28by%20ref%29))
  ;[1 1 1] Set Var for in/out of Col box
  (Variables|Default|SetIsOnIsland? true)
  (if (Variables|Default|GetIsOnIsland?)
    (Variables|Default|SetIsland%20Number 1)
    (Variables|/Game/Limbo_Content/Map_Widget/Map_Widget.Map_Widget_C|SetCurrentIslandNum (Variables|/Game/Reign_Assets/Player_Character/Blueprints/MC_Prototype_BP.MC_Prototype_BP_C|GetMapWidget (Variables|Default|GetPlayerRef)) 0)
    (else
      (Variables|Default|SetIsland%20Number 0))))

(event EventBeginPlay
  (bind _asmc_prototype_bp (Utilities|Casting|CastToMC_Prototype_BP (Game|GetPlayerCharacter 0)))
  (Variables|Default|SetPlayerRef _asmc_prototype_bp))

(fn ConstructionScript)