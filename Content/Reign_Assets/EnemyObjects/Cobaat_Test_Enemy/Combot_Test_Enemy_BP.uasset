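; Test combat enemy that reacts to the player's combo and chain attacks by damage type.
; Air, spike and uppercut hits juggle it through launches, velocity stops and timed zero-gravity hangs, gated on whether it is airborne.
; Grapple and pull-to hits subtract health, then timelines drag the enemy toward the player or the player toward it.
; During the drag the weapon's chain beam tracks the enemy's choke point, and the weapon resets afterward.
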(event Custom|LaunchEnemy
  (params (ZVelocity :type Float%20%28single-precision%29))
  (bind _returnvalue (Transformation|GetActorLocation))
  (bind _playerref (Variables|Default|GetPlayerRef))
  (bind _returnvalue_2 (Transformation|GetActorLocation _playerref))
  (bind _returnvalue_3 (- _returnvalue _returnvalue_2))
  (bind _returnvalue_4 (Math|Vector|Normalize _returnvalue_3))
  (Character|LaunchCharacter (Math|Vector|MakeVector (* (.x _returnvalue_4) 5e+02) (* (.y _returnvalue_4) 5e+02) ZVelocity) false true)
  (Utilities|FlowControl|Delay 0.25)
  (Variables|/Script/Engine.MovementComponent|SetVelocity (Variables|Character|GetCharacterMovement) "0, 0, 0")
  (Variables|/Script/Engine.CharacterMovementComponent|SetGravityScale (Variables|Character|GetCharacterMovement) 0.0)
  (Utilities|FlowControl|Delay 1.0)
  (Variables|/Script/Engine.CharacterMovementComponent|SetGravityScale (Variables|Character|GetCharacterMovement) 1.0))

(event Custom|HitInAir
  (bind _charactermovement (Variables|Character|GetCharacterMovement))
  (Variables|/Script/Engine.CharacterMovementComponent|SetGravityScale _charactermovement 0.0)
  (Variables|/Script/Engine.MovementComponent|SetVelocity _charactermovement "0, 0, 0")
  (Utilities|FlowControl|RetriggerableDelay 1.0)
  (Variables|/Script/Engine.CharacterMovementComponent|SetGravityScale _charactermovement 1.0))

(event Custom|Spike
  (params (ZVelocity :type Float%20%28single-precision%29))
  (Variables|/Script/Engine.CharacterMovementComponent|SetGravityScale (Variables|Character|GetCharacterMovement) 1.0)
  (Character|LaunchCharacter (Math|Vector|MakeVector 0.0 0.0 ZVelocity) false true)
  (Utilities|FlowControl|Delay 0.25)
  (Variables|/Script/Engine.MovementComponent|SetVelocity (Variables|Character|GetCharacterMovement) "0, 0, 0"))

(event Custom|GrappleDamageEvent
  (bind _returnvalue (Transformation|GetActorLocation))
  (bind _playerref (Variables|Default|GetPlayerRef))
  (bind _aoe_point (Variables|/Game/Reign_Assets/Player_Character/Blueprints/MC_Prototype_BP.MC_Prototype_BP_C|GetAoE%20Point _playerref))
  (bind _returnvalue_2 (Transformation|GetWorldLocation _aoe_point))
  (Variables|Default|SetCurrentHealth (- (Variables|Default|GetCurrentHealth) (Variables|Default|GetTakenDamage)))
  (bind _newtrack_0 (Timeline|Timeline_1 PlayFromStart)
    (:Update
      (Class|ParticleSystemComponent|SetBeamEndPoint (Variables|/Game/Reign_Assets/Weapon_BP/Master_Weapon_BP.Master_Weapon_BP_C|GetChainParticle (Variables|/Game/Reign_Assets/Player_Character/Blueprints/MC_Prototype_BP.MC_Prototype_BP_C|GetEquippedWeapon (Variables|Default|GetPlayerRef))) 0 (Transformation|GetWorldLocation (Variables|Default|GetChokePoint)))
      (Transformation|SetActorLocation (Math|Vector|Lerp(Vector) (Math|Vector|MakeVector (.x _returnvalue) (.y _returnvalue) (.z _returnvalue)) (Math|Vector|MakeVector (.x _returnvalue_2) (.y _returnvalue_2) (.z _returnvalue)) _newtrack_0) false false))
    (:Finished
      (Default|WeaponReset (Variables|/Game/Reign_Assets/Player_Character/Blueprints/MC_Prototype_BP.MC_Prototype_BP_C|GetEquippedWeapon (Variables|Default|GetPlayerRef))))))

(event Custom|PullToDamageEvent
  (bind _capsulecomponent (Variables|Default|GetCapsuleComponent))
  (bind _playerref (Variables|Default|GetPlayerRef))
  (bind _returnvalue (Transformation|GetWorldLocation _capsulecomponent))
  (bind _capsulecomponent_2 (Variables|/Script/Engine.Character|GetCapsuleComponent _playerref))
  (bind _returnvalue_2 (Transformation|GetWorldLocation _capsulecomponent_2))
  ;[1 1 1] PullTo Damage Event
  (Variables|Default|SetCurrentHealth (- (Variables|Default|GetCurrentHealth) (Variables|Default|GetTakenDamage)))
  (bind _newtrack_0 (Timeline|Timeline_0 PlayFromStart)
    (:Update
      (Class|ParticleSystemComponent|SetBeamEndPoint (Variables|/Game/Reign_Assets/Weapon_BP/Master_Weapon_BP.Master_Weapon_BP_C|GetChainParticle (Variables|/Game/Reign_Assets/Player_Character/Blueprints/MC_Prototype_BP.MC_Prototype_BP_C|GetEquippedWeapon (Variables|Default|GetPlayerRef))) 0 (Transformation|GetWorldLocation (Variables|Default|GetChokePoint)))
      (Transformation|SetActorLocation (Variables|Default|GetPlayerRef) (Math|Vector|Lerp(Vector) (Math|Vector|MakeVector (.x _returnvalue_2) (.y _returnvalue_2) (.z _returnvalue)) (Math|Vector|MakeVector (.x _returnvalue) (.y _returnvalue) (.z _returnvalue)) _newtrack_0) false false))
    (:Finished
      (Default|WeaponReset (Variables|/Game/Reign_Assets/Player_Character/Blueprints/MC_Prototype_BP.MC_Prototype_BP_C|GetEquippedWeapon (Variables|Default|GetPlayerRef))))))

(event EventBeginPlay
  (|CallParentFunction))

(event Collision|EventActorBeginOverlap
  (params (OtherActor :type Actor%20Object%20Reference)))

(event EventTick
  (params (DeltaSeconds :type Float%20%28single-precision%29))
  (|CallParentFunction DeltaSeconds))

(event EventDealingDamage
  (params (Sent%20Damage :type Integer) (Sender :type Actor%20Object%20Reference) (DamageType :type Name :default "None"))
  (bind _returnvalue (Transformation|GetVelocity))
  (bind _charactermovement (Variables|Character|GetCharacterMovement))
  (bind _returnvalue_2 (AI|Components|NavMovement|IsFalling _charactermovement))
  (bind _returnvalue_3 (>= (.z _returnvalue) 0.0))
  (bind _returnvalue_4 (and _returnvalue_2 _returnvalue_3))
  (switch name DamageType
    (:AIR
      (if _returnvalue_4
        (CallFunction|HitinAir)))
    (:SPIKE
      (if _returnvalue_4
        (CallFunction|Spike -2.5e+03)))
    (:UPPERCUT
      (if (not _returnvalue_2)
        (CallFunction|LaunchEnemy 2.5e+03)))
    (:Grapple
      (Utilities|FlowControl|Delay 0.2)
      (Variables|/Script/Engine.MovementComponent|SetVelocity (Variables|/Script/Engine.Character|GetCharacterMovement (Variables|Default|GetPlayerRef)) "0, 0, 0")
      (CallFunction|GrappleDamageEvent))
    (:PullTo
      (Utilities|FlowControl|Delay 0.15)
      (Variables|/Script/Engine.MovementComponent|SetVelocity (Variables|/Script/Engine.Character|GetCharacterMovement (Variables|Default|GetPlayerRef)) "0, 0, 0")
      (CallFunction|PulltoDamageEvent))))

(fn ConstructionScript
  (|CallParentFunction))