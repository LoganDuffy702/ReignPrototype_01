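; Beatup training dummy enemy that takes hits and can optionally damage the player.
; When enabled, a looping one-second timer sphere-traces for nearby pawns and damages the stored player reference.
; Hits either unlock a player skill when Alt is set, or subtract fixed health and show the sent damage via healthbar and spawned actor.
; They also feed the damage-type solver and a running total cleared by a retriggerable delay.
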(event Custom|HurtPlayer
  (bind _returnvalue (Transformation|GetActorLocation))
  (bind _returnvalue_2 (Collision|SphereTraceForObjects _returnvalue _returnvalue 4e+02 (Utilities|Array|MakeArray "ObjectTypeQuery3") false 0 "ForDuration" true "(R=1.000000,G=0.000000,B=0.000000,A=1.000000)" "(R=0.000000,G=1.000000,B=0.000000,A=1.000000)" 0.5))
  (if _returnvalue_2
    (Default|DealingDamage (Variables|Default|GetPlayerRef) 2 0 "None"))
  (Utilities|Time|SetTimerbyEvent (delegate Custom|HurtPlayer) 1.0 true))

(event EventBeginPlay
  (|CallParentFunction)
  (if (Variables|Default|GetHurtPlayer?)
    (CallFunction|HurtPlayer)))

(event Collision|EventActorBeginOverlap
  (params (OtherActor :type Actor%20Object%20Reference)))

(event EventTick
  (params (DeltaSeconds :type Float%20%28single-precision%29))
  (|CallParentFunction DeltaSeconds) ; This node is disabled and will not be called.\nDrag off pins to build functionality.
)

(event EventDealingDamage
  (params (Sent%20Damage :type Integer) (Sender :type Actor%20Object%20Reference) (DamageType :type Name :default "None"))
  (if (Variables|Default|GetAlt?)
    (Default|UnlockNewSkill (Variables|Default|GetPlayerRef))
    (else
      (CallFunction|ShowHealthbar)
      (Variables|Default|SetCurrentHealth (- (Variables|Default|GetCurrentHealth) 2))
      (Game|SpawnActorfromClass "/Game/Reign_Assets/Reign_UI/ShowDmg_Actor.ShowDmg_Actor_C" (Math|Transform|MakeTransform (Transformation|GetActorLocation) "0, 0, 0" "1,1,1") "AlwaysSpawn" 0 Sent%20Damage 0)
      (CallFunction|UpdateHealth)
      (Default|LogansDmgSolver (Variables|Default|GetLogans_Damage_Component) DamageType 0.0 self 0.0 0.0 2e+02 3.5e+02)
      (Variables|Default|SetPrevious%20Dmg (+ Sent%20Damage (Variables|Default|GetPrevious%20Dmg)))
      (Development|PrintString (Utilities|String|ToString(Integer) Sent%20Damage) true true "(R=0.000000,G=0.660000,B=1.000000,A=1.000000)" 1.0)
      (Utilities|FlowControl|RetriggerableDelay 1.0)
      (Variables|Default|SetPrevious%20Dmg 0))))

(fn ConstructionScript
  (|CallParentFunction))