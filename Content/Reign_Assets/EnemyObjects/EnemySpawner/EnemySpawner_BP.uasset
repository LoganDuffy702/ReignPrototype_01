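; EnemySpawner_BP is an enemy spawner actor that stages a portal unlock.
; The first activation overlap blends the camera to the spawner, starts its particle system, returns the view to the player and unlocks the portal.
; SpawnEnemies spawns the first listed class at a random SpawnZone point with tunnel FX and records it in SpawnArray.
; Wave logic is unfinished: SpawnEnemies has no caller here, the alive-check timer is disconnected and WaveCheck does nothing.
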(event OnComponentBeginOverlap(ActivationCollision)
  (params (OverlappedComponent :type Primitive%20Component%20Object%20Reference) (OtherActor :type Actor%20Object%20Reference) (OtherComp :type Primitive%20Component%20Object%20Reference) (OtherBodyIndex :type Integer) (bFromSweep :type Boolean) (SweepResult :type Hit%20Result%20Structure%20%28by%20ref%29))
  (Utilities|FlowControl|DoOnce false
    (:Completed
      (Game|Player|SetViewTargetwithBlend (Game|GetPlayerController 0) self 1.0 "VTBlend_Linear" 0.0 false)
      (Utilities|FlowControl|Delay 1.0)
      (Components|Activation|Activate (Variables|Default|GetParticleSystem) false)
      (Utilities|FlowControl|Delay 3.0)
      (Game|Player|SetViewTargetwithBlend (Game|GetPlayerController 0) (Variables|Default|GetPlayerRef) 1.0 "VTBlend_Linear" 0.0 false)
      (Default|UnlockPortal (Variables|Default|GetActivatePortal_Component)))))

(event Custom|Wave%20Check
  (if (>= (Variables|Default|GetWaveCount) (Variables|Default|GetTotalWaves))
    _))

(event Custom|CheckForNextWave
  (for _array_element (Variables|Default|GetSpawnArray)
    (Utilities|IsValid _array_element
      (:Is%20Valid
        (Variables|Default|SetAllAlive? true))))
  (if (not (Variables|Default|GetAllAlive?))
    (Development|PrintString "Hello")
    (Components|Activation|Deactivate (Variables|Default|GetParticleSystem))))

(event EventBeginPlay
  (bind _asmc_prototype_bp (Utilities|Casting|CastToMC_Prototype_BP (Game|GetPlayerCharacter 0)))
  (Variables|Default|SetPlayerRef _asmc_prototype_bp))

(fn ConstructionScript)

(fn SpawnEnemies
  (bind _spawnzone (Variables|Default|GetSpawnZone))
  (LocalVariables|SetSpawnPoint (Math|Random|RandomPointinBoundingBox (Transformation|GetWorldLocation _spawnzone) (Variables|/Script/Engine.BoxComponent|GetBoxExtent _spawnzone)))
  (Effects|SpawnEmitteratLocation "/Game/Reign_Assets/World_Objects/Tunnel_Object/Tunnel_Spawn_FX.Tunnel_Spawn_FX" (LocalVariables|GetSpawnPoint) "0, 0, 0" "2.000000,2.000000,2.000000")
  (bind _returnvalue (Game|SpawnActorfromClass (Utilities|Array|Get(acopy) (Variables|Default|GetSpawnActors)) (Math|Transform|MakeTransform (LocalVariables|GetSpawnPoint) "0, 0, 0" "2.000000,2.000000,2.000000") "Undefined" 0 0))
  (bind _output_get (Variables|Default|SetLastSpawn _returnvalue))
  (Utilities|Array|Add (Variables|Default|GetSpawnArray) _output_get))