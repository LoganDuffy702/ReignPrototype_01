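; Big flower enemy with three eyeballs that track the player while connected, with overlap volumes for waking and attacking.
; Attack overlap starts a delayed random MultiGate that sets spin or basic attack flags, or waits again.
; Melee, grapple and pull hits all deal equal damage; death launches the eyeballs with physics, drives their dynamic material speed parameter, then explodes them, damaging the player via sphere trace, before destroying the actor.
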(event OnComponentBeginOverlap(WakeUpCollision)
  (params (OverlappedComponent :type Primitive%20Component%20Object%20Reference) (OtherActor :type Actor%20Object%20Reference) (OtherComp :type Primitive%20Component%20Object%20Reference) (OtherBodyIndex :type Integer) (bFromSweep :type Boolean) (SweepResult :type Hit%20Result%20Structure%20%28by%20ref%29))
  (Variables|Default|SetAsleep? false))

(event OnComponentEndOverlap(WakeUpCollision)
  (params (OverlappedComponent :type Primitive%20Component%20Object%20Reference) (OtherActor :type Actor%20Object%20Reference) (OtherComp :type Primitive%20Component%20Object%20Reference) (OtherBodyIndex :type Integer))
  (Variables|Default|SetAsleep? true))

(event OnComponentBeginOverlap(AttackCollision)
  (params (OverlappedComponent :type Primitive%20Component%20Object%20Reference) (OtherActor :type Actor%20Object%20Reference) (OtherComp :type Primitive%20Component%20Object%20Reference) (OtherBodyIndex :type Integer) (bFromSweep :type Boolean) (SweepResult :type Hit%20Result%20Structure%20%28by%20ref%29))
  (Utilities|FlowControl|RetriggerableDelay 2.0)
  (CallFunction|PrepareNextAtk))

(event Custom|EyeTimer
  (params (DeltaTime :type Float%20%28single-precision%29))
  (for _array_element (Variables|Default|GetDynamicMAt)
    (Rendering|Material|SetScalarParameterValue _array_element "F_Speed" (Math|Interpolation|FInterptoConstant 0.0 5.0 0.01 2e+02) :!class /Script/Engine.MaterialInstanceDynamic)))

(event Custom|DestroyEye
  (for _array_element (Utilities|Array|MakeArray (Variables|Default|GetEyeBall) (Variables|Default|GetEyeBall_2) (Variables|Default|GetEyeBall_3))
    (Effects|SpawnEmitteratLocation "/Game/StarterContent/Particles/P_Explosion.P_Explosion" (Transformation|GetWorldLocation _array_element) "0, 0, 0" "3.000000,3.000000,3.000000")
    (Audio|PlaySoundatLocation "/Game/StarterContent/Audio/Explosion01.Explosion01" (Transformation|GetWorldLocation _array_element) "0, 0, 0" 0.2 1.0 0.0 0 0 0)
    (bind _returnvalue (Collision|SphereTraceForObjects (Transformation|GetWorldLocation _array_element) (Transformation|GetWorldLocation _array_element) 3e+02 (Utilities|Array|MakeArray "ObjectTypeQuery3") false (Utilities|Array|MakeArray self) "None"))
    (if _returnvalue
      (Default|DealingDamage (Variables|Default|GetPlayerRef) 20 self "None"))
    (Components|DestroyComponent _array_element)))

(event Custom|DestroyFlower
  (Utilities|FlowControl|Delay 7.0)
  (Actor|DestroyActor))

(event Custom|PrepareNextAtk
  ;[1 1 1] Comment
  (Utilities|FlowControl|Delay 3.0)
  (Utilities|FlowControl|MultiGate true true -1
    (:Out%200
      (Variables|Default|SetSpinAttack? true))
    (:Out%201
      (Variables|Default|SetBasicAttack? true))
    (:Out%202
      (CallFunction|PrepareNextAtk))))

(event EventBeginPlay
  (|CallParentFunction)
  (for _array_element (Utilities|Array|MakeArray (Variables|Default|GetEyeBall) (Variables|Default|GetEyeBall_2) (Variables|Default|GetEyeBall_3))
    (bind _returnvalue (Rendering|Material|CreateDynamicMaterialInstance _array_element 0 "/Game/Reign_Assets/EnemyObjects/FlowerEnemy/Mesh/Materials/Eyeball_Mat_Inst.Eyeball_Mat_Inst" "None" :!class /Script/Engine.PrimitiveComponent))
    (Utilities|Array|Add (Variables|Default|GetDynamicMAt) _returnvalue)))

(event Collision|EventActorBeginOverlap
  (params (OtherActor :type Actor%20Object%20Reference)))

(event EventTick
  (params (DeltaSeconds :type Float%20%28single-precision%29))
  (bind (_x _y _returnvalue_yaw) (|LookAtNode))
  (|CallParentFunction DeltaSeconds)
  (if (Variables|Default|GetConnected?)
    (for _array_element (Utilities|Array|MakeArray (Variables|Default|GetEyeBall) (Variables|Default|GetEyeBall_2) (Variables|Default|GetEyeBall_3))
      (Transformation|SetWorldRotation _array_element (Math|Rotator|MakeRotator _x _y _returnvalue_yaw) false false))
    (else
      (CallFunction|EyeTimer 0.0))))

(event EventDealingDamage
  (params (Sent%20Damage :type Integer) (Sender :type Actor%20Object%20Reference) (DamageType :type Name :default "None"))
  (switch name DamageType
    (:Melee
      _)
    (:Grapple
      _)
    (:PullTo
      _))
  (Variables|Default|SetCurrentHealth (- (Variables|Default|GetCurrentHealth) 15))
  (CallFunction|ShowHealthbar)
  (CallFunction|UpdateHealth)
  (if (<= (Variables|Default|GetCurrentHealth) 0)
    (Variables|Default|SetConnected? false)
    (for _array_element (Utilities|Array|MakeArray (Variables|Default|GetEyeBall) (Variables|Default|GetEyeBall_2) (Variables|Default|GetEyeBall_3))
      (Physics|SetSimulatePhysics _array_element true)
      (Physics|AddImpulse _array_element (|LogansVelocitySolver) "None" false))
    (Variables|Default|SetAlive? false)
    (Utilities|FlowControl|Sequence
      (:then_0
        (Utilities|FlowControl|Delay 0.4)
        (Default|WeaponReset (Variables|/Game/Reign_Assets/Player_Character/Blueprints/MC_Prototype_BP.MC_Prototype_BP_C|GetEquippedWeapon (Variables|Default|GetPlayerRef))))
      (:then_1
        (Utilities|FlowControl|Delay 3.0)
        (CallFunction|DestroyEye))
      (:then_2
        (CallFunction|DestroyFlower)))))

(fn ConstructionScript
  (|CallParentFunction))