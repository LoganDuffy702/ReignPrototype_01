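; Flower enemy whose eyeball yaws to track the player while attached and becomes a delayed bomb when hit.
; The first hit detaches it with a physics impulse against the player's facing, lifted by distance, and drives a material speed parameter.
; The eye later explodes, damaging the player if a sphere trace finds any pawn, and the flower destroys itself afterwards.
; An overlap volume toggles its Asleep flag.
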(event OnComponentBeginOverlap(WakeUpCollision)
  (params (OverlappedComponent :type Primitive%20Component%20Object%20Reference) (OtherActor :type Actor%20Object%20Reference) (OtherComp :type Primitive%20Component%20Object%20Reference) (OtherBodyIndex :type Integer) (bFromSweep :type Boolean) (SweepResult :type Hit%20Result%20Structure%20%28by%20ref%29))
  (Variables|Default|SetAsleep? false))

(event OnComponentEndOverlap(WakeUpCollision)
  (params (OverlappedComponent :type Primitive%20Component%20Object%20Reference) (OtherActor :type Actor%20Object%20Reference) (OtherComp :type Primitive%20Component%20Object%20Reference) (OtherBodyIndex :type Integer))
  (Variables|Default|SetAsleep? true))

(event Custom|EyeTimer
  (params (DeltaTime :type Float%20%28single-precision%29))
  (Rendering|Material|SetScalarParameterValue (Variables|Default|GetDynamicMAt) "F_Speed" (Math|Interpolation|FInterptoConstant 0.0 5.0 0.01 2e+02) :!class /Script/Engine.MaterialInstanceDynamic))

(event Custom|DestroyEye
  (bind _eyeball (Variables|Default|GetEyeBall))
  (bind _eyeball_2 (Variables|Default|GetEyeBall))
  (bind _returnvalue (Transformation|GetWorldLocation _eyeball))
  (bind _returnvalue_2 (Transformation|GetWorldLocation _eyeball_2))
  (Effects|SpawnEmitteratLocation "/Game/StarterContent/Particles/P_Explosion.P_Explosion" _returnvalue "0, 0, 0" "3.000000,3.000000,3.000000")
  (Audio|PlaySoundatLocation "/Game/StarterContent/Audio/Explosion01.Explosion01" _returnvalue "0, 0, 0" 0.2 1.0 0.0 0 0 0)
  (bind _returnvalue_3 (Collision|SphereTraceForObjects _returnvalue_2 _returnvalue_2 3e+02 (Utilities|Array|MakeArray "ObjectTypeQuery3") false (Utilities|Array|MakeArray self) "None"))
  (if _returnvalue_3
    (Default|DealingDamage (Variables|Default|GetPlayerRef) 20 self "None"))
  (Components|DestroyComponent (Variables|Default|GetEyeBall)))

(event Custom|DestroyFlower
  (Utilities|FlowControl|Delay 7.0)
  (Actor|DestroyActor))

(event EventBeginPlay
  (|CallParentFunction)
  (bind _returnvalue (Rendering|Material|CreateDynamicMaterialInstance (Variables|Default|GetEyeBall) 0 "/Game/Reign_Assets/EnemyObjects/FlowerEnemy/Mesh/Materials/Eyeball_Mat_Inst.Eyeball_Mat_Inst" "None" :!class /Script/Engine.PrimitiveComponent))
  (Variables|Default|SetDynamicMAt _returnvalue))

(event Collision|EventActorBeginOverlap
  (params (OtherActor :type Actor%20Object%20Reference)))

(event EventTick
  (params (DeltaSeconds :type Float%20%28single-precision%29))
  (|CallParentFunction DeltaSeconds)
  (if (Variables|Default|GetConnected?)
    (Transformation|SetWorldRotation (Variables|Default|GetEyeBall) (Math|Rotator|MakeRotator 0.0 0.0 (.yaw (Math|Rotator|FindLookatRotation (Transformation|GetWorldLocation (Variables|Default|GetEyeBall)) (Transformation|GetWorldLocation (Variables|/Script/Engine.Character|GetCapsuleComponent (Variables|Default|GetPlayerRef)))))) false false)
    (else
      (CallFunction|EyeTimer 0.0))))

(event EventDealingDamage
  (params (Sent%20Damage :type Integer) (Sender :type Actor%20Object%20Reference) (DamageType :type Name :default "None"))
  (bind _playerref (Variables|Default|GetPlayerRef))
  (bind _capsulecomponent (Variables|/Script/Engine.Character|GetCapsuleComponent _playerref))
  (bind _returnvalue (Math|Vector|GetForwardVector _capsulecomponent))
  (bind _returnvalue_2 (* _returnvalue -1))
  (bind (_x _y) (Math|Vector|BreakVector _returnvalue_2))
  (Variables|Default|SetCanBeLockedOn? false)
  (if (Variables|Default|GetAlive?)
    (Utilities|FlowControl|MultiGate false false -1
      (:Out%200
        (Variables|Default|SetConnected? false)
        (Physics|SetSimulatePhysics (Variables|Default|GetEyeBall) true)
        (Physics|AddImpulse (Variables|Default|GetEyeBall) (+ (* _returnvalue_2 50000) (Math|Vector|MakeVector _x _y (* (Math|Vector|VectorLength (- (Transformation|GetWorldLocation _capsulecomponent) (Transformation|GetWorldLocation (Variables|Default|GetEyeBall)))) 2e+02))) "None" false)
        (Variables|Default|SetAlive? false)
        (Utilities|FlowControl|Sequence
          (:then_0
            (Utilities|FlowControl|Delay 0.4)
            (Default|WeaponReset (Variables|/Game/Reign_Assets/Player_Character/Blueprints/MC_Prototype_BP.MC_Prototype_BP_C|GetEquippedWeapon (Variables|Default|GetPlayerRef))))
          (:then_1
            (Utilities|FlowControl|Delay 3.0)
            (CallFunction|DestroyEye))
          (:then_2
            (CallFunction|DestroyFlower))))
      (:Out%201
        (Utilities|FlowControl|Delay 0.4)
        (Default|WeaponReset (Variables|/Game/Reign_Assets/Player_Character/Blueprints/MC_Prototype_BP.MC_Prototype_BP_C|GetEquippedWeapon (Variables|Default|GetPlayerRef)))))))

(fn ConstructionScript
  (|CallParentFunction))