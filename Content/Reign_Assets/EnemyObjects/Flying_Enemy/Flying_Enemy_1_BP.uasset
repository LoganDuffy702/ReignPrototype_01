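; Flying enemy that hovers on four hover components, chases the player with physics forces once aggroed, and dies below a height limit.
; It repeatedly fires a charged beam at the player's sampled position after a short delay, dealing damage on a trace hit.
; Grapples freeze it and reel the player in, pulls spin and drop it temporarily, and melee knocks it back, with pull and melee costing health.
; Wall-avoidance logic exists but is unwired.
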(event OnComponentBeginOverlap(AgroCollision)
  (params (OverlappedComponent :type Primitive%20Component%20Object%20Reference) (OtherActor :type Actor%20Object%20Reference) (OtherComp :type Primitive%20Component%20Object%20Reference) (OtherBodyIndex :type Integer) (bFromSweep :type Boolean) (SweepResult :type Hit%20Result%20Structure%20%28by%20ref%29))
  (Variables|Default|SetAgroed? true))

(event Custom|PullTo%20Event
  (bind _capsulecomponent (Variables|Default|GetCapsuleComponent))
  (bind _hovercomponent_bp2 (Variables|Default|GetHoverComponent_BP2))
  (bind _hovercomponent_bp3 (Variables|Default|GetHoverComponent_BP3))
  (bind _hovercomponent_bp (Variables|Default|GetHoverComponent_BP))
  (bind _hovercomponent_bp1 (Variables|Default|GetHoverComponent_BP1))
  (bind _array (Utilities|Array|MakeArray _hovercomponent_bp2 _hovercomponent_bp3 _hovercomponent_bp _hovercomponent_bp1))
  ;[1 1 1] Pull To
  (if (Variables|Default|GetFlyingActive?)
    (Variables|Default|SetCurrentHealth (- (Variables|Default|GetCurrentHealth) 20))
    (CallFunction|UpdateHealth)
    (if (<= (Variables|Default|GetCurrentHealth) 0)
      (Default|WeaponReset (Variables|/Game/Reign_Assets/Player_Character/Blueprints/MC_Prototype_BP.MC_Prototype_BP_C|GetEquippedWeapon (Variables|Default|GetPlayerRef)))
      (CallFunction|DeathEvent)
      (else
        (Variables|Default|SetFlyingActive? false)
        (Variables|Default|SetAgroed? false)
        (Class|PrimitiveComponent|AddTorqueinDegrees (Variables|Default|GetCapsuleComponent) "0,0.000000,2000000000.000000" "None" false)
        (Variables|Default|SetResetLoc (Transformation|GetWorldLocation _capsulecomponent))
        (Variables|Default|SetResetRot (Transformation|GetWorldRotation _capsulecomponent))
        (Utilities|FlowControl|Delay 0.2)
        (Default|WeaponReset (Variables|/Game/Reign_Assets/Player_Character/Blueprints/MC_Prototype_BP.MC_Prototype_BP_C|GetEquippedWeapon (Variables|Default|GetPlayerRef)))
        (for _array_element _array
          (Variables|/Game/Reign_Assets/EnemyObjects/Flying_Enemy/HoverComponent_BP.HoverComponent_BP_C|SetHoverDistance _array_element 5e+01))
        (Utilities|FlowControl|Delay (Variables|Default|GetRecoverTime))
        (Variables|Default|SetAgroed? true)
        (Variables|Default|SetFlyingActive? true)
        (for _array_element_2 _array
          (Variables|/Game/Reign_Assets/EnemyObjects/Flying_Enemy/HoverComponent_BP.HoverComponent_BP_C|SetHoverDistance _array_element_2 5e+02))))
    (else
      (Variables|Default|SetCurrentHealth (- (Variables|Default|GetCurrentHealth) 10))
      (CallFunction|UpdateHealth)
      (if (<= (Variables|Default|GetCurrentHealth) 0)
        (Default|WeaponReset (Variables|/Game/Reign_Assets/Player_Character/Blueprints/MC_Prototype_BP.MC_Prototype_BP_C|GetEquippedWeapon (Variables|Default|GetPlayerRef)))
        (CallFunction|DeathEvent)
        (else
          (Development|PrintString "wait")
          (Utilities|FlowControl|Delay 0.2)
          (Default|WeaponReset (Variables|/Game/Reign_Assets/Player_Character/Blueprints/MC_Prototype_BP.MC_Prototype_BP_C|GetEquippedWeapon (Variables|Default|GetPlayerRef))))))))

(event Custom|MeleeDamge
  (bind _capsulecomponent (Variables|Default|GetCapsuleComponent))
  ;[1 1 1] Melle + PullTo
  (CallFunction|ShowHealthbar)
  (Variables|Default|SetCurrentHealth (- (Variables|Default|GetCurrentHealth) 15))
  (CallFunction|UpdateHealth)
  (if (<= (Variables|Default|GetCurrentHealth) 0)
    (CallFunction|DeathEvent)
    (else
      (if (Variables|Default|GetIWasGrappled?)
        (Utilities|FlowControl|RetriggerableDelay 0.6)
        (else
          (|SetLastVec&KnockBack
            (:ex
              _))))
      (for _array_element (Utilities|Array|MakeArray (Variables|Default|GetHoverComponent_BP2) (Variables|Default|GetHoverComponent_BP3) (Variables|Default|GetHoverComponent_BP) (Variables|Default|GetHoverComponent_BP1))
        (Variables|/Game/Reign_Assets/EnemyObjects/Flying_Enemy/HoverComponent_BP.HoverComponent_BP_C|SetI%20Can%20Hover? _array_element true)
        (Physics|SetSimulatePhysics _capsulecomponent true)
        (if (Variables|Default|GetIWasGrappled?)
          (Physics|AddImpulse _capsulecomponent (Variables|Default|GetLastFV) "None" false)
          (Variables|Default|SetIWasGrappled? false)
          (else
            (Physics|AddImpulse _capsulecomponent (Variables|Default|GetLastFV) "None" false)))
        (Utilities|FlowControl|Delay 0.2)
        (Variables|Default|SetFlyingActive? true))
      (Physics|SetSimulatePhysics _capsulecomponent true)
      (if (Variables|Default|GetIWasGrappled?)
        (Physics|AddImpulse _capsulecomponent (Variables|Default|GetLastFV) "None" false)
        (Variables|Default|SetIWasGrappled? false)
        (else
          (Physics|AddImpulse _capsulecomponent (Variables|Default|GetLastFV) "None" false)))
      (Utilities|FlowControl|Delay 0.2)
      (Variables|Default|SetFlyingActive? true))))

(event Custom|Grappling%20Event
  (bind _capsulecomponent (Variables|Default|GetCapsuleComponent))
  (bind _playerref (Variables|Default|GetPlayerRef))
  (bind _playerref_2 (Variables|Default|GetPlayerRef))
  (bind _playerref_3 (Variables|Default|GetPlayerRef))
  ;[1 1 1] Melle + PullTo
  (Variables|Default|SetIWasGrappled? true)
  (Variables|Default|SetFlyingActive? false)
  (for _array_element (Utilities|Array|MakeArray (Variables|Default|GetHoverComponent_BP2) (Variables|Default|GetHoverComponent_BP3) (Variables|Default|GetHoverComponent_BP) (Variables|Default|GetHoverComponent_BP1))
    (Variables|/Game/Reign_Assets/EnemyObjects/Flying_Enemy/HoverComponent_BP.HoverComponent_BP_C|SetI%20Can%20Hover? _array_element false))
  (Physics|SetSimulatePhysics (Variables|Default|GetCapsuleComponent) false)
  (Components|Movement|StopMovementImmediately (Variables|Character|GetCharacterMovement))
  (Variables|Default|SetPlayerLastLoc (Transformation|GetWorldLocation (Variables|/Script/Engine.Character|GetCapsuleComponent _playerref)))
  (Variables|/Script/Engine.CharacterMovementComponent|SetGravityScale (Variables|/Script/Engine.Character|GetCharacterMovement _playerref) 0.0)
  (bind _newtrack_0 (Timeline|PlayerToEnemyTimeline PlayFromStart)
    (:Update
      (Transformation|SetWorldLocation (Variables|/Script/Engine.Character|GetCapsuleComponent (Variables|Default|GetPlayerRef)) (Math|Vector|Lerp(Vector) (Variables|Default|GetPlayerLastLoc) (+ (Transformation|GetWorldLocation (Variables|Default|GetCapsuleComponent)) "0, 0,25.000000") _newtrack_0) false false))
    (:Finished
      (|SetLastVec&KnockBack_2
        (:ex
          (Default|WeaponReset (Variables|/Game/Reign_Assets/Player_Character/Blueprints/MC_Prototype_BP.MC_Prototype_BP_C|GetEquippedWeapon _playerref_2))
          (Variables|/Game/Reign_Assets/Player_Character/Blueprints/MC_Prototype_BP.MC_Prototype_BP_C|SetPlayingAnimation? _playerref_2 true)
          (Variables|/Script/Engine.CharacterMovementComponent|SetGravityScale (Variables|/Script/Engine.Character|GetCharacterMovement _playerref_3) 2.0)
          (Variables|/Game/Reign_Assets/Player_Character/Blueprints/MC_Prototype_BP.MC_Prototype_BP_C|SetPlayingAnimation? _playerref_3 false)
          (Utilities|FlowControl|RetriggerableDelay 0.6)
          (for _array_element_2 (Utilities|Array|MakeArray (Variables|Default|GetHoverComponent_BP2) (Variables|Default|GetHoverComponent_BP3) (Variables|Default|GetHoverComponent_BP) (Variables|Default|GetHoverComponent_BP1))
            (Variables|/Game/Reign_Assets/EnemyObjects/Flying_Enemy/HoverComponent_BP.HoverComponent_BP_C|SetI%20Can%20Hover? _array_element_2 true)
            (Physics|SetSimulatePhysics _capsulecomponent true)
            (if (Variables|Default|GetIWasGrappled?)
              (Physics|AddImpulse _capsulecomponent (Variables|Default|GetLastFV) "None" false)
              (Variables|Default|SetIWasGrappled? false)
              (else
                (Physics|AddImpulse _capsulecomponent (Variables|Default|GetLastFV) "None" false)))
            (Utilities|FlowControl|Delay 0.2)
            (Variables|Default|SetFlyingActive? true))
          (Physics|SetSimulatePhysics _capsulecomponent true)
          (if (Variables|Default|GetIWasGrappled?)
            (Physics|AddImpulse _capsulecomponent (Variables|Default|GetLastFV) "None" false)
            (Variables|Default|SetIWasGrappled? false)
            (else
              (Physics|AddImpulse _capsulecomponent (Variables|Default|GetLastFV) "None" false)))
          (Utilities|FlowControl|Delay 0.2)
          (Variables|Default|SetFlyingActive? true))))))

(event Custom|Check%20Distance
  (if (<= (|GetPlayerVectorLenght) (Variables|Default|GetAggroRange))
    (Utilities|FlowControl|DoOnce false
      (:Completed
        (Variables|Default|SetAgroed? true)))))

(event Custom|FollowPlayer
  ;[1 1 1] Follow Player
  (Transformation|SetWorldRotation (Variables|Default|GetCapsuleComponent) (Math|Rotator|MakeRotator 0.0 0.0 (.yaw (Math|Rotator|FindLookatRotation (Transformation|GetWorldLocation (Variables|Default|GetCapsuleComponent)) (Transformation|GetWorldLocation (Variables|/Script/Engine.Character|GetCapsuleComponent (Variables|Default|GetPlayerRef)))))) false false)
  (Physics|AddForce (Variables|Default|GetCapsuleComponent) (* (Math|Vector|GetForwardVector (Variables|Default|GetCapsuleComponent)) (Variables|Default|GetChaseSpeedDefault)) "None" false))

(event Custom|AttackPlayer
  ;[1 1 1] AttackPlayer
  (bind _returnvalue (Effects|SpawnEmitterAttached "/Game/Reign_Assets/EnemyObjects/Flying_Enemy/FlyingCharge_FX.FlyingCharge_FX" (Variables|Default|GetCone) "None"))
  (EventDispatchers|BindEventtoOnSystemFinished _returnvalue (delegate Custom|OnChargeComplete))
  (Utilities|Time|SetTimerbyEvent (delegate Custom|AttackPlayer) (Variables|Default|GetAttackTime) true))

(event Custom|FallOff%20Death
  ;[1 1 1] Falloff Check
  (if (<= (.z (Transformation|GetWorldLocation (Variables|Default|GetCapsuleComponent))) -4e+02)
    (CallFunction|DeathEvent)))

(event Custom|CheckForwalls
  (bind _capsulecomponent (Variables|Default|GetCapsuleComponent))
  (bind _returnvalue (Transformation|GetWorldLocation _capsulecomponent))
  (bind _returnvalue_2 (Collision|LineTraceForObjects _returnvalue (- _returnvalue (* (Math|Vector|GetForwardVector (Transformation|GetWorldRotation _capsulecomponent)) -2e+02)) (Utilities|Array|MakeArray "ObjectTypeQuery1") false (Utilities|Array|MakeArray self) "ForDuration" true "(R=1.000000,G=0.000000,B=0.000000,A=1.000000)" "(R=0.000000,G=1.000000,B=0.000000,A=1.000000)" 1.0))
  (if _returnvalue_2
    (for _array_element (Utilities|Array|MakeArray (Variables|Default|GetHoverComponent_BP2) (Variables|Default|GetHoverComponent_BP3) (Variables|Default|GetHoverComponent_BP) (Variables|Default|GetHoverComponent_BP1))
      (Variables|/Game/Reign_Assets/EnemyObjects/Flying_Enemy/HoverComponent_BP.HoverComponent_BP_C|SetHoverDistance _array_element (+ (Variables|/Game/Reign_Assets/EnemyObjects/Flying_Enemy/HoverComponent_BP.HoverComponent_BP_C|GetHoverDistance _array_element) 2.0)))
    (else
      (for _array_element_2 (Utilities|Array|MakeArray (Variables|Default|GetHoverComponent_BP2) (Variables|Default|GetHoverComponent_BP3) (Variables|Default|GetHoverComponent_BP) (Variables|Default|GetHoverComponent_BP1))
        (Variables|/Game/Reign_Assets/EnemyObjects/Flying_Enemy/HoverComponent_BP.HoverComponent_BP_C|SetHoverDistance _array_element_2 (Math|Interpolation|FInterpTo (Variables|/Game/Reign_Assets/EnemyObjects/Flying_Enemy/HoverComponent_BP.HoverComponent_BP_C|GetHoverDistance _array_element_2) 5e+02 0.01 5.0))))))

(event Custom|OnChargeComplete
  (params (PSystem :type Particle%20System%20Component%20Object%20Reference))
  (bind _cone (Variables|Default|GetCone))
  (bind _returnvalue (Transformation|GetWorldLocation _cone))
  ;[1 1 1] AttackPlayer
  (Variables|Default|SetPlayersLastLoc (Transformation|GetWorldLocation (Variables|/Script/Engine.Character|GetCapsuleComponent (Variables|Default|GetPlayerRef))))
  (Utilities|FlowControl|Delay 0.2)
  (bind (_outhit _returnvalue_2) (Collision|LineTraceForObjects (Transformation|GetWorldLocation (Variables|Default|GetCone)) (Variables|Default|GetPlayersLastLoc) (Utilities|Array|MakeArray "ObjectTypeQuery3") false (Utilities|Array|MakeArray self) "None"))
  (bind _returnvalue_3 (Effects|SpawnEmitteratLocation "/Game/Reign_Assets/EnemyObjects/Flying_Enemy/LazerAttack_FX.LazerAttack_FX" _returnvalue))
  (Class|ParticleSystemComponent|SetBeamSourcePoint _returnvalue_3 0 _returnvalue)
  (Class|ParticleSystemComponent|SetBeamEndPoint _returnvalue_3 0 (.TraceEnd (Collision|BreakHitResult _outhit)))
  (if _returnvalue_2
    (Default|DealingDamage (Variables|Default|GetPlayerRef) 20 0 "None"))
  (Variables|Default|SetAgroed? true))

(event EventBeginPlay
  (|CallParentFunction) ; This node is disabled and will not be called.\nDrag off pins to build functionality.
)

(event Collision|EventActorBeginOverlap
  (params (OtherActor :type Actor%20Object%20Reference)))

(event EventTick
  (params (DeltaSeconds :type Float%20%28single-precision%29))
  ;[1 1 1] Tick
  (|CallParentFunction DeltaSeconds)
  (CallFunction|FallOffDeath)
  (if (Variables|Default|GetFlyingActive?)
    (Pawn|Input|AddMovementInput (Math|Vector|GetForwardVector (Transformation|GetActorRotation)) 1.0 false)
    (if (Variables|Default|GetAgroed?)
      (CallFunction|FollowPlayer)
      (Utilities|FlowControl|DoOnce false
        (:Completed
          (CallFunction|AttackPlayer))))))

(event EventDealingDamage
  (params (Sent%20Damage :type Integer) (Sender :type Actor%20Object%20Reference) (DamageType :type Name :default "None"))
  (CallFunction|ShowHealthbar)
  (switch name DamageType
    (:Grapple
      (CallFunction|GrapplingEvent))
    (:PullTo
      (CallFunction|PulltoEvent))
    (:Melee
      (CallFunction|MeleeDamge))))

(fn ConstructionScript
  (|CallParentFunction))