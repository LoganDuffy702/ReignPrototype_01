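; Flying enemy that chases and shoots at the player once MC_Prototype_BP enters its aggro collision.
; While aggroed, Tick turns the capsule's yaw toward the player, pushes it forward with force and updates a distance check.
; A looping timer spawns Flying_Enemy_Projectile at the Firepoint when the player is close enough.
; Aggro persists after overlap ends because the de-aggro logic is disconnected; DealingDamage is an empty stub.
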(event OnComponentBeginOverlap(AggroCollision)
  (params (OverlappedComponent :type Primitive%20Component%20Object%20Reference) (OtherActor :type Actor%20Object%20Reference) (OtherComp :type Primitive%20Component%20Object%20Reference) (OtherBodyIndex :type Integer) (bFromSweep :type Boolean) (SweepResult :type Hit%20Result%20Structure%20%28by%20ref%29))
  (bind _asmc_prototype_bp (Utilities|Casting|CastToMC_Prototype_BP OtherActor))
  (Variables|Default|SetPlayerRef _asmc_prototype_bp)
  (Variables|Default|SetAgroed? true)
  (CallFunction|CheckAttackLength)
  (CallFunction|FireatPlayer))

(event OnComponentEndOverlap(AggroCollision)
  (params (OverlappedComponent :type Primitive%20Component%20Object%20Reference) (OtherActor :type Actor%20Object%20Reference) (OtherComp :type Primitive%20Component%20Object%20Reference) (OtherBodyIndex :type Integer)))

(event Custom|Follow%20Player
  (bind _returnvalue (Transformation|GetActorRotation))
  (bind _capsule (Variables|Default|GetCapsule))
  (Transformation|SetWorldRotation (Variables|Default|GetCapsule) (Math|Rotator|MakeRotator (.roll _returnvalue) (.pitch _returnvalue) (.Yaw (Math|Rotator|BreakRotator (Math|Rotator|FindLookatRotation (Transformation|GetActorLocation) (Transformation|GetActorLocation (Variables|Default|GetPlayerRef)))))) false false)
  (Physics|AddForce _capsule (* (Math|Vector|GetForwardVector _capsule) 9e+05) "None" false))

(event Custom|FireAtPlayer
  (bind _firepoint (Variables|Default|GetFirepoint))
  (bind _returnvalue (Transformation|GetWorldTransform _firepoint))
  (if (Variables|Default|GetCloseEnough?)
    (Game|SpawnActorfromClass "/Game/Reign_Assets/EnemyObjects/Flying_Enemy/Flying_Enemy_Projectile.Flying_Enemy_Projectile_C" (Math|Transform|MakeTransform (.location _returnvalue) (.rotation _returnvalue) "1.250000,0.500000,0.500000") "Undefined" 0 0)
    (Utilities|Time|SetTimerbyFunctionName 0 "FireAtPlayer" 0.5 true)
    (else
      (Utilities|Time|SetTimerbyFunctionName 0 "FireAtPlayer" 0.5 true))))

(event Custom|CheckAttackLength
  (Variables|Default|SetCloseEnough? (<= (Math|Vector|VectorLength (- (Transformation|GetActorLocation (Variables|Default|GetPlayerRef)) (Transformation|GetActorLocation))) 1e+03)))

(event EventTick
  (params (DeltaSeconds :type Float%20%28single-precision%29))
  (if (Variables|Default|GetAgroed?)
    (CallFunction|FollowPlayer)
    (CallFunction|CheckAttackLength)))

(event EventDealingDamage
  (params (Sent%20Damage :type Integer) (Sender :type Actor%20Object%20Reference) (DamageType :type Name :default "None")))

(fn ConstructionScript)