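; Grapple target actor that, when its DealingDamage event fires, launches the player character along the forward vector of their grapple origin.
; It zeroes the player's gravity and velocity, then applies a one-shot launch that differs when airborne.
; After a short delay or on ChokePoint overlap, it resets the weapon, movement rotation and gravity, with overlap also damping airborne velocity.
; An interpolated pull toward ChokePoint remains in disconnected nodes.
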(event OnComponentBeginOverlap(ChokePoint)
  (params (OverlappedComponent :type Primitive%20Component%20Object%20Reference) (OtherActor :type Actor%20Object%20Reference) (OtherComp :type Primitive%20Component%20Object%20Reference) (OtherBodyIndex :type Integer) (bFromSweep :type Boolean) (SweepResult :type Hit%20Result%20Structure%20%28by%20ref%29))
  (bind _asmc_prototype_bp (Utilities|Casting|CastToMC_Prototype_BP OtherActor))
  (Variables|Default|SetActiveGrapple? false)
  (CallFunction|StopPullEvent)
  (if (AI|Components|NavMovement|IsFalling (Variables|/Script/Engine.Character|GetCharacterMovement _asmc_prototype_bp))
    (Variables|/Script/Engine.MovementComponent|SetVelocity (Variables|/Script/Engine.Character|GetCharacterMovement _asmc_prototype_bp) (* (Variables|/Script/Engine.MovementComponent|GetVelocity (Variables|/Script/Engine.Character|GetCharacterMovement _asmc_prototype_bp)) 0.7))))

(event EventBeginPlay
  (|CallParentFunction) ; This node is disabled and will not be called.\nDrag off pins to build functionality.
)

(event Collision|EventActorBeginOverlap
  (params (OtherActor :type Actor%20Object%20Reference)))

(event EventDealingDamage
  (params (Sent%20Damage :type Integer) (Sender :type Actor%20Object%20Reference) (DamageType :type Name :default "None"))
  (bind _asmc_prototype_bp (Utilities|Casting|CastToMC_Prototype_BP (Game|GetPlayerCharacter 0)))
  (bind _output_get (Variables|Default|SetPlayerRef _asmc_prototype_bp))
  (Variables|/Script/Engine.CharacterMovementComponent|SetGravityScale (Variables|/Script/Engine.Character|GetCharacterMovement _output_get) 0.0)
  (Variables|/Script/Engine.MovementComponent|SetVelocity (Variables|/Script/Engine.Character|GetCharacterMovement _output_get) "0, 0, 0")
  (CallFunction|PullEvent))

(event EventPullEvent
  (bind _playerref (Variables|Default|GetPlayerRef))
  (bind _playerref_2 (Variables|Default|GetPlayerRef))
  (bind _playergrappleorigin (Variables|/Game/Reign_Assets/Player_Character/Blueprints/MC_Prototype_BP.MC_Prototype_BP_C|GetPlayerGrappleOrigin _playerref_2))
  (bind _returnvalue (Math|Vector|GetForwardVector _playergrappleorigin))
  (Utilities|FlowControl|DoOnce false
    (:Completed
      (if (AI|Components|NavMovement|IsFalling (Variables|/Script/Engine.Character|GetCharacterMovement (Variables|Default|GetPlayerRef)))
        (Character|LaunchCharacter (Variables|Default|GetPlayerRef) (* (Math|Vector|MakeVector (.x _returnvalue) (.y _returnvalue) (* (.z _returnvalue) 2.0)) 7e+03) false false)
        (Variables|Default|SetActiveGrapple? true)
        (else
          (Character|LaunchCharacter _playerref (* (Math|Vector|GetForwardVector (Variables|/Game/Reign_Assets/Player_Character/Blueprints/MC_Prototype_BP.MC_Prototype_BP_C|GetPlayerGrappleOrigin _playerref)) 1e+04) false false)
          (Variables|Default|SetActiveGrapple? true)))
      (Utilities|FlowControl|Delay 0.5)
      (CallFunction|StopPullEvent))))

(event EventStopPullEvent
  (bind _playerref (Variables|Default|GetPlayerRef))
  (bind _playerref_2 (Variables|Default|GetPlayerRef))
  (bind _playerref_3 (Variables|Default|GetPlayerRef))
  (bind _playergrappleorigin (Variables|/Game/Reign_Assets/Player_Character/Blueprints/MC_Prototype_BP.MC_Prototype_BP_C|GetPlayerGrappleOrigin _playerref_3))
  (bind _charactermovement (Variables|/Script/Engine.Character|GetCharacterMovement _playerref_2))
  (bind _returnvalue (Math|Vector|GetForwardVector _playergrappleorigin))
  (Variables|Default|SetActiveGrapple? false)
  (Default|WeaponReset (Variables|/Game/Reign_Assets/Player_Character/Blueprints/MC_Prototype_BP.MC_Prototype_BP_C|GetEquippedWeapon _playerref_2))
  (Variables|/Script/Engine.CharacterMovementComponent|SetbOrientRotationToMovement _charactermovement true)
  (Variables|/Script/Engine.CharacterMovementComponent|SetbUseControllerDesiredRotation _charactermovement false)
  (Variables|/Script/Engine.CharacterMovementComponent|SetGravityScale _charactermovement 2.0)
  (Utilities|FlowControl|DoOnce false) ; enters at Reset
)

(fn ConstructionScript
  (|CallParentFunction))