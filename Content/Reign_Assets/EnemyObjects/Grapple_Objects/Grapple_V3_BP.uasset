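; Grapple target object that responds to the player's grapple and pull hits, with its type setting its behavior and, for Grapple and Launch, its material.
; DealingDamage halts the player and calls PullEvent, which either lerps the player to the object by timeline with gravity off or launches them at a fixed pitch.
; Pull-to hits drag the object toward the player unless it is non-moving; StopCollision overlaps reset the equipped weapon.
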(event OnComponentBeginOverlap(StopCollision)
  (params (OverlappedComponent :type Primitive%20Component%20Object%20Reference) (OtherActor :type Actor%20Object%20Reference) (OtherComp :type Primitive%20Component%20Object%20Reference) (OtherBodyIndex :type Integer) (bFromSweep :type Boolean) (SweepResult :type Hit%20Result%20Structure%20%28by%20ref%29))
  (if (not (== OtherActor "/Game/Reign_Assets/EnemyObjects/Flying_Enemy/Flying_Enemy_1_BP.Flying_Enemy_1_BP"))
    (Default|WeaponReset (Variables|/Game/Reign_Assets/Player_Character/Blueprints/MC_Prototype_BP.MC_Prototype_BP_C|GetEquippedWeapon (Variables|Default|GetPlayerRef)))
    (Development|PrintString "Not Possible")))

(event EventBeginPlay
  (|CallParentFunction)
  (switch Utilities|FlowControl|Switch|SwitchonGrappleType (Variables|Default|GetGrappleType)
    (:NewEnumerator0
      (Rendering|Material|SetMaterial (Variables|Default|Getstaticmesh) 0 "/Game/Reign_Assets/EnemyObjects/Grapple_Objects/Basic_Grapple_Mat.Basic_Grapple_Mat"))
    (:NewEnumerator1
      (Rendering|Material|SetMaterial (Variables|Default|Getstaticmesh) 0 "/Game/Reign_Assets/EnemyObjects/Grapple_Objects/Launch_Grapple_Mat.Launch_Grapple_Mat"))))

(event Collision|EventActorBeginOverlap
  (params (OtherActor :type Actor%20Object%20Reference)))

(event EventTick
  (params (DeltaSeconds :type Float%20%28single-precision%29))
  (|CallParentFunction DeltaSeconds))

(event EventDealingDamage
  (params (Sent%20Damage :type Integer) (Sender :type Actor%20Object%20Reference) (DamageType :type Name :default "None"))
  (Variables|Default|SetDmg%20Type DamageType)
  (if (or (Utilities|Name|Equal(Name) DamageType "Grapple") (Utilities|Name|Equal(Name) DamageType "PullTo"))
    (Utilities|FlowControl|Delay 0.15)
    (Variables|/Script/Engine.MovementComponent|SetVelocity (Variables|/Script/Engine.Character|GetCharacterMovement (Variables|Default|GetPlayerRef)) "0, 0, 0")
    (CallFunction|PullEvent)))

(event EventPullEvent
  (bind _returnvalue (Transformation|GetActorLocation))
  (bind _playerref (Variables|Default|GetPlayerRef))
  (bind _playerref_2 (Variables|Default|GetPlayerRef))
  (bind _playerref_3 (Variables|Default|GetPlayerRef))
  (bind _playerref_4 (Variables|Default|GetPlayerRef))
  (bind _playerref_5 (Variables|Default|GetPlayerRef))
  (bind _aoe_point (Variables|/Game/Reign_Assets/Player_Character/Blueprints/MC_Prototype_BP.MC_Prototype_BP_C|GetAoE%20Point _playerref_2))
  (bind _capsulecomponent (Variables|/Script/Engine.Character|GetCapsuleComponent _playerref_5))
  (bind _returnvalue_2 (Transformation|GetWorldLocation _aoe_point))
  (bind _returnvalue_3 (Transformation|GetWorldLocation _capsulecomponent))
  (bind _returnvalue_4 (Math|Rotator|FindLookatRotation _returnvalue_3 _returnvalue))
  (switch name (Variables|Default|GetDmg%20Type)
    (:Grapple
      (switch Utilities|FlowControl|Switch|SwitchonGrappleType (Variables|Default|GetGrappleType)
        (:NewEnumerator0
          (Variables|Default|SetPlayerLastLoc (Transformation|GetActorLocation _playerref_3) :!label _label)
          (Variables|/Script/Engine.CharacterMovementComponent|SetGravityScale (Variables|/Script/Engine.Character|GetCharacterMovement _playerref_3) 0.0)
          (bind _newtrack_0 (Timeline|GroundGrapple_TL PlayFromStart)
            (:Update
              (Transformation|SetActorLocation (Variables|Default|GetPlayerRef) (Math|Vector|Lerp(Vector) (Variables|Default|GetPlayerLastLoc) (+ (Transformation|GetWorldLocation (Variables|Default|GetCapsuleComponent)) "0, 0,100.000000") _newtrack_0) false false))
            (:Finished
              (if (Variables|Default|GetGroundBased?)
                (Default|WeaponReset (Variables|/Game/Reign_Assets/Player_Character/Blueprints/MC_Prototype_BP.MC_Prototype_BP_C|GetEquippedWeapon (Variables|Default|GetPlayerRef)))
                (Variables|/Script/Engine.CharacterMovementComponent|SetGravityScale (Variables|/Script/Engine.Character|GetCharacterMovement (Variables|Default|GetPlayerRef)) 2.0)
                (else
                  (Default|WeaponReset (Variables|/Game/Reign_Assets/Player_Character/Blueprints/MC_Prototype_BP.MC_Prototype_BP_C|GetEquippedWeapon _playerref))
                  (Variables|/Game/Reign_Assets/Player_Character/Blueprints/MC_Prototype_BP.MC_Prototype_BP_C|SetPlayingAnimation? _playerref true)
                  (if (Variables|/Game/Reign_Assets/Player_Character/Blueprints/MC_Prototype_BP.MC_Prototype_BP_C|GetCannot%20Attack (Variables|Default|GetPlayerRef))
                    (Development|PrintString "Attacking")
                    (else
                      (Variables|/Script/Engine.CharacterMovementComponent|SetGravityScale (Variables|/Script/Engine.Character|GetCharacterMovement _playerref_4) 2.0)
                      (Variables|/Game/Reign_Assets/Player_Character/Blueprints/MC_Prototype_BP.MC_Prototype_BP_C|SetPlayingAnimation? _playerref_4 false))))))))
        (:NewEnumerator1
          ;[1 1 1] Launch Mode
          (Transformation|SetWorldRotation (Variables|/Game/Reign_Assets/Player_Character/Blueprints/MC_Prototype_BP.MC_Prototype_BP_C|GetPlayerGrappleOrigin (Variables|Default|GetPlayerRef)) (Math|Rotator|MakeRotator (.roll _returnvalue_4) 5e+01 (.yaw _returnvalue_4)) false false)
          (Character|LaunchCharacter (Variables|Default|GetPlayerRef) (* (Math|Vector|GetForwardVector (Variables|/Game/Reign_Assets/Player_Character/Blueprints/MC_Prototype_BP.MC_Prototype_BP_C|GetPlayerGrappleOrigin (Variables|Default|GetPlayerRef))) (Variables|Default|GetAirGrapplePower)) false false)
          (Utilities|FlowControl|Delay 0.2)
          (Default|WeaponReset (Variables|/Game/Reign_Assets/Player_Character/Blueprints/MC_Prototype_BP.MC_Prototype_BP_C|GetEquippedWeapon (Variables|Default|GetPlayerRef))))
        (:NewEnumerator2
          (goto _label))))
    (:PullTo
      (if (Utilities|Enum|Equal(Enum) (Variables|Default|GetGrappleType) "NewEnumerator2")
        (goto _label)
        (else
          (Variables|Default|SetActorLastLoc (Transformation|GetWorldLocation (Variables|Default|GetCapsuleComponent)))
          (bind _newtrack_0_2 (Timeline|PullTimeline PlayFromStart)
            (:Update
              (Class|ParticleSystemComponent|SetBeamEndPoint (Variables|/Game/Reign_Assets/Weapon_BP/Master_Weapon_BP.Master_Weapon_BP_C|GetChainParticle (Variables|/Game/Reign_Assets/Player_Character/Blueprints/MC_Prototype_BP.MC_Prototype_BP_C|GetEquippedWeapon (Variables|Default|GetPlayerRef))) 0 (Transformation|GetWorldLocation (Variables|Default|GetChokePoint)))
              (Transformation|SetWorldLocation (Variables|Default|GetCapsuleComponent) (Math|Vector|Lerp(Vector) (Math|Vector|MakeVector (.x (Variables|Default|GetActorLastLoc)) (.y (Variables|Default|GetActorLastLoc)) (.z (Variables|Default|GetActorLastLoc))) (Math|Vector|MakeVector (.x _returnvalue_2) (.y _returnvalue_2) (.z (Variables|Default|GetActorLastLoc))) _newtrack_0_2) false false))
            (:Finished
              (Default|WeaponReset (Variables|/Game/Reign_Assets/Player_Character/Blueprints/MC_Prototype_BP.MC_Prototype_BP_C|GetEquippedWeapon (Variables|Default|GetPlayerRef))))))))))

(fn ConstructionScript
  (|CallParentFunction))