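; Pullable grapple object that slides toward the player when hit by Grapple or "Pull to" damage, unless OnButton is set.
; A timeline lerps the capsule horizontally toward a point two-thirds of the way to the player, keeping its height and stopping within StopRange.
; OnButtonStop halts the pull, and the DisableCol overlap volume switches the capsule's collision object channel on enter and exit.
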(event OnComponentBeginOverlap(DisableCol)
  (params (OverlappedComponent :type Primitive%20Component%20Object%20Reference) (OtherActor :type Actor%20Object%20Reference) (OtherComp :type Primitive%20Component%20Object%20Reference) (OtherBodyIndex :type Integer) (bFromSweep :type Boolean) (SweepResult :type Hit%20Result%20Structure%20%28by%20ref%29))
  (Collision|SetCollisionObjectType (Variables|Default|GetCapsule) "ECC_GameTraceChannel8"))

(event OnComponentEndOverlap(DisableCol)
  (params (OverlappedComponent :type Primitive%20Component%20Object%20Reference) (OtherActor :type Actor%20Object%20Reference) (OtherComp :type Primitive%20Component%20Object%20Reference) (OtherBodyIndex :type Integer))
  (Collision|SetCollisionObjectType (Variables|Default|GetCapsule) "ECC_GameTraceChannel1"))

(event Custom|On%20Button%20Stop
  (bind _lastloc (Variables|Default|GetLastLoc))
  (bind _playerref (Variables|Default|GetPlayerRef))
  (bind _returnvalue (Math|Vector|MakeVector (.x _lastloc) (.y _lastloc) (.z _lastloc)))
  (bind _capsulecomponent (Variables|/Script/Engine.Character|GetCapsuleComponent _playerref))
  (bind _returnvalue_2 (Transformation|GetWorldLocation _capsulecomponent))
  (bind _newtrack_0 (Timeline|PullToTimeline Stop)
    (:Update
      (if (<= (Math|Vector|VectorLength (- (Transformation|GetWorldLocation (Variables|Default|GetCapsule)) (Transformation|GetWorldLocation (Variables|/Script/Engine.Character|GetCapsuleComponent (Variables|Default|GetPlayerRef))))) (Variables|Default|GetStopRange))
        (Timeline|PullToTimeline Stop)
        (else
          (Transformation|SetWorldLocation (Variables|Default|GetCapsule) (Math|Vector|Lerp(Vector) _returnvalue (+ (* (Math|Vector|MakeVector (.x _returnvalue_2) (.y _returnvalue_2) (.z _lastloc)) (/ 2.0 3.0)) (* _returnvalue (/ 1.0 3.0))) _newtrack_0) false false))))))

(event EventBeginPlay
  (bind _asmc_prototype_bp (Utilities|Casting|CastToMC_Prototype_BP (Game|GetPlayerCharacter 0)))
  (Variables|Default|SetPlayerRef _asmc_prototype_bp))

(event EventDealingDamage
  (params (Sent%20Damage :type Integer) (Sender :type Actor%20Object%20Reference) (DamageType :type Name :default "None"))
  (bind _playerref (Variables|Default|GetPlayerRef))
  (bind _capsulecomponent (Variables|/Script/Engine.Character|GetCapsuleComponent _playerref))
  (bind _returnvalue (Transformation|GetWorldLocation _capsulecomponent))
  (if (not (Variables|Default|GetOnButton?))
    (switch name DamageType
      (:Grapple
        _)
      (:PullTo
        _))
    (Variables|Default|SetLastLoc (Transformation|GetWorldLocation (Variables|Default|GetCapsule)))
    (bind _newtrack_0 (Timeline|PullToTimeline PlayFromStart)
      (:Update
        (if (<= (Math|Vector|VectorLength (- (Transformation|GetWorldLocation (Variables|Default|GetCapsule)) (Transformation|GetWorldLocation (Variables|/Script/Engine.Character|GetCapsuleComponent (Variables|Default|GetPlayerRef))))) (Variables|Default|GetStopRange))
          (Timeline|PullToTimeline Stop)
          (else
            (Transformation|SetWorldLocation (Variables|Default|GetCapsule) (Math|Vector|Lerp(Vector) (Math|Vector|MakeVector (.x (Variables|Default|GetLastLoc)) (.y (Variables|Default|GetLastLoc)) (.z (Variables|Default|GetLastLoc))) (+ (* (Math|Vector|MakeVector (.x _returnvalue) (.y _returnvalue) (.z (Variables|Default|GetLastLoc))) (/ 2.0 3.0)) (* (Math|Vector|MakeVector (.x (Variables|Default|GetLastLoc)) (.y (Variables|Default|GetLastLoc)) (.z (Variables|Default|GetLastLoc))) (/ 1.0 3.0))) _newtrack_0) false false)))))))

(fn ConstructionScript)