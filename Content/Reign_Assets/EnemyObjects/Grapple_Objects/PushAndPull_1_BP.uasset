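; Grapple object that gets pulled toward the player when it receives Grapple or Pull to damage.
; A timeline lerps it from its saved location to two-thirds of the way to the player's current position, keeping its height, and pins the weapon's chain beam to its ChokePoint.
; Mesh hits or StopTimeline halt the pull.
; Box overlaps toggle the capsule's collision object channel.
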(event OnComponentBeginOverlap(Box)
  (params (OverlappedComponent :type Primitive%20Component%20Object%20Reference) (OtherActor :type Actor%20Object%20Reference) (OtherComp :type Primitive%20Component%20Object%20Reference) (OtherBodyIndex :type Integer) (bFromSweep :type Boolean) (SweepResult :type Hit%20Result%20Structure%20%28by%20ref%29))
  (Collision|SetCollisionObjectType (Variables|Default|GetCapsuleComponent) "ECC_GameTraceChannel8"))

(event OnComponentEndOverlap(Box)
  (params (OverlappedComponent :type Primitive%20Component%20Object%20Reference) (OtherActor :type Actor%20Object%20Reference) (OtherComp :type Primitive%20Component%20Object%20Reference) (OtherBodyIndex :type Integer))
  (Collision|SetCollisionObjectType (Variables|Default|GetCapsuleComponent) "ECC_GameTraceChannel1"))

(event OnComponentHit(VisualMesh)
  (params (HitComponent :type Primitive%20Component%20Object%20Reference) (OtherActor :type Actor%20Object%20Reference) (OtherComp :type Primitive%20Component%20Object%20Reference) (NormalImpulse :type Vector :default "0, 0, 0") (Hit :type Hit%20Result%20Structure%20%28by%20ref%29))
  (bind _lastloc (Variables|Default|GetLastLoc))
  (bind _playerref (Variables|Default|GetPlayerRef))
  (bind _returnvalue (Math|Vector|MakeVector (.x _lastloc) (.y _lastloc) (.z _lastloc)))
  (bind _capsulecomponent (Variables|/Script/Engine.Character|GetCapsuleComponent _playerref))
  (bind _returnvalue_2 (Transformation|GetWorldLocation _capsulecomponent))
  (bind _newtrack_0 (Timeline|Timeline_0 Stop)
    (:Update
      (Class|ParticleSystemComponent|SetBeamEndPoint (Variables|/Game/Reign_Assets/Weapon_BP/Master_Weapon_BP.Master_Weapon_BP_C|GetChainParticle (Variables|/Game/Reign_Assets/Player_Character/Blueprints/MC_Prototype_BP.MC_Prototype_BP_C|GetEquippedWeapon (Variables|Default|GetPlayerRef))) 0 (Transformation|GetWorldLocation (Variables|Default|GetChokePoint)))
      (Transformation|SetActorLocation (Math|Vector|Lerp(Vector) _returnvalue (+ (* (Math|Vector|MakeVector (.x _returnvalue_2) (.y _returnvalue_2) (.z _lastloc)) (/ 2.0 3.0)) (* _returnvalue (/ 1.0 3.0))) _newtrack_0) false false))))

(event Custom|StopTimeline
  (bind _lastloc (Variables|Default|GetLastLoc))
  (bind _playerref (Variables|Default|GetPlayerRef))
  (bind _returnvalue (Math|Vector|MakeVector (.x _lastloc) (.y _lastloc) (.z _lastloc)))
  (bind _capsulecomponent (Variables|/Script/Engine.Character|GetCapsuleComponent _playerref))
  (bind _returnvalue_2 (Transformation|GetWorldLocation _capsulecomponent))
  (bind _newtrack_0 (Timeline|Timeline_0 Stop)
    (:Update
      (Class|ParticleSystemComponent|SetBeamEndPoint (Variables|/Game/Reign_Assets/Weapon_BP/Master_Weapon_BP.Master_Weapon_BP_C|GetChainParticle (Variables|/Game/Reign_Assets/Player_Character/Blueprints/MC_Prototype_BP.MC_Prototype_BP_C|GetEquippedWeapon (Variables|Default|GetPlayerRef))) 0 (Transformation|GetWorldLocation (Variables|Default|GetChokePoint)))
      (Transformation|SetActorLocation (Math|Vector|Lerp(Vector) _returnvalue (+ (* (Math|Vector|MakeVector (.x _returnvalue_2) (.y _returnvalue_2) (.z _lastloc)) (/ 2.0 3.0)) (* _returnvalue (/ 1.0 3.0))) _newtrack_0) false false))))

(event Custom|CheckForPull)

(event EventBeginPlay
  (|CallParentFunction) ; This node is disabled and will not be called.\nDrag off pins to build functionality.
)

(event Collision|EventActorBeginOverlap
  (params (OtherActor :type Actor%20Object%20Reference)))

(event EventTick
  (params (DeltaSeconds :type Float%20%28single-precision%29))
  (|CallParentFunction DeltaSeconds) ; This node is disabled and will not be called.\nDrag off pins to build functionality.
)

(event EventDealingDamage
  (params (Sent%20Damage :type Integer) (Sender :type Actor%20Object%20Reference) (DamageType :type Name :default "None"))
  (bind _playerref (Variables|Default|GetPlayerRef))
  (bind _capsulecomponent (Variables|/Script/Engine.Character|GetCapsuleComponent _playerref))
  (bind _returnvalue (Transformation|GetWorldLocation _capsulecomponent))
  (switch name DamageType
    (:Grapple
      _)
    (:PullTo
      _))
  (Variables|Default|SetLastLoc (Transformation|GetActorLocation))
  (bind _newtrack_0 (Timeline|Timeline_0 PlayFromStart)
    (:Update
      (Class|ParticleSystemComponent|SetBeamEndPoint (Variables|/Game/Reign_Assets/Weapon_BP/Master_Weapon_BP.Master_Weapon_BP_C|GetChainParticle (Variables|/Game/Reign_Assets/Player_Character/Blueprints/MC_Prototype_BP.MC_Prototype_BP_C|GetEquippedWeapon (Variables|Default|GetPlayerRef))) 0 (Transformation|GetWorldLocation (Variables|Default|GetChokePoint)))
      (Transformation|SetActorLocation (Math|Vector|Lerp(Vector) (Math|Vector|MakeVector (.x (Variables|Default|GetLastLoc)) (.y (Variables|Default|GetLastLoc)) (.z (Variables|Default|GetLastLoc))) (+ (* (Math|Vector|MakeVector (.x _returnvalue) (.y _returnvalue) (.z (Variables|Default|GetLastLoc))) (/ 2.0 3.0)) (* (Math|Vector|MakeVector (.x (Variables|Default|GetLastLoc)) (.y (Variables|Default|GetLastLoc)) (.z (Variables|Default|GetLastLoc))) (/ 1.0 3.0))) _newtrack_0) false false))))

(fn ConstructionScript
  (|CallParentFunction))