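; Heavy melee enemy that roams at random, steering back toward its start point when too far, and chases the player once alerted.
; Sight or aggro overlap plays a shocked montage, then Tick steers toward the player with direct movement input, without navigation.
; Timed capsule traces trigger the attack montage, with a separate sphere-trace damage event.
; Body contact damages and knocks back the player; taking damage briefly shows a health bar.
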(event OnComponentEndOverlap(Agro)
  (params (OverlappedComponent :type Primitive%20Component%20Object%20Reference) (OtherActor :type Actor%20Object%20Reference) (OtherComp :type Primitive%20Component%20Object%20Reference) (OtherBodyIndex :type Integer))
  ;[1 1 1] (AI)
)

(event OnComponentBeginOverlap(Agro)
  (params (OverlappedComponent :type Primitive%20Component%20Object%20Reference) (OtherActor :type Actor%20Object%20Reference) (OtherComp :type Primitive%20Component%20Object%20Reference) (OtherBodyIndex :type Integer) (bFromSweep :type Boolean) (SweepResult :type Hit%20Result%20Structure%20%28by%20ref%29))
  ;[1 1 1] (AI)
  (Class|KismetSystemLibrary|UnPauseTimer 0 "ResetRoam")
  (Utilities|FlowControl|DoOnce false
    (:Completed
      (|AgroSolverNode))))

(event OnSeePawn(PawnSensing)
  (params (Pawn :type Pawn%20Object%20Reference))
  ;[1 1 1] (AI)
  (Class|KismetSystemLibrary|UnPauseTimer 0 "ResetRoam")
  (Utilities|FlowControl|DoOnce false
    (:Completed
      (|AgroSolverNode))))

(event OnComponentHit(CapsuleComponent)
  (params (HitComponent :type Primitive%20Component%20Object%20Reference) (OtherActor :type Actor%20Object%20Reference) (OtherComp :type Primitive%20Component%20Object%20Reference) (NormalImpulse :type Vector :default "0, 0, 0") (Hit :type Hit%20Result%20Structure%20%28by%20ref%29))
  (bind _playerref (Variables|Default|GetPlayerRef))
  (if (== OtherActor (Variables|Default|GetPlayerRef))
    (Default|DealingDamage (Variables|Default|GetPlayerRef) 1 0 "None")
    (Utilities|FlowControl|DoOnce false
      (:Completed
        (Variables|/Script/Engine.MovementComponent|SetVelocity (Variables|/Script/Engine.Character|GetCharacterMovement _playerref) "0, 0, 0")
        (Character|LaunchCharacter _playerref (* (* (Math|Vector|GetForwardVector (Variables|/Script/Engine.Character|GetCapsuleComponent _playerref)) -2e+03) "1.000000,1.000000,1.200000") false false)
        (Utilities|Time|SetTimerbyFunctionName 0 "Reset Player Knockback" 0.2)))))

(event Custom|Reset%20Attack
  ;[1 1 1] (AI)
  (Utilities|FlowControl|Delay 1.0)
  (Variables|Default|SetChasePlayer? true)
  (Variables|Default|SetActiveMovement? true)
  (Utilities|Time|SetTimerbyFunctionName 0 "CheckForPlayer" 1.5))

(event Custom|CheckForPlayer
  ;[1 1 1] (AI)
  (|CheckForPlayerNode))

(event Custom|CheckforOthers
  (bind _capsulecomponent (Variables|Collision|GetCapsuleComponent))
  (bind _returnvalue (Transformation|GetWorldLocation _capsulecomponent))
  (bind _returnvalue_2 (Collision|CapsuleTraceByChannel _returnvalue _returnvalue 3e+02 5e+02 "TraceTypeQuery3" false 0 "ForDuration" true "(R=0.000000,G=1.000000,B=0.917567,A=1.000000)" "(R=1.000000,G=0.000000,B=0.790900,A=1.000000)" 1.0))
  (if _returnvalue_2
    (Variables|Default|SetBumped? true)
    (else
      (Utilities|Time|SetTimerbyFunctionName 0 "CheckforOthers" 0.5 true))))

(event Custom|Roam
  ;[1 1 1] (AI)
  (CallFunction|FindNewLoc)
  (Utilities|Time|SetTimerbyEvent (delegate Custom|Roam) 3.0 true))

(event Custom|ResetRoam
  ;[1 1 1] (AI)
  (Variables|Default|SetChasePlayer? false)
  (CallFunction|Roam)
  (Variables|/Script/Engine.CharacterMovementComponent|SetMaxWalkSpeed (Variables|Character|GetCharacterMovement) 3e+02)
  (Utilities|FlowControl|DoOnce false) ; enters at Reset
)

(event Custom|To%20Far%20Event
  ;[1 1 1] (AI)
  (CallFunction|CheckiftoFar)
  (Utilities|Time|SetTimerbyEvent (delegate Custom|To%20Far%20Event) 1.0 true))

(event Custom|AttackTrace%20Event
  (bind _capsulecomponent (Variables|Collision|GetCapsuleComponent))
  (bind _returnvalue (Transformation|GetWorldLocation _capsulecomponent))
  (bind _returnvalue_2 (Math|Vector|GetForwardVector _capsulecomponent))
  (bind _returnvalue_3 (* _returnvalue_2 4e+02))
  (bind _returnvalue_4 (+ _returnvalue _returnvalue_3))
  (bind _returnvalue_5 (- _returnvalue_4 "0, 0,300.000000"))
  (bind _returnvalue_6 (Collision|SphereTraceForObjects _returnvalue_5 _returnvalue_5 6e+02 (Utilities|Array|MakeArray "ObjectTypeQuery3") false 0 "ForDuration" true "(R=1.000000,G=0.000000,B=0.000000,A=1.000000)" "(R=0.000000,G=1.000000,B=0.000000,A=1.000000)" 2.0))
  (if _returnvalue_6
    (Default|DealingDamage (Variables|Default|GetPlayerRef) 3 0 "None")))

(event Custom|Reset%20Player%20Knockback
  (bind _playerref (Variables|Default|GetPlayerRef))
  (Utilities|FlowControl|DoOnce false) ; enters at Reset
)

(event EventBeginPlay
  ;[1 1 1] On Begin
  (bind _asmc_prototype_bp (Utilities|Casting|CastToMC_Prototype_BP (Game|GetPlayerCharacter 0)))
  (Variables|Default|SetPlayerRef _asmc_prototype_bp)
  (Rendering|SetVisibility (Variables|Default|GetHP_Widget) false false)
  (CallFunction|InitStartingPoint)
  (CallFunction|Roam)
  (Variables|/Script/Engine.CharacterMovementComponent|SetMaxWalkSpeed (Variables|Character|GetCharacterMovement) 3e+02)
  (CallFunction|ToFarEvent))

(event EventDealingDamage
  (params (Sent%20Damage :type Integer) (Sender :type Actor%20Object%20Reference) (DamageType :type Name :default "None"))
  ;[1 1 1] Damage Solving
  (CallFunction|PlayImpactSound)
  (Variables|Default|SetCurrentHealth (- (Variables|Default|GetCurrentHealth) 5.0))
  (CallFunction|UpdateHealth)
  (Utilities|FlowControl|RetriggerableDelay 2.0)
  (CallFunction|HideHP))

(event EventTick
  (params (DeltaSeconds :type Float%20%28single-precision%29))
  ;[1 1 1] Tick
  (if (Variables|Default|GetActiveMovement?)
    (if (Variables|Default|GetChasePlayer?)
      (CallFunction|MovementFuntion)
      (Pawn|Input|AddMovementInput (Variables|Default|GetDirectionVector) 1.0 false)
      (else
        (Pawn|Input|AddMovementInput (Variables|Default|GetDirectionVector) 1.0 false)))))

(fn ConstructionScript)

(fn UpdateHealth
  (bind _hp_widget (Variables|Default|GetHP_Widget))
  (Rendering|SetVisibility _hp_widget true false)
  (bind _asenemy_health (Utilities|Casting|CastToEnemyHealth (UserInterface|GetUserWidgetObject _hp_widget)))
  (Progress|SetPercent (Variables|/Game/Reign_Assets/EnemyObjects/EnemyHealth.EnemyHealth_C|GetEnemyHealth _asenemy_health) (/ (Variables|Default|GetCurrentHealth) (Variables|Default|GetMaxHealth))))

(fn HideHP
  (Rendering|SetVisibility (Variables|Default|GetHP_Widget) false false))

(fn MovementFuntion
  (Variables|Default|SetDirectionVector (Math|Vector|GetForwardVector (Math|Rotator|FindLookatRotation (Transformation|GetWorldLocation (Variables|Collision|GetCapsuleComponent)) (Transformation|GetWorldLocation (Variables|/Script/Engine.Character|GetCapsuleComponent (Variables|Default|GetPlayerRef)))))))

(fn CheckiftoFar
  (Math|Float|CompareFloat (Math|Vector|VectorLength (- (Variables|Default|GetStartingPoint) (Transformation|GetWorldLocation (Variables|Collision|GetCapsuleComponent)))) 2e+03
    (:>
      (Variables|Default|SetMaxRange? true))
    (:==
      (Variables|Default|SetMaxRange? false :!label _label))
    (:<
      (goto _label)))
  (return))

(fn InitStartingPoint
  (bind _capsulecomponent (Variables|Collision|GetCapsuleComponent))
  (bind _returnvalue (Transformation|GetWorldLocation _capsulecomponent))
  (bind (_outhit _returnvalue_2) (Collision|LineTraceByChannel _returnvalue (- _returnvalue (* (Math|Vector|GetUpVector _capsulecomponent) 1.5e+03)) "TraceTypeQuery1" false 0 "None"))
  (if _returnvalue_2
    (Variables|Default|SetStartingPoint (+ (.impactpoint _outhit) "0, 0,100.000000"))))

(fn FindNewLoc
  (bind _capsulecomponent (Variables|Collision|GetCapsuleComponent))
  (bind _returnvalue (Transformation|GetWorldLocation _capsulecomponent))
  (if (Variables|Default|GetMaxRange?)
    (Variables|Default|SetDirectionVector (Math|Vector|GetForwardVector (Math|Rotator|FindLookatRotation (Transformation|GetWorldLocation (Variables|Collision|GetCapsuleComponent)) (Variables|Default|GetStartingPoint))))
    (else
      (Variables|Default|SetDirectionVector (Math|Vector|GetForwardVector (Math|Rotator|FindLookatRotation _returnvalue (+ _returnvalue (Math|Vector|MakeVector (Math|Random|RandomFloatinRange -5e+03 5e+03) (Math|Random|RandomFloatinRange -3e+03 3e+03) 0.0))))))))

(fn HeavyDeathCheck
  (if (<= (Variables|Default|GetCurrentHealth) 0.0)
    (Variables|Default|SetAlive? false)
    (else
      (Variables|Default|SetAlive? true))))