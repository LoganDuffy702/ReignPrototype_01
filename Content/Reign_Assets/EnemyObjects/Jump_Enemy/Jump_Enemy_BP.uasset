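; Hopping enemy character that moves in repeated leaps and lunges at the player within aggro range.
; Each landing spawns FX and schedules the next leap after a random delay, alternating yaw offsets to zigzag outside that range.
; Lunges ignore pawn collision and use a looping timer line trace to deal damage, then launch again.
; Grapple and pull hits trigger random sideways dodges; only melee reduces its health.
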(event OnComponentBeginOverlap(AgroCollision)
  (params (OverlappedComponent :type Primitive%20Component%20Object%20Reference) (OtherActor :type Actor%20Object%20Reference) (OtherComp :type Primitive%20Component%20Object%20Reference) (OtherBodyIndex :type Integer) (bFromSweep :type Boolean) (SweepResult :type Hit%20Result%20Structure%20%28by%20ref%29)))

(event Custom|Leap%20Event
  (bind _capsulecomponent (Variables|Default|GetCapsuleComponent))
  (bind _capsulecomponent_2 (Variables|Default|GetCapsuleComponent))
  (Transformation|SetWorldRotation (Variables|Default|GetCapsuleComponent) (Math|Rotator|MakeRotator 0.0 0.0 (|GetLookAtRot)) false false)
  (if (<= (|GetVectorLengthofActortoPlayer) (Variables|Default|GetAgro%20Distance))
    (Collision|SetCollisionResponsetoChannel _capsulecomponent_2 "ECC_Pawn" "ECR_Ignore")
    (Collision|SetCollisionResponsetoChannel _capsulecomponent_2 "ECC_GameTraceChannel1" "ECR_Ignore")
    (CallFunction|LeapAttack)
    (else
      (Collision|SetCollisionResponsetoChannel _capsulecomponent "ECC_Pawn" "ECR_Block")
      (Collision|SetCollisionResponsetoChannel _capsulecomponent "ECC_GameTraceChannel1" "ECR_Block")
      (Class|KismetSystemLibrary|PauseTimer 0 "AttackTrace")
      (Utilities|FlowControl|MultiGate false true -1
        (:Out%200
          (Transformation|AddWorldRotation (Variables|Default|GetCapsuleComponent) "0.000000,-25.000000, 0" false false))
        (:Out%201
          (Transformation|AddWorldRotation (Variables|Default|GetCapsuleComponent) "0.000000,25.000000, 0" false false)))
      (Effects|SpawnEmitteratLocation "/Game/Reign_Assets/EnemyObjects/Jump_Enemy/Jump_FX/JumpStart_Enemy_LeapFX1.JumpStart_Enemy_LeapFX1" (- (Transformation|GetWorldLocation (Variables|Default|GetCapsuleComponent)) "0, 0,50.000000") "0, 0, 0" (.scale (Transformation|GetActorTransform)))
      (Character|LaunchCharacter (* (+ (Math|Vector|GetForwardVector (Variables|Default|GetCapsuleComponent)) "0, 0,1.500000") (Variables|Default|GetLaunchPower)) false false))))

(event Custom|DodgeAttackEvent
  (Variables|/Script/Engine.MovementComponent|SetVelocity (Variables|Character|GetCharacterMovement) "0, 0, 0")
  (Utilities|FlowControl|MultiGate true true -1
    (:Out%200
      (Character|LaunchCharacter (* (+ (Math|Vector|GetRightVector (Variables|Default|GetCapsuleComponent)) "0, 0,1.500000") (Variables|Default|GetLaunchPower)) false false))
    (:Out%201
      (Character|LaunchCharacter (* (+ (Math|Vector|GetRightVector (Variables|Default|GetCapsuleComponent)) "0, 0,1.500000") (* (Variables|Default|GetLaunchPower) -1.0)) false false))))

(event Custom|LeapAttack
  (Transformation|SetWorldRotation (Variables|Default|GetCapsuleComponent) (Math|Rotator|MakeRotator 0.0 0.0 (|GetLookAtRot_2)) false false)
  (Utilities|FlowControl|Delay 0.2)
  (Character|LaunchCharacter (* (+ (Math|Vector|GetForwardVector (Variables|Default|GetCapsuleComponent)) "0, 0,0.300000") (* (Variables|Default|GetLaunchPower) (Variables|Default|GetAttackDistanceMulti))) false false)
  (Utilities|Time|SetTimerbyFunctionName 0 "AttackTrace" 0.01 true))

(event Custom|AttackTrace
  (bind _capsulecomponent (Variables|Default|GetCapsuleComponent))
  (bind _returnvalue (Transformation|GetWorldLocation _capsulecomponent))
  (bind _returnvalue_2 (Collision|LineTraceForObjects _returnvalue (- _returnvalue (* (Math|Vector|GetForwardVector (Transformation|GetWorldRotation _capsulecomponent)) 1e+02)) (Utilities|Array|MakeArray "ObjectTypeQuery3") false (Utilities|Array|MakeArray self) "None" true "(R=1.000000,G=0.000000,B=0.000000,A=1.000000)" "(R=0.000000,G=1.000000,B=0.000000,A=1.000000)" 0.5))
  (if _returnvalue_2
    (Default|DealingDamage (Variables|Default|GetPlayerRef) 7 0 "None")
    (Class|KismetSystemLibrary|PauseTimer 0 "AttackTrace")
    (Utilities|FlowControl|Delay 0.2)
    (Character|LaunchCharacter (* (+ (Math|Vector|GetForwardVector (Variables|Default|GetCapsuleComponent)) "0, 0,0.500000") (* (Variables|Default|GetLaunchPower) 1.3)) false false)))

(event EventBeginPlay
  (|CallParentFunction)
  (Utilities|FlowControl|Delay (Math|Random|RandomFloatinRange 1.0 3.0))
  (CallFunction|LeapEvent))

(event Collision|EventActorBeginOverlap
  (params (OtherActor :type Actor%20Object%20Reference)))

(event EventTick
  (params (DeltaSeconds :type Float%20%28single-precision%29))
  (|CallParentFunction DeltaSeconds) ; This node is disabled and will not be called.\nDrag off pins to build functionality.
)

(event EventDealingDamage
  (params (Sent%20Damage :type Integer) (Sender :type Actor%20Object%20Reference) (DamageType :type Name :default "None"))
  (switch name DamageType
    (:Grapple
      (CallFunction|DodgeAttackEvent :!label _label))
    (:PullTo
      (goto _label))
    (:Melee
      (CallFunction|ShowHealthbar)
      (Variables|Default|SetCurrentHealth (- (Variables|Default|GetCurrentHealth) 70))
      (CallFunction|UpdateHealth)
      (if (<= (Variables|Default|GetCurrentHealth) 0)
        (CallFunction|DeathEvent)))))

(event EventOnLanded
  (params (Hit :type Hit%20Result%20Structure%20%28by%20ref%29))
  (Effects|SpawnEmitteratLocation "/Game/Reign_Assets/EnemyObjects/Jump_Enemy/Jump_FX/JumpEnd_Enemy_LeapFX.JumpEnd_Enemy_LeapFX" (.impactpoint Hit) "0, 0, 0" (.scale (Transformation|GetActorTransform)))
  (Utilities|FlowControl|Delay (Math|Random|RandomFloatinRange 0.5 2.0))
  (CallFunction|LeapEvent))

(fn ConstructionScript
  (|CallParentFunction))