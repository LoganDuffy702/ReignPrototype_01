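; Laser turret enemy that tracks the player within range of its tower and deals repeated damage with a beam.
; Each tick it turns an arrow's yaw toward the player at a constant rate, line-traces for pawns and stretches the beam effect along the trace.
; A hit starts a looping damage timer through a DoOnce; losing the target pauses it.
; Its DealingDamage event resets the player's equipped weapon after a short delay.
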(event Custom|DealDamage
  (Default|DealingDamage (Variables|Default|GetPlayerRef) 2 0 "None")
  (Utilities|Time|SetTimerbyEvent (delegate Custom|DealDamage) 0.2 true))

(event EventBeginPlay
  (|CallParentFunction))

(event Collision|EventActorBeginOverlap
  (params (OtherActor :type Actor%20Object%20Reference)))

(event EventTick
  (params (DeltaSeconds :type Float%20%28single-precision%29))
  (bind _arrow1 (Variables|Default|GetArrow1))
  (bind _lazer_fx (Variables|Default|GetLazer_FX))
  (bind _returnvalue (Transformation|GetWorldLocation _arrow1))
  (|CallParentFunction DeltaSeconds)
  (if (<= (Math|Vector|VectorLength (- (Transformation|GetActorLocation (Variables|Default|GetPlayerRef)) (Transformation|GetWorldLocation (Variables|Default|GetTower)))) 1e+03)
    (Rendering|SetVisibility (Variables|Default|GetLazer_FX) true false)
    (Transformation|SetWorldRotation (Variables|Default|GetArrow1) (Math|Rotator|MakeRotator 0.0 0.0 (.yaw (Class|KismetMathLibrary|RInterptoConstant (Transformation|GetWorldRotation (Variables|Default|GetArrow1)) (Math|Rotator|FindLookatRotation (Transformation|GetWorldLocation (Variables|Default|GetArrow1)) (Transformation|GetActorLocation (Variables|Default|GetPlayerRef))) 0.01 45.0))) false false)
    (bind (_outhit _returnvalue_2) (Collision|LineTraceForObjects _returnvalue (- _returnvalue (* (Math|Vector|GetForwardVector _arrow1) -1e+03)) (Utilities|Array|MakeArray "ObjectTypeQuery3") false (Utilities|Array|MakeArray self) "None"))
    (Class|ParticleSystemComponent|SetBeamSourcePoint _lazer_fx 0 (.TraceStart (Collision|BreakHitResult _outhit)))
    (Class|ParticleSystemComponent|SetBeamEndPoint _lazer_fx 0 (.TraceEnd (Collision|BreakHitResult _outhit)))
    (if _returnvalue_2
      (Utilities|FlowControl|DoOnce false :!label _label
        (:Completed
          (CallFunction|DealDamage)))
      (else
        (Class|KismetSystemLibrary|PauseTimer 0 "DealDamage")
        (goto _label Reset)))
    (else
      (Rendering|SetVisibility (Variables|Default|GetLazer_FX) false false)
      (Class|KismetSystemLibrary|PauseTimer 0 "DealDamage"))))

(event EventDealingDamage
  (params (Sent%20Damage :type Integer) (Sender :type Actor%20Object%20Reference) (DamageType :type Name :default "None"))
  (Utilities|FlowControl|Delay 0.2)
  (Default|WeaponReset (Variables|/Game/Reign_Assets/Player_Character/Blueprints/MC_Prototype_BP.MC_Prototype_BP_C|GetEquippedWeapon (Variables|Default|GetPlayerRef))))

(fn ConstructionScript
  (|CallParentFunction))