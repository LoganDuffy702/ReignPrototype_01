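; Master enemy Blueprint that tracks health and shows it on an attached health bar widget.
; The DealingDamage event subtracts damage from CurrentHealth without clamping or death handling, then calls UpdateHealth, which also runs on BeginPlay.
; UpdateHealth casts the widget component's user widget to EnemyHealth and sets its bar percent to current over max health.
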(event EventBeginPlay
  (CallFunction|UpdateHealth))

(event EventDealingDamage
  (params (Damage :type Integer) (Sender :type Actor%20Object%20Reference))
  (Variables|Default|SetCurrentHealth (- (Variables|Default|GetCurrentHealth) Damage))
  (CallFunction|UpdateHealth))

(fn ConstructionScript)

(fn UpdateHealth
  (bind _asenemy_health (Utilities|Casting|CastToEnemyHealth (UserInterface|GetUserWidgetObject (Variables|Default|GetEnemyHealth))))
  (Progress|SetPercent (Variables|/Game/Reign_Assets/EnemyObjects/EnemyHealth.EnemyHealth_C|GetEnemyHealth _asenemy_health) (/ (Math|Conversions|ToFloat(Integer) (Variables|Default|GetCurrentHealth)) (Math|Conversions|ToFloat(Integer) (Variables|Default|GetMaxHealth))))
  (return))