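; Master enemy Blueprint that provides shared health, lock-on and death behavior, with empty attack, reset and pull functions.
; It drives a health bar widget that can show briefly, toggles a lock-on marker, and line-traces to the player for targetability.
; DeathEvent drops random healing orbs, updates player souls and destroys the actor.
; DealingDamage is empty; the typed damage logic with hit montages and death check is disconnected.
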(event Custom|Death%20Event
  (bind _chokepoint (Variables|Default|GetChokePoint))
  (bind _returnvalue (Transformation|GetWorldLocation _chokepoint))
  ;[1 1 1] Death
  (for _index (range 0 (Math|Random|RandomIntegerinRange 1 3))
    (switch int (Math|Random|RandomIntegerinRange 0 1)
      (:0
        (bind _returnvalue_2 (Game|SpawnActorfromClass "/Game/Reign_Assets/World_Objects/Drop_Objects/Healing_Orb_Large_BP.Healing_Orb_Large_BP_C" (Math|Transform|MakeTransform _returnvalue "0, 0, 0" "0.500000,0.500000,0.500000") "Undefined" 0 0))
        (Variables|/Game/Reign_Assets/World_Objects/Drop_Objects/Healing_Orb_Large_BP.Healing_Orb_Large_BP_C|SetHealAmount _returnvalue_2 8))
      (:1
        (bind _returnvalue_3 (Game|SpawnActorfromClass "/Game/Reign_Assets/World_Objects/Drop_Objects/Healing_Orb_Small_BP.Healing_Orb_Small_BP_C" (Math|Transform|MakeTransform _returnvalue "0, 0, 0" "0.300000,0.300000,0.300000") "Undefined" 0 0))
        (Variables|/Game/Reign_Assets/World_Objects/Drop_Objects/Healing_Orb_Small_BP.Healing_Orb_Small_BP_C|SetHealAmount _returnvalue_3 2))))
  (bind _asmc_prototype_bp (Utilities|Casting|CastToMC_Prototype_BP (Game|GetPlayerCharacter 0)))
  (Default|UpdateSouls _asmc_prototype_bp)
  (Actor|DestroyActor))

(event Custom|ShowHealthbar
  ;[1 1 1] Health bar
  (Rendering|SetVisibility (Variables|Default|GetEnemyHealth) true false)
  (Utilities|FlowControl|RetriggerableDelay 2.0)
  (CallFunction|HideHealthBar))

(event Custom|HideHealthBar
  ;[1 1 1] Health bar
  (Rendering|SetVisibility (Variables|Default|GetEnemyHealth) false false))

(event EventLockon
  ;[1 1 1] LockOnEvent
  (Utilities|FlowControl|FlipFlop
    (:A
      (Rendering|SetVisibility (Variables|Default|GetLockOnMarker) true false))
    (:B
      (Rendering|SetVisibility (Variables|Default|GetLockOnMarker) false false))))

(event EventBeginPlay
  ;[1 1 1] On Begin
  (Variables|Default|SetCurrentHealth (Variables|Default|GetMaxHealth))
  (CallFunction|UpdateHealth)
  (bind _asmc_prototype_bp (Utilities|Casting|CastToMC_Prototype_BP (Game|GetPlayerCharacter 0)))
  (Variables|Default|SetPlayerRef _asmc_prototype_bp))

(event EventDealingDamage
  (params (Sent%20Damage :type Integer) (Sender :type Actor%20Object%20Reference) (DamageType :type Name :default "None"))
  ;[1 1 1] Damage Solver
)

(fn ConstructionScript)

(fn UpdateHealth
  (bind _asenemy_health (Utilities|Casting|CastToEnemyHealth (UserInterface|GetUserWidgetObject (Variables|Default|GetEnemyHealth))))
  (Progress|SetPercent (Variables|/Game/Reign_Assets/EnemyObjects/EnemyHealth.EnemyHealth_C|GetEnemyHealth _asenemy_health) (/ (Math|Conversions|ToFloat(Integer) (Variables|Default|GetCurrentHealth)) (Math|Conversions|ToFloat(Integer) (Variables|Default|GetMaxHealth))))
  (return))

(fn DistancetoPlayer
  (bind (_outhit _returnvalue) (Collision|LineTraceForObjects (Transformation|GetActorLocation) (Transformation|GetActorLocation (Game|GetPlayerCharacter 0)) (Utilities|Array|MakeArray "ObjectTypeQuery3") false (Utilities|Array|MakeArray self) "None" true "(R=1.000000,G=0.000000,B=0.000000,A=1.000000)" "(R=0.000000,G=1.000000,B=0.000000,A=1.000000)" 0.1))
  (if _returnvalue
    (Variables|Default|SetPlayerToEnemyDistance (.Distance (Collision|BreakHitResult _outhit)))
    (Variables|Default|SetCanBeTargeted true)
    (return)
    (else
      (Variables|Default|SetCanBeTargeted false))))

(fn MeleeEnemyAttackTrace)

(fn ResetEnemy)

(fn PullEvent)

(fn StopPullEvent)