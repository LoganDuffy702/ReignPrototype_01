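; Grapple V3 is an enemy-object grapple point in the lock-on Blueprint folder that pulls the player when its DealingDamage event fires.
; The event zeroes the player's velocity, then launches them hard along the forward vector of their PlayerGrappleOrigin component.
; After a short delay it resets the player's equipped weapon, waiting slightly longer if the player is still falling.
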(event EventBeginPlay
  (|CallParentFunction) ; This node is disabled and will not be called.\nDrag off pins to build functionality.
)

(event Collision|EventActorBeginOverlap
  (params (OtherActor :type Actor%20Object%20Reference)))

(event EventTick
  (params (DeltaSeconds :type Float%20%28single-precision%29))
  (|CallParentFunction DeltaSeconds) ; This node is disabled and will not be called.\nDrag off pins to build functionality.
)

(event EventDealingDamage
  (params (Sent%20Damage :type Integer) (Sender :type Actor%20Object%20Reference) (DamageType :type Name :default "None"))
  (Variables|/Script/Engine.MovementComponent|SetVelocity (Variables|/Script/Engine.Character|GetCharacterMovement (Variables|Default|GetPlayerRef)) "0, 0, 0")
  (CallFunction|PullEvent))

(event EventPullEvent
  (Character|LaunchCharacter (Variables|Default|GetPlayerRef) (* (Math|Vector|GetForwardVector (Variables|/Game/Reign_Assets/Player_Character/Blueprints/MC_Prototype_BP.MC_Prototype_BP_C|GetPlayerGrappleOrigin (Variables|Default|GetPlayerRef))) 1e+04) false false)
  (Utilities|FlowControl|Delay 0.3)
  (if (AI|Components|NavMovement|IsFalling (Variables|/Script/Engine.Character|GetCharacterMovement (Variables|Default|GetPlayerRef)))
    (Utilities|FlowControl|Delay 0.4)
    (Default|WeaponReset (Variables|/Game/Reign_Assets/Player_Character/Blueprints/MC_Prototype_BP.MC_Prototype_BP_C|GetEquippedWeapon (Variables|Default|GetPlayerRef)))
    (else
      (Default|WeaponReset (Variables|/Game/Reign_Assets/Player_Character/Blueprints/MC_Prototype_BP.MC_Prototype_BP_C|GetEquippedWeapon (Variables|Default|GetPlayerRef))))))

(fn ConstructionScript
  (|CallParentFunction))