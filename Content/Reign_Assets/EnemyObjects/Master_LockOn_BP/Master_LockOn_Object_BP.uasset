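; Base lock-on target for enemy objects, with a health bar, lock-on marker, player-linked beam and death drops.
; While active, Tick line-traces to the player to update distance and targetability.
; Repeated Lockon calls keep marker and beam visible through a retriggerable delay, with beam material set by Grapple or Pull-to attack type.
; Death spawns random healing orbs and updates player souls; attack, reset and pull functions are empty stubs.
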(event Custom|Death%20Event
  (bind _chokepoint (Variables|Default|GetChokePoint))
  (bind _returnvalue (Transformation|GetWorldLocation _chokepoint))
  ;[1 1 1] Death
  (for _index (range 0 (Math|Random|RandomIntegerinRange 1 3))
    (switch int (Math|Random|RandomIntegerinRange 0 1)
      (:0
        (bind _returnvalue_2 (Game|SpawnActorfromClass "/Game/Reign_Assets/World_Objects/Drop_Objects/Healing_Orb_Large_BP.Healing_Orb_Large_BP_C" (Math|Transform|MakeTransform _returnvalue "0, 0, 0" "0.500000,0.500000,0.500000") "Undefined" 0 0))
        (Variables|/Game/Reign_Assets/World_Objects/Drop_Objects/Healing_Orb_Large_BP.Healing_Orb_Large_BP_C|SetHealAmount _returnvalue_2 8))
      (:1
        (bind _returnvalue_3 (Game|SpawnActorfromClass "/Game/Reign_Assets/World_Objects/Drop_Objects/Healing_Orb_Small_BP.Healing_Orb_Small_BP_C" (Math|Transform|MakeTransform _returnvalue "0, 0, 0" "0.300000,0.300000,0.300000") "Undefined" 0 0))
        (Variables|/Game/Reign_Assets/World_Objects/Drop_Objects/Healing_Orb_Small_BP.Healing_Orb_Small_BP_C|SetHealAmount _returnvalue_3 2))))
  (bind _asmc_prototype_bp (Utilities|Casting|CastToMC_Prototype_BP (Game|GetPlayerCharacter 0)))
  (Default|UpdateSouls _asmc_prototype_bp)
  (Actor|DestroyActor))

(event Custom|SetCameraEvent
  (bind _capsulecomponent (Variables|Collision|GetCapsuleComponent))
  (bind _camlastlocation (Variables|Default|GetCamLastLocation))
  (bind _returnvalue (Transformation|GetWorldLocation _capsulecomponent))
  (bind (_x _y) (Math|Vector|BreakVector _camlastlocation))
  (bind (_x_2 _y_2 _z) (Math|Vector|BreakVector _returnvalue))
  ;[1 1 1] Camera Movement
  (Transformation|SetWorldLocation (Variables|/Game/Reign_Assets/Player_Character/Blueprints/MC_Prototype_BP.MC_Prototype_BP_C|GetSpringArm (Variables|Default|GetPlayerRef)) (Math|Interpolation|VInterpTo _camlastlocation (Math|Vector|MakeVector (/ (+ _x _x_2) 2.0) (/ (+ _y _y_2) 2.0) _z) 0.1 2e+01) false false))

(event Custom|CheckLockOn%20Event
  ;[1 1 1] DistanceCheck
)

(event Custom|Link%20FX
  (bind _particlesystem (Variables|Default|GetParticleSystem))
  ;[1 1 1] Comment
  (switch name (Variables|/Game/Reign_Assets/Player_Character/Blueprints/MC_Prototype_BP.MC_Prototype_BP_C|GetAttackType (Variables|Default|GetPlayerRef))
    (:Grapple
      (Rendering|Material|SetMaterial _particlesystem 0 "/Game/Reign_Assets/FX/Gun/CableBased/WeaponChain/LockOnGrapple_Mat.LockOnGrapple_Mat"))
    (:PullTo
      (Rendering|Material|SetMaterial _particlesystem 0 "/Game/Reign_Assets/FX/Gun/CableBased/WeaponChain/LockOnPullTo_Mat.LockOnPullTo_Mat")))
  (Class|ParticleSystemComponent|SetBeamTargetPoint (Variables|Default|GetParticleSystem) 0 (Transformation|GetWorldLocation (Variables|/Game/Reign_Assets/Weapon_BP/Master_Weapon_BP.Master_Weapon_BP_C|GetFirepoint (Variables|/Game/Reign_Assets/Player_Character/Blueprints/MC_Prototype_BP.MC_Prototype_BP_C|GetEquippedWeapon (Variables|Default|GetPlayerRef))))))

(event Custom|ShowHealthbar
  ;[1 1 1] Health bar
  (Rendering|SetVisibility (Variables|Default|GetEnemyHealth) true false)
  (Utilities|FlowControl|RetriggerableDelay 2.0)
  (CallFunction|HideHealthBar))

(event Custom|HideHealthBar
  ;[1 1 1] Health bar
  (Rendering|SetVisibility (Variables|Default|GetEnemyHealth) false false))

(event EventLockon
  ;[1 1 1] LockOnEvent
  (if (Variables|Default|GetCanBeLockedOn?)
    (if (Variables|Default|GetIsLinked?)
      (Rendering|SetVisibility (Variables|Default|GetLockOnMarker) true false)
      (Rendering|SetVisibility (Variables|Default|GetParticleSystem) true false)
      (CallFunction|LinkFX)
      (Utilities|FlowControl|RetriggerableDelay 0.1)
      (else
        (Variables|/Game/Reign_Assets/Player_Character/Blueprints/MC_Prototype_BP.MC_Prototype_BP_C|SetNearestTarget (Variables|Default|GetPlayerRef) 0)))
    (Rendering|SetVisibility (Variables|Default|GetLockOnMarker) false false)
    (Rendering|SetVisibility (Variables|Default|GetParticleSystem) false false)))

(event EventTick
  (params (DeltaSeconds :type Float%20%28single-precision%29))
  ;[1 1 1] Tick event
  (Class|ParticleSystemComponent|SetBeamSourcePoint (Variables|Default|GetParticleSystem) 0 (Transformation|GetWorldLocation (Variables|Default|GetChokePoint)))
  (if (Variables|Default|GetActivePlayerCheck)
    (CallFunction|DistancetoPlayer)))

(event EventBeginPlay
  ;[1 1 1] On Begin
  (Variables|Default|SetCurrentHealth (Variables|Default|GetMaxHealth))
  (CallFunction|UpdateHealth)
  (bind _asmc_prototype_bp (Utilities|Casting|CastToMC_Prototype_BP (Game|GetPlayerCharacter 0)))
  (Variables|Default|SetPlayerRef _asmc_prototype_bp)
  (bind _outactors (Actor|GetAllActorsOfClass "/Game/Reign_Assets/Player_Character/Blueprints/Mouse_Companion/Mouse_Or_Companion_BP.Mouse_Or_Companion_BP_C"))
  (Variables|Default|SetMouseObject (Utilities|Array|Get(acopy) _outactors)))

(fn ConstructionScript)

(fn UpdateHealth
  (bind _asenemy_health (Utilities|Casting|CastToEnemyHealth (UserInterface|GetUserWidgetObject (Variables|Default|GetEnemyHealth))))
  (Progress|SetPercent (Variables|/Game/Reign_Assets/EnemyObjects/EnemyHealth.EnemyHealth_C|GetEnemyHealth _asenemy_health) (/ (Math|Conversions|ToFloat(Integer) (Variables|Default|GetCurrentHealth)) (Math|Conversions|ToFloat(Integer) (Variables|Default|GetMaxHealth))))
  (return))

(fn DistancetoPlayer
  (bind (_outhit _returnvalue) (Collision|LineTraceForObjects (Transformation|GetActorLocation) (Transformation|GetWorldLocation (Variables|/Script/Engine.Character|GetCapsuleComponent (Variables|Default|GetPlayerRef))) (Utilities|Array|MakeArray "ObjectTypeQuery3") false (Utilities|Array|MakeArray self) "ForOneFrame" true "(R=0.000000,G=0.657399,B=1.000000,A=1.000000)" "(R=0.000000,G=1.000000,B=0.000000,A=1.000000)" 0.1))
  (if _returnvalue
    (Variables|Default|SetPlayerToEnemyDistance (.Distance (Collision|BreakHitResult _outhit)))
    (Variables|Default|SetCanBeTargeted true)
    (return)
    (else
      (Variables|Default|SetCanBeTargeted false))))

(fn MeleeEnemyAttackTrace)

(fn ResetEnemy)

(fn PullEvent)

(fn StopPullEvent)