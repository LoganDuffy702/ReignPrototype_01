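; Lock-on object that responds to the player's chain weapon by either launching the player or being pulled in, based on the damage type in DealingDamage.
; Grapple launches the player along their grapple origin's forward vector, then resets the weapon after a short delay, extended if airborne.
; Pull to uses a timeline to lerp the object to the player's AoE point at constant height, updating the chain beam's end, then resets the weapon.
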(event EventBeginPlay
  (|CallParentFunction) ; This node is disabled and will not be called.\nDrag off pins to build functionality.
)

(event Collision|EventActorBeginOverlap
  (params (OtherActor :type Actor%20Object%20Reference)))

(event EventTick
  (params (DeltaSeconds :type Float%20%28single-precision%29))
  (|CallParentFunction DeltaSeconds) ; This node is disabled and will not be called.\nDrag off pins to build functionality.
)

(event EventDealingDamage
  (params (Sent%20Damage :type Integer) (Sender :type Actor%20Object%20Reference) (DamageType :type Name :default "None"))
  (bind _playerref (Variables|Default|GetPlayerRef))
  (bind _aoe_point (Variables|/Game/Reign_Assets/Player_Character/Blueprints/MC_Prototype_BP.MC_Prototype_BP_C|GetAoE%20Point _playerref))
  (bind _returnvalue (Transformation|GetWorldLocation _aoe_point))
  (switch name DamageType
    (:Grapple
      (Development|PrintString "Grapple")
      (Character|LaunchCharacter (Variables|Default|GetPlayerRef) (* (Math|Vector|GetForwardVector (Variables|/Game/Reign_Assets/Player_Character/Blueprints/MC_Prototype_BP.MC_Prototype_BP_C|GetPlayerGrappleOrigin (Variables|Default|GetPlayerRef))) 1e+04) false false)
      (Utilities|FlowControl|Delay 0.3)
      (if (AI|Components|NavMovement|IsFalling (Variables|/Script/Engine.Character|GetCharacterMovement (Variables|Default|GetPlayerRef)))
        (Utilities|FlowControl|Delay 0.2)
        (Default|WeaponReset (Variables|/Game/Reign_Assets/Player_Character/Blueprints/MC_Prototype_BP.MC_Prototype_BP_C|GetEquippedWeapon (Variables|Default|GetPlayerRef)))
        (else
          (Default|WeaponReset (Variables|/Game/Reign_Assets/Player_Character/Blueprints/MC_Prototype_BP.MC_Prototype_BP_C|GetEquippedWeapon (Variables|Default|GetPlayerRef))))))
    (:PullTo
      (Variables|Default|SetLastLoc (Transformation|GetActorLocation))
      (bind _newtrack_0 (Timeline|Timeline_0 PlayFromStart)
        (:Update
          (Class|ParticleSystemComponent|SetBeamEndPoint (Variables|/Game/Reign_Assets/Weapon_BP/Master_Weapon_BP.Master_Weapon_BP_C|GetChainParticle (Variables|/Game/Reign_Assets/Player_Character/Blueprints/MC_Prototype_BP.MC_Prototype_BP_C|GetEquippedWeapon (Variables|Default|GetPlayerRef))) 0 (Transformation|GetWorldLocation (Variables|Default|GetChokePoint)))
          (Transformation|SetActorLocation (Math|Vector|Lerp(Vector) (Math|Vector|MakeVector (.x (Variables|Default|GetLastLoc)) (.y (Variables|Default|GetLastLoc)) (.z (Variables|Default|GetLastLoc))) (Math|Vector|MakeVector (.x _returnvalue) (.y _returnvalue) (.z (Variables|Default|GetLastLoc))) _newtrack_0) false false))
        (:Finished
          (Default|WeaponReset (Variables|/Game/Reign_Assets/Player_Character/Blueprints/MC_Prototype_BP.MC_Prototype_BP_C|GetEquippedWeapon (Variables|Default|GetPlayerRef))))))))

(fn ConstructionScript
  (|CallParentFunction))