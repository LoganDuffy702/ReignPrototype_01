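; Melee enemy character that can dodge backward, with its dodge state tied to the player.
; Each Tick copies the player's CannotAttack flag into Dodge.
; DodgeAnim plays a backward dodge animation directly on the mesh, then returns it to Animation Blueprint mode after a short delay.
; C_Move adds movement input along the mesh's forward or right vector, chosen by LeftRight and scaled by MovementValue.
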(event Custom|Dodge%20Anim
  (Components|Animation|PlayAnimation (Variables|Character|GetMesh) "/Game/Reign_Assets/EnemyObjects/EnemyAnimations/Standing_Dodge_Backward.Standing_Dodge_Backward" false)
  (Utilities|FlowControl|Delay 1.0)
  (Components|Animation|SetAnimationMode (Variables|Character|GetMesh) "AnimationBlueprint"))

(event EventBeginPlay
  (|CallParentFunction) ; This node is disabled and will not be called.\nDrag off pins to build functionality.
)

(event Collision|EventActorBeginOverlap
  (params (OtherActor :type Actor%20Object%20Reference))
  (|CallParentFunction OtherActor) ; This node is disabled and will not be called.\nDrag off pins to build functionality.
)

(event EventTick
  (params (DeltaSeconds :type Float%20%28single-precision%29))
  (|CallParentFunction DeltaSeconds)
  (Variables|Default|SetDodge? (Variables|/Game/Reign_Assets/Player_Character/Blueprints/MC_Prototype_BP.MC_Prototype_BP_C|GetCannot%20Attack (Variables|Default|GetPlayerRef))))

(fn ConstructionScript
  (|CallParentFunction))

(fn CMove
  (bind _mesh (Variables|Character|GetMesh))
  (if (Variables|Default|GetLeft/Right)
    (Pawn|Input|AddMovementInput (Math|Vector|GetForwardVector _mesh) (Variables|Default|GetMovement%20Value) false)
    (return)
    (else
      (Pawn|Input|AddMovementInput (Math|Vector|GetRightVector _mesh) (Variables|Default|GetMovement%20Value) false)
      (return))))