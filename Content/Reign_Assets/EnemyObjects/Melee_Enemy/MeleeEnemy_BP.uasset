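; Melee enemy character that attacks the player inside its aggro range and reacts to incoming damage.
; An attack montage repeats through a reset event after an interval, while a sphere trace ignoring fellow enemies deals damage.
; Damage type selects the reaction: knockback, hit animation, or a grapple pull that disables gravity and interpolates toward the player on a looping timer.
; A collapsed death check disables the enemy and plays a random death montage.
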(event OnComponentBeginOverlap(AggroCollision)
  (params (OverlappedComponent :type Primitive%20Component%20Object%20Reference) (OtherActor :type Actor%20Object%20Reference) (OtherComp :type Primitive%20Component%20Object%20Reference) (OtherBodyIndex :type Integer) (bFromSweep :type Boolean) (SweepResult :type Hit%20Result%20Structure%20%28by%20ref%29))
  ;[1 1 1] Agro
  (Variables|Default|SetCanAttack? true)
  (bind _asmc_prototype_bp (Utilities|Casting|CastToMC_Prototype_BP (Game|GetPlayerCharacter 0)))
  (Variables|Default|SetPlayerRef _asmc_prototype_bp)
  (if (not (Variables|Default|GetPlayingAnimation?))
    (CallFunction|EnemyMeleeAttack)))

(event OnComponentEndOverlap(AggroCollision)
  (params (OverlappedComponent :type Primitive%20Component%20Object%20Reference) (OtherActor :type Actor%20Object%20Reference) (OtherComp :type Primitive%20Component%20Object%20Reference) (OtherBodyIndex :type Integer))
  ;[1 1 1] Agro
  (Variables|Default|SetCanAttack? false)
  (Variables|Default|SetPlayingAnimation? false))

(event Custom|EnemyMeleeAttack
  ;[1 1 1] Agro
  (if (Variables|Default|GetIsAlive?)
    (if (Variables|Default|GetCanAttack?)
      (Utilities|FlowControl|Delay 0.2)
      (Variables|Default|SetPlayingAnimation? true)
      (Animation|PlayAnimMontage (Variables|Default|GetMeleeAtkAnimation) (Variables|Default|GetAttackSpeed) "None"))))

(event EventBeginPlay
  (|CallParentFunction) ; This node is disabled and will not be called.\nDrag off pins to build functionality.
)

(event Collision|EventActorBeginOverlap
  (params (OtherActor :type Actor%20Object%20Reference)))

(event EventStopPullEvent
  (bind _playerref (Variables|Default|GetPlayerRef))
  (bind _charactermovement (Variables|/Script/Engine.Character|GetCharacterMovement _playerref))
  ;[1 1 1] Melee Enemy Damage Solver
  (Variables|/Script/Engine.CharacterMovementComponent|SetGravityScale (Variables|Character|GetCharacterMovement) 1.0)
  (Variables|Default|SetPullActive? true)
  (Class|KismetSystemLibrary|PauseTimer 0 "Pull Event")
  (Default|WeaponReset (Variables|/Game/Reign_Assets/Player_Character/Blueprints/MC_Prototype_BP.MC_Prototype_BP_C|GetEquippedWeapon _playerref))
  (Variables|/Script/Engine.CharacterMovementComponent|SetbOrientRotationToMovement _charactermovement true)
  (Variables|/Script/Engine.CharacterMovementComponent|SetbUseControllerDesiredRotation _charactermovement false)
  (|CheckDeath_Enemy_2_2))

(event EventMeleeEnemyAttackTrace
  (bind _aggrocollision (Variables|Default|GetAggroCollision))
  (bind _returnvalue (Transformation|GetWorldLocation _aggrocollision))
  ;[1 1 1] Attacking
  (bind _outactors (Actor|GetAllActorsOfClass "/Game/Reign_Assets/EnemyObjects/Master_Enemy_BP/Master_Enemy_BP.Master_Enemy_BP_C"))
  (bind (_outhit _returnvalue_2) (Collision|SphereTraceForObjects _returnvalue _returnvalue (Variables|Default|GetAttackRadius) (Utilities|Array|MakeArray "ObjectTypeQuery3") false _outactors "None"))
  (if _returnvalue_2
    (Effects|SpawnEmitteratLocation "/Game/Reign_Assets/FX/Impacts/Impact1/Impact_1_FX.Impact_1_FX" (.ImpactPoint (Collision|BreakHitResult _outhit)))
    (Default|DealingDamage (Variables|Default|GetPlayerRef) (Variables|Default|GetMeleeDmg) self "None")))

(event EventDealingDamage
  (params (Sent%20Damage :type Integer) (Sender :type Actor%20Object%20Reference) (DamageType :type Name :default "None"))
  ;[1 1 1] Melee Enemy Damage Solver
  (Development|PrintString "Hello")
  (bind _returnvalue (Animation|GetCurrentMontage :!class /Script/Engine.Character))
  (Animation|StopAnimMontage _returnvalue)
  (Variables|Default|SetTakenDamage Sent%20Damage)
  (CallFunction|ShowHealthbar)
  (switch name DamageType
    (:Normal
      (Variables|Default|SetCurrentHealth (- (Variables|Default|GetCurrentHealth) (Variables|Default|GetTakenDamage)))
      (Animation|PlayAnimMontage (Variables|Default|GetHit%20Animation) 2.0 "None")
      (Physics|AddImpulse (Variables|Default|GetCapsuleComponent) (* (Math|Vector|GetForwardVector (Variables|/Script/Engine.Character|GetCapsuleComponent (Variables|Default|GetPlayerRef))) (Variables|Default|GetKnockBackStr)) "None" false)
      (CallFunction|UpdateHealth :!label _label)
      (|CheckDeath_Enemy_2_2))
    (:Special
      (Variables|Default|SetCurrentHealth (- (Variables|Default|GetCurrentHealth) (Variables|Default|GetTakenDamage)))
      (goto _label))
    (:Air
      (Variables|Default|SetCurrentHealth (- (Variables|Default|GetCurrentHealth) (Variables|Default|GetTakenDamage)))
      (Animation|PlayAnimMontage (Variables|Default|GetHit%20Animation) 1.0 "None")
      (goto _label))
    (:Grapple
      (bind _asmc_prototype_bp (Utilities|Casting|CastToMC_Prototype_BP (Game|GetPlayerCharacter 0)))
      (Variables|Default|SetPlayerRef _asmc_prototype_bp)
      (Variables|Default|SetPullActive? false)
      (Variables|Default|SetCurrentHealth (- (Variables|Default|GetCurrentHealth) (Variables|Default|GetTakenDamage)))
      (Variables|/Script/Engine.CharacterMovementComponent|SetGravityScale (Variables|Character|GetCharacterMovement) 0.0)
      (CallFunction|PullEvent)
      (Animation|PlayAnimMontage (Variables|Default|GetLinkedAnimation) 2.0 "None")
      (CallFunction|UpdateHealth))))

(event EventResetEnemy
  ;[1 1 1] Attacking
  (Variables|Default|SetPlayingAnimation? false)
  (Utilities|FlowControl|Delay (Variables|Default|GetAttackIntervalSpeed))
  (CallFunction|EnemyMeleeAttack))

(event EventPullEvent
  (bind _returnvalue (Transformation|GetActorLocation))
  (bind _playerref (Variables|Default|GetPlayerRef))
  (bind _aoe_point (Variables|/Game/Reign_Assets/Player_Character/Blueprints/MC_Prototype_BP.MC_Prototype_BP_C|GetAoE%20Point _playerref))
  (bind _returnvalue_2 (Transformation|GetWorldLocation _aoe_point))
  ;[1 1 1] Melee Enemy Damage Solver
  (if (Variables|Default|GetPullActive?)
    (CallFunction|StopPullEvent)
    (Variables|Default|SetPullActive? true)
    (elif (>= (Math|Vector|VectorLength (- (Transformation|GetActorLocation) (Transformation|GetWorldLocation (Variables|/Game/Reign_Assets/Player_Character/Blueprints/MC_Prototype_BP.MC_Prototype_BP_C|GetAoE%20Point (Variables|Default|GetPlayerRef))))) 55.0)
      (Transformation|SetActorLocation (Math|Interpolation|VInterpTo (Math|Vector|MakeVector (.x _returnvalue) (.y _returnvalue) (.z _returnvalue)) (Math|Vector|MakeVector (.x _returnvalue_2) (.y _returnvalue_2) (.z _returnvalue_2)) 0.01 7.0) false false)
      (Utilities|Time|SetTimerbyFunctionName 0 "Pull Event" 0.01)
      (else
        (CallFunction|StopPullEvent)))))

(fn ConstructionScript
  (|CallParentFunction)
  (Variables|Default|SetAIControllerClass "/Game/Reign_Assets/EnemyObjects/Master_Enemy_BP/MasterEnemy_AI/Tree_Tests/NewEnemyControl.NewEnemyControl_C"))