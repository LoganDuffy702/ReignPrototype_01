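; Melee human enemy that attacks the player with a montage and sphere trace, and reacts to melee, grapple and pull hits.
; DealingDamage routes hits by type, updating health and checking for death, which plays a random montage before destroying the actor.
; Grapple timelines lerp the player toward the enemy or the enemy toward the player while updating the weapon's chain beam.
; Older timer-based pull events also remain in the graph.
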(event Custom|Walk
  ;[1 1 1] Movement
  (Variables|/Script/Engine.CharacterMovementComponent|SetMaxWalkSpeed (Variables|Character|GetCharacterMovement) 3e+02))

(event Custom|Run
  ;[1 1 1] Movement
  (Variables|/Script/Engine.CharacterMovementComponent|SetMaxWalkSpeed (Variables|Character|GetCharacterMovement) 8e+02))

(event Custom|Enemies%20Not%20Getting%20Too%20Close)

(event Custom|EnemyMeleeAttack
  ;[1 1 1] Melee Attack
  (Variables|Default|SetAttacking? true)
  (Animation|PlayAnimMontage (Variables|Default|GetMeleeAtkAnimation) 1.0 "None")
  (Variables|Default|SetAttacking? false)
  (Utilities|FlowControl|Delay 2.0)
  (Components|Animation|SetAnimationMode (Variables|Character|GetMesh) "AnimationBlueprint"))

(event Custom|Check%20Death
  ;[1 1 1] Check Death
  (if (<= (Variables|Default|GetCurrentHealth) 1)
    (Components|Movement|StopMovementImmediately (Variables|Character|GetCharacterMovement))
    (bind _returnvalue (Animation|GetCurrentMontage :!class /Script/Engine.Character))
    (Animation|StopAnimMontage _returnvalue)
    (Variables|Default|SetIsAlive? false)
    (Collision|SetCollisionObjectType (Variables|Default|GetCapsuleComponent) "ECC_WorldStatic")
    (Animation|PlayAnimMontage (Utilities|Array|Get(acopy) (Variables|Default|GetDeathAnimation) (Math|Random|RandomIntegerinRange 0 2)) 1.0 "None")
    (Utilities|FlowControl|Delay 1.5)
    (CallFunction|DeathEvent)
    (Actor|DestroyActor)))

(event Custom|PullTo
  (bind _returnvalue (Transformation|GetActorLocation))
  (bind _playerref (Variables|Default|GetPlayerRef))
  (bind _aoe_point (Variables|/Game/Reign_Assets/Player_Character/Blueprints/MC_Prototype_BP.MC_Prototype_BP_C|GetAoE%20Point _playerref))
  (bind _returnvalue_2 (Transformation|GetWorldLocation _aoe_point))
  ;[1 1 1] Pull Enemy To Player Old Version
  (if (Variables|Default|GetPull%20Active?)
    (CallFunction|StopPullEvent)
    (Variables|Default|SetPull%20Active? true)
    (elif (>= (Math|Vector|VectorLength (- (Transformation|GetActorLocation) (Transformation|GetWorldLocation (Variables|/Game/Reign_Assets/Player_Character/Blueprints/MC_Prototype_BP.MC_Prototype_BP_C|GetAoE%20Point (Variables|Default|GetPlayerRef))))) 2e+02)
      (Transformation|SetActorLocation (Math|Interpolation|VInterpTo (Math|Vector|MakeVector (.x _returnvalue) (.y _returnvalue) (.z _returnvalue)) (Math|Vector|MakeVector (.x _returnvalue_2) (.y _returnvalue_2) (.z _returnvalue_2)) 0.01 7.0) false false)
      (Utilities|Time|SetTimerbyFunctionName 0 "PullTo" 0.01)
      (else
        (CallFunction|StopPullEvent)))))

(event Custom|Pull%20Player%20To%20Enemy
  (bind _returnvalue (Transformation|GetActorLocation))
  (bind _playerref (Variables|Default|GetPlayerRef))
  (bind _aoe_point (Variables|/Game/Reign_Assets/Player_Character/Blueprints/MC_Prototype_BP.MC_Prototype_BP_C|GetAoE%20Point _playerref))
  (bind _returnvalue_2 (Transformation|GetWorldLocation _aoe_point))
  ;[1 1 1] Pull Player To Enemy Old Version
  (if (Variables|Default|GetPull%20Active?)
    (CallFunction|StopPullEvent)
    (Variables|Default|SetPull%20Active? true)
    (elif (not (>= (Math|Vector|VectorLength (- (Transformation|GetWorldLocation (Variables|/Game/Reign_Assets/Player_Character/Blueprints/MC_Prototype_BP.MC_Prototype_BP_C|GetAoE%20Point (Variables|Default|GetPlayerRef))) (Transformation|GetActorLocation))) 55.0))
      (CallFunction|StopPullEvent)
      (Transformation|SetActorLocation (Variables|Default|GetPlayerRef) (Math|Interpolation|VInterpTo (Math|Vector|MakeVector (.x _returnvalue_2) (.y _returnvalue_2) (.z _returnvalue_2)) (Math|Vector|MakeVector (.x _returnvalue) (.y _returnvalue) (.z _returnvalue)) 0.01 7.0) false false)
      (Utilities|Time|SetTimerbyFunctionName 0 "Pull Player To Enemy" 0.01))))

(event Custom|MeleeDamgeTakenEvent
  ;[1 1 1] MeleeDamge Event
  (Variables|Default|SetCurrentHealth (- (Variables|Default|GetCurrentHealth) (Variables|Default|GetTakenDamage)))
  (Animation|PlayAnimMontage (Variables|Default|GetHit%20Animation) 2.0 "None")
  (CallFunction|UpdateHealth)
  (CallFunction|CheckDeath))

(event Custom|GrappleDamageEvent
  (bind _capsulecomponent (Variables|Default|GetCapsuleComponent))
  (bind _returnvalue (Transformation|GetWorldLocation _capsulecomponent))
  ;[1 1 1] PullTo Damage Event
  (Variables|Default|SetCurrentHealth (- (Variables|Default|GetCurrentHealth) (Variables|Default|GetTakenDamage)))
  (Variables|Default|SetPlayerLastLoc (Transformation|GetWorldLocation (Variables|/Script/Engine.Character|GetCapsuleComponent (Variables|Default|GetPlayerRef))))
  (bind _newtrack_0 (Timeline|PullToTimeline PlayFromStart)
    (:Update
      (Class|ParticleSystemComponent|SetBeamEndPoint (Variables|/Game/Reign_Assets/Weapon_BP/Master_Weapon_BP.Master_Weapon_BP_C|GetChainParticle (Variables|/Game/Reign_Assets/Player_Character/Blueprints/MC_Prototype_BP.MC_Prototype_BP_C|GetEquippedWeapon (Variables|Default|GetPlayerRef))) 0 (Transformation|GetWorldLocation (Variables|Default|GetChokePoint)))
      (Transformation|SetActorLocation (Variables|Default|GetPlayerRef) (Math|Vector|Lerp(Vector) (Math|Vector|MakeVector (.x (Variables|Default|GetPlayerLastLoc)) (.y (Variables|Default|GetPlayerLastLoc)) (.z _returnvalue)) (+ (* (Math|Vector|MakeVector (.x _returnvalue) (.y _returnvalue) (.z _returnvalue)) (/ 3.0 4.0)) (* (Math|Vector|MakeVector (.x (Variables|Default|GetPlayerLastLoc)) (.y (Variables|Default|GetPlayerLastLoc)) (.z _returnvalue)) (/ 1.0 4.0))) _newtrack_0) false false)
      (CallFunction|UpdateHealth)
      (CallFunction|CheckDeath))
    (:Finished
      (Default|WeaponReset (Variables|/Game/Reign_Assets/Player_Character/Blueprints/MC_Prototype_BP.MC_Prototype_BP_C|GetEquippedWeapon (Variables|Default|GetPlayerRef))))))

(event Custom|PullToDamageEvent
  (bind _playerref (Variables|Default|GetPlayerRef))
  (bind _aoe_point (Variables|/Game/Reign_Assets/Player_Character/Blueprints/MC_Prototype_BP.MC_Prototype_BP_C|GetAoE%20Point _playerref))
  (bind _returnvalue (Transformation|GetWorldLocation _aoe_point))
  ;[1 1 1] Grapple Damge Event
  (Variables|Default|SetCurrentHealth (- (Variables|Default|GetCurrentHealth) (Variables|Default|GetTakenDamage)))
  (Variables|Default|SetEnemyLastLoc (Transformation|GetWorldLocation (Variables|Default|GetCapsuleComponent)))
  (bind _newtrack_0 (Timeline|Timeline_1 PlayFromStart)
    (:Update
      (Class|ParticleSystemComponent|SetBeamEndPoint (Variables|/Game/Reign_Assets/Weapon_BP/Master_Weapon_BP.Master_Weapon_BP_C|GetChainParticle (Variables|/Game/Reign_Assets/Player_Character/Blueprints/MC_Prototype_BP.MC_Prototype_BP_C|GetEquippedWeapon (Variables|Default|GetPlayerRef))) 0 (Transformation|GetWorldLocation (Variables|Default|GetChokePoint)))
      (Transformation|SetActorLocation (Math|Vector|Lerp(Vector) (Math|Vector|MakeVector (.x (Variables|Default|GetEnemyLastLoc)) (.y (Variables|Default|GetEnemyLastLoc)) (.z (Variables|Default|GetEnemyLastLoc))) (+ (* (Math|Vector|MakeVector (.x _returnvalue) (.y _returnvalue) (+ (.z (Variables|Default|GetEnemyLastLoc)) 5e+01)) (/ 3.0 4.0)) (* (Math|Vector|MakeVector (.x (Variables|Default|GetEnemyLastLoc)) (.y (Variables|Default|GetEnemyLastLoc)) (.z (Variables|Default|GetEnemyLastLoc))) (/ 1.0 4.0))) _newtrack_0) false false)
      (CallFunction|UpdateHealth)
      (CallFunction|CheckDeath))
    (:Finished
      (Default|WeaponReset (Variables|/Game/Reign_Assets/Player_Character/Blueprints/MC_Prototype_BP.MC_Prototype_BP_C|GetEquippedWeapon (Variables|Default|GetPlayerRef))))))

(event Custom|Battle_Check
  (Variables|Default|SetIsInBattle? (Collision|IsOverlappingActor (Variables|/Game/Reign_Assets/Player_Character/Blueprints/MC_Prototype_BP.MC_Prototype_BP_C|GetBattle_Check (Variables|Default|GetPlayerRef)) self :!class /Script/Engine.PrimitiveComponent)))

(event EventBeginPlay
  (|CallParentFunction))

(event Collision|EventActorBeginOverlap
  (params (OtherActor :type Actor%20Object%20Reference)))

(event EventTick
  (params (DeltaSeconds :type Float%20%28single-precision%29))
  (|CallParentFunction DeltaSeconds)
  (CallFunction|BattleCheck))

(event EventMeleeEnemyAttackTrace
  (bind _aggrocollision (Variables|Default|GetAggroCollision))
  (bind _returnvalue (Transformation|GetWorldLocation _aggrocollision))
  ;[1 1 1] Attack Trace
  (bind _outactors (Actor|GetAllActorsOfClass "/Game/Reign_Assets/World_Objects/GrappleObjects/Master_Grapple_Object.Master_Grapple_Object_C"))
  (bind (_outhit _returnvalue_2) (Collision|SphereTraceForObjects _returnvalue _returnvalue (Variables|Default|GetAttackRadius) (Utilities|Array|MakeArray "ObjectTypeQuery3") false _outactors "None"))
  (if _returnvalue_2
    (Effects|SpawnEmitteratLocation "/Game/Reign_Assets/FX/Impacts/Impact1/Impact_1_FX.Impact_1_FX" (.ImpactPoint (Collision|BreakHitResult _outhit)))
    (Default|DealingDamage (Variables|Default|GetPlayerRef) (Variables|Default|GetMeleeDamage) self "None")))

(event EventDealingDamage
  (params (Sent%20Damage :type Integer) (Sender :type Actor%20Object%20Reference) (DamageType :type Name :default "None"))
  ;[1 1 1] Incoming Damage Solver
  (if (Variables|Default|GetCan%20Be%20Damaged?)
    (bind _returnvalue (Animation|GetCurrentMontage :!class /Script/Engine.Character))
    (Animation|StopAnimMontage _returnvalue)
    (Variables|Default|SetTakenDamage Sent%20Damage)
    (CallFunction|ShowHealthbar)
    (switch name DamageType
      (:Melee
        (CallFunction|MeleeDamgeTakenEvent))
      (:Grapple
        (Utilities|FlowControl|Delay 0.3)
        (CallFunction|GrappleDamageEvent))
      (:PullTo
        (Utilities|FlowControl|Delay 0.3)
        (CallFunction|PulltoDamageEvent)))))

(event EventResetEnemy
  ;[1 1 1] Reset enemy
  (Variables|Default|SetPlayingAnimation? false)
  (Utilities|FlowControl|Delay (Variables|Default|GetAttackIntervalSpeed))
  (CallFunction|EnemyMeleeAttack))

(event EventStopPullEvent
  (bind _playerref (Variables|Default|GetPlayerRef))
  (bind _charactermovement (Variables|/Script/Engine.Character|GetCharacterMovement _playerref))
  ;[1 1 1] Stop Pull
  (Variables|/Script/Engine.CharacterMovementComponent|SetGravityScale (Variables|Character|GetCharacterMovement) 1.0)
  (Variables|Default|SetPull%20Active? true)
  (Class|KismetSystemLibrary|PauseTimer 0 "PullTo")
  (Class|KismetSystemLibrary|PauseTimer 0 "Pull Player To Enemy")
  (Default|WeaponReset (Variables|/Game/Reign_Assets/Player_Character/Blueprints/MC_Prototype_BP.MC_Prototype_BP_C|GetEquippedWeapon _playerref))
  (Variables|/Script/Engine.CharacterMovementComponent|SetbOrientRotationToMovement _charactermovement true)
  (Variables|/Script/Engine.CharacterMovementComponent|SetbUseControllerDesiredRotation _charactermovement false))

(fn ConstructionScript
  (|CallParentFunction))