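; EnemyTower_BP is a stationary ranged enemy tower that shoots at the player and can be destroyed.
; Entering its attack collision starts a fast looping LookAt timer that aims CenterPoint at the player, with a debug-drawn trace showing the aim.
; After a short delay, a timer repeatedly spawns TowerProjectileBP from FirePoint until overlap ends.
; Damage briefly shows a widget health bar, and zero health triggers an explosion and destroys the tower.
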(event OnComponentBeginOverlap(CanAttackCollision)
  (params (OverlappedComponent :type Primitive%20Component%20Object%20Reference) (OtherActor :type Actor%20Object%20Reference) (OtherComp :type Primitive%20Component%20Object%20Reference) (OtherBodyIndex :type Integer) (bFromSweep :type Boolean) (SweepResult :type Hit%20Result%20Structure%20%28by%20ref%29))
  ;[1 1 1] Collisions
  (bind _asmc_prototype_bp (Utilities|Casting|CastToMC_Prototype_BP (Game|GetPlayerCharacter 0)))
  (Variables|Default|SetPlayerRef _asmc_prototype_bp)
  (CallFunction|TargetPlayer)
  (Variables|Default|SetCanFire? true)
  (Utilities|FlowControl|Delay 1.0)
  (CallFunction|Fire))

(event OnComponentEndOverlap(CanAttackCollision)
  (params (OverlappedComponent :type Primitive%20Component%20Object%20Reference) (OtherActor :type Actor%20Object%20Reference) (OtherComp :type Primitive%20Component%20Object%20Reference) (OtherBodyIndex :type Integer))
  ;[1 1 1] Collisions
  (Class|KismetSystemLibrary|PauseTimer 0 "TargetPlayer")
  (Variables|Default|SetCanFire? false)
  (Class|KismetSystemLibrary|PauseTimer 0 "Fire"))

(event Custom|Fire
  (bind _firepoint (Variables|Default|GetFirePoint))
  ;[1 1 1] Fireing
  (Game|SpawnActorfromClass "/Game/Reign_Assets/EnemyObjects/Ranged_Enemys/TowerProjectileBP.TowerProjectileBP_C" (Math|Transform|MakeTransform (Transformation|GetWorldLocation _firepoint) (Math|Conversions|RotationFromXVector (Math|Vector|GetRightVector (Transformation|GetWorldRotation _firepoint))) "0.100000,0.100000,0.500000") "Undefined" 0 0)
  (Utilities|Time|SetTimerbyFunctionName 0 "Fire" (Variables|Default|GetFire%20Interval)))

(event Custom|Lock%20On%20Event
  ;[1 1 1] Follow Player
)

(event Custom|TargetPlayer
  (bind _firepoint (Variables|Default|GetFirePoint))
  (bind _returnvalue (Transformation|GetWorldLocation _firepoint))
  ;[1 1 1] Follow Player
  (Transformation|SetWorldTransform (Variables|Default|GetCenterPoint) (Class|KismetAnimationLibrary|Lookat (Transformation|GetWorldTransform (Variables|Default|GetCenterPoint)) (Transformation|GetWorldLocation (Variables|/Script/Engine.Character|GetCapsuleComponent (Variables|Default|GetPlayerRef))) "0,1.000000, 0" false "0, 0, 0" 0.0) false false)
  (Collision|LineTraceByChannel _returnvalue (- _returnvalue (* (Math|Vector|GetRightVector (Transformation|GetWorldRotation _firepoint)) -2000)) "TraceTypeQuery1" false 0 "ForDuration" true "(R=1.000000,G=0.000000,B=0.000000,A=1.000000)" "(R=0.000000,G=1.000000,B=0.000000,A=1.000000)" 0.1)
  (Utilities|Time|SetTimerbyFunctionName 0 "TargetPlayer" 0.01 true))

(event Custom|Show%20HealthBar
  (Rendering|SetVisibility (Variables|Default|GetTowerHealth) true false)
  (Utilities|FlowControl|Delay 2.0)
  (CallFunction|HideHealthbar))

(event Custom|Hide%20Healthbar
  (Rendering|SetVisibility (Variables|Default|GetTowerHealth) false false))

(event EventBeginPlay
  (Variables|Default|SetCurrentHealth (Variables|Default|GetMaxHealth))
  (CallFunction|UpdateHealth))

(event EventDealingDamage
  (params (Damage :type Integer) (Sender :type Actor%20Object%20Reference))
  ;[1 1 1] Delt damage
  (Variables|Default|SetCurrentHealth (- (Variables|Default|GetCurrentHealth) Damage))
  (CallFunction|ShowHealthBar)
  (CallFunction|UpdateHealth)
  (CallFunction|CheckDeath))

(fn ConstructionScript)

(fn UpdateHealth
  (bind _asenemy_health (Utilities|Casting|CastToEnemyHealth (UserInterface|GetUserWidgetObject (Variables|Default|GetTowerHealth))))
  (Progress|SetPercent (Variables|/Game/Reign_Assets/EnemyObjects/EnemyHealth.EnemyHealth_C|GetEnemyHealth _asenemy_health) (/ (Math|Conversions|ToFloat(Integer) (Variables|Default|GetCurrentHealth)) (Math|Conversions|ToFloat(Integer) (Variables|Default|GetMaxHealth))))
  (return))

(fn CheckDeath
  (if (<= (Variables|Default|GetCurrentHealth) 0)
    (Effects|SpawnEmitteratLocation "/Game/StarterContent/Particles/P_Explosion.P_Explosion" (Transformation|GetWorldLocation (Variables|Default|GetCenterPoint)))
    (Actor|DestroyActor)))