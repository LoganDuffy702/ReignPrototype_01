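; Ranged tower enemy projectile that damages the player character on contact and removes itself after a five-second lifetime.
; Any Sphere overlap spawns an impact effect at the sweep's impact point and destroys the actor, provided the player pawn casts to MC_Prototype_BP.
; If the overlapped actor is that player, it also calls DealingDamage with the projectile's Damage value, just after DestroyActor.
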(event OnComponentBeginOverlap(Sphere)
  (params (OverlappedComponent :type Primitive%20Component%20Object%20Reference) (OtherActor :type Actor%20Object%20Reference) (OtherComp :type Primitive%20Component%20Object%20Reference) (OtherBodyIndex :type Integer) (bFromSweep :type Boolean) (SweepResult :type Hit%20Result%20Structure%20%28by%20ref%29))
  (bind _impactpoint (Collision|BreakHitResult SweepResult))
  (bind _asmc_prototype_bp (Utilities|Casting|CastToMC_Prototype_BP (Game|GetPlayerCharacter 0)))
  (if (== OtherActor _asmc_prototype_bp)
    (Effects|SpawnEmitteratLocation "/Game/Reign_Assets/FX/Impacts/Impact1/Impact_1_FX.Impact_1_FX" _impactpoint)
    (Actor|DestroyActor)
    (Default|DealingDamage _asmc_prototype_bp (Variables|Default|GetDamage))
    (else
      (Effects|SpawnEmitteratLocation "/Game/Reign_Assets/FX/Impacts/Impact1/Impact_1_FX.Impact_1_FX" _impactpoint)
      (Actor|DestroyActor))))

(event Custom|killme
  (Actor|DestroyActor))

(event EventBeginPlay
  (Utilities|FlowControl|Delay 5.0)
  (CallFunction|Killme))

(event Collision|EventActorBeginOverlap
  (params (OtherActor :type Actor%20Object%20Reference)))

(event EventTick
  (params (DeltaSeconds :type Float%20%28single-precision%29)))

(fn ConstructionScript)