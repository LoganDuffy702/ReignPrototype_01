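; Mortar projectile Blueprint for a static enemy, which explodes on overlap and damages the player.
; The construction script feeds Speed and StartVelocity into its ProjectileMovement component.
; Sphere overlap spawns an explosion and traces a radius for Pawns; any hit damages player character 0 through MC_Prototype_BP's DealingDamage, even if the Pawn found is not the player.
; The shell destroys itself after impact or a timed lifespan from BeginPlay.
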(event OnComponentBeginOverlap(Sphere)
  (params (OverlappedComponent :type Primitive%20Component%20Object%20Reference) (OtherActor :type Actor%20Object%20Reference) (OtherComp :type Primitive%20Component%20Object%20Reference) (OtherBodyIndex :type Integer) (bFromSweep :type Boolean) (SweepResult :type Hit%20Result%20Structure%20%28by%20ref%29))
  (bind _returnvalue (Transformation|GetActorLocation))
  (Effects|SpawnEmitteratLocation "/Game/StarterContent/Particles/P_Explosion.P_Explosion" (Transformation|GetActorLocation) "0, 0, 0" "3.000000,3.000000,3.000000")
  (bind _returnvalue_2 (Collision|SphereTraceForObjects _returnvalue _returnvalue 2.5e+02 (Utilities|Array|MakeArray "ObjectTypeQuery3") false (Utilities|Array|MakeArray self) "None" true "(R=1.000000,G=0.000000,B=0.000000,A=1.000000)" "(R=0.000000,G=1.000000,B=0.000000,A=1.000000)" 1.0))
  (if _returnvalue_2
    (bind _asmc_prototype_bp (Utilities|Casting|CastToMC_Prototype_BP (Game|GetPlayerCharacter 0)))
    (Default|DealingDamage _asmc_prototype_bp 3 0 "None")
    (CallFunction|KillMe)
    (else
      (CallFunction|KillMe))))

(event Custom|Kill%20Me
  (Actor|DestroyActor))

(event EventBeginPlay
  (Utilities|FlowControl|Delay 7.0)
  (CallFunction|KillMe))

(fn ConstructionScript
  (bind _projectilemovement (Variables|Default|GetProjectileMovement))
  (bind _speed (Variables|Default|GetSpeed))
  (Variables|/Script/Engine.ProjectileMovementComponent|SetInitialSpeed _projectilemovement _speed)
  (Variables|/Script/Engine.ProjectileMovementComponent|SetMaxSpeed _projectilemovement _speed)
  (Variables|/Script/Engine.MovementComponent|SetVelocity _projectilemovement (Variables|Default|GetStartVelocity)))