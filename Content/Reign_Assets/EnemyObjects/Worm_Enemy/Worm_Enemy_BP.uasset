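; Worm enemy that faces the player, relocates by random launches and fires projectiles.
; First player overlap starts relocation, then timers and Enter/Attacking flags drive the attack cycle, with Shoot and collision toggles exposed as events.
; Hits land only while lockable, deal flat damage and branch by type into melee reaction, air juggle, stun, grapple pulling the player in, or meteor slam.
; Death plays an exit montage, then destroys the actor.
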(event OnComponentBeginOverlap(AgroCheckPlayer)
  (params (OverlappedComponent :type Primitive%20Component%20Object%20Reference) (OtherActor :type Actor%20Object%20Reference) (OtherComp :type Primitive%20Component%20Object%20Reference) (OtherBodyIndex :type Integer) (bFromSweep :type Boolean) (SweepResult :type Hit%20Result%20Structure%20%28by%20ref%29))
  (Utilities|Casting|CastToMC_Prototype_BP OtherActor)
  (Utilities|FlowControl|DoOnce false
    (:Completed
      (Utilities|FlowControl|Delay (Math|Random|RandomFloatinRange 1.0 2.0))
      (CallFunction|FindRandomLocation))))

(event Custom|Find%20Random%20Location
  ;[1 1 1] Go To The Random Location
  (Character|LaunchCharacter (Math|Vector|MakeVector (Math|Random|RandomFloatinRange -3e+03 3e+03) (Math|Random|RandomFloatinRange -3e+03 3e+03) 0.0) false false)
  (Utilities|FlowControl|Delay 1.0)
  (Components|Movement|StopMovementImmediately (Variables|Character|GetCharacterMovement))
  (Variables|Default|SetEnter? true)
  (Effects|SpawnEmitteratLocation "/Game/Reign_Assets/EnemyObjects/Worm_Enemy/Worm_FX/Worm_Ground_FX.Worm_Ground_FX" (Transformation|GetActorLocation))
  (Utilities|Time|SetTimerbyFunctionName 0 "Trigger Fire" (Variables|Default|GetPre%20Attack%20Duration)))

(event Custom|WaitForNextAtk
  ;[1 1 1] Wait Timer
  (Variables|Default|SetEnter? false)
  (Utilities|Time|SetTimerbyFunctionName 0 "Find Random Location" (Variables|Default|GetHide%20Duration)))

(event Custom|Death%20Final
  ;[1 1 1] Check Death
  (CallFunction|DeathEvent)
  (Actor|DestroyActor))

(event Custom|Disable%20Collision
  (CallFunction|HideHealthBar)
  (Collision|SetCollisionResponsetoChannel (Variables|Default|GetCapsuleComponent) "ECC_Pawn" "ECR_Ignore")
  (Variables|Default|SetCanBeLockedOn? false)
  (Rendering|SetVisibility (Variables|Default|GetLockOnWidget) false false))

(event Custom|Activate%20Collision
  (CallFunction|HideHealthBar)
  (Collision|SetCollisionResponsetoChannel (Variables|Default|GetCapsuleComponent) "ECC_Pawn" "ECR_Block")
  (Variables|Default|SetCanBeLockedOn? true)
  (Rendering|SetVisibility (Variables|Default|GetLockOnWidget) true false))

(event Custom|WormAirCombat
  ;[1 1 1] Air combat
  (Variables|/Script/Engine.SkeletalMeshComponent|SetbPauseAnims (Variables|Character|GetMesh) true)
  (CallFunction|UpdateHealth)
  (CallFunction|CheckDeath)
  (|JuggleNode (Variables|Character|GetCharacterMovement) (Variables|Character|GetMesh)))

(event Custom|Meteor
  (bind _charactermovement (Variables|Character|GetCharacterMovement))
  ;[1 1 1] Meteor
  (Variables|/Script/Engine.CharacterMovementComponent|SetGravityScale _charactermovement 2.5)
  (Variables|/Script/Engine.MovementComponent|SetVelocity _charactermovement "0, 0, 0")
  (if (AI|Components|NavMovement|IsFalling _charactermovement) :!label _label
    (Transformation|AddWorldOffset (Variables|Default|GetCapsuleComponent) "0, 0,-100.000000" false false)
    (Utilities|FlowControl|Delay 0.01)
    (goto _label)
    (else
      (Audio|PlaySoundatLocation "/Game/StarterContent/Audio/Explosion_Cue.Explosion_Cue" (stale Collision|EventHit HitLocation) "0, 0, 0" 1.0 1.0 0.0 0 0 0)
      (Effects|SpawnEmitteratLocation "/Game/Reign_Assets/EnemyObjects/DummyEnemy/Enemy_Slam_Dmg_FX.Enemy_Slam_Dmg_FX" (stale Collision|EventHit HitLocation) "0, 0, 0" "2.500000,2.500000,2.500000"))))

(event Custom|Shoot
  (bind _shoot_point (Variables|Default|GetShoot%20Point))
  ;[1 1 1] Fire At Player
  (Game|SpawnActorfromClass "/Game/Reign_Assets/EnemyObjects/Worm_Enemy/Worm_Projectile_BP.Worm_Projectile_BP_C" (Math|Transform|MakeTransform (Transformation|GetWorldLocation _shoot_point) (Math|Conversions|RotationFromXVector (Math|Vector|GetForwardVector (Transformation|GetWorldRotation _shoot_point))) "0.500000,0.500000,0.500000") "Undefined" 0 0))

(event Custom|Check%20Death
  ;[1 1 1] Check Death
  (if (<= (Variables|Default|GetCurrentHealth) 0)
    (Components|Movement|StopMovementImmediately (Variables|Character|GetCharacterMovement))
    (Animation|Montage|PlayMontage (Variables|Character|GetMesh) "/Game/Reign_Assets/EnemyObjects/Worm_Enemy/Mesh/Worm_Animations/Worm_Exit_Montage.Worm_Exit_Montage"
      (:then
        (Collision|SetCollisionObjectType (Variables|Default|GetCapsuleComponent) "ECC_WorldStatic"))
      (:OnCompleted
        (CallFunction|DeathEvent)
        (Actor|DestroyActor)))))

(event Custom|Check%20Location%20Avaliable
  ;[1 1 1] Check If New Location is Possible
  (bind (_outhit _returnvalue) (Collision|LineTraceByChannel (Math|Vector|MakeVector (.x (Variables|Default|GetNew%20Enemy%20Location)) (.y (Variables|Default|GetNew%20Enemy%20Location)) (+ (.z (Variables|Default|GetNew%20Enemy%20Location)) 1e+03)) (Math|Vector|MakeVector (.x (Variables|Default|GetNew%20Enemy%20Location)) (.y (Variables|Default|GetNew%20Enemy%20Location)) (- (.z (Variables|Default|GetNew%20Enemy%20Location)) 1e+03)) "TraceTypeQuery1" false (Utilities|Array|MakeArray self) "None"))
  (if _returnvalue
    (Variables|Default|SetNew%20Enemy%20Location (+ (.Location (Collision|BreakHitResult _outhit)) "0, 0,50.000000"))
    (Variables|Default|SetEnter? true)
    (else
      (CallFunction|GetRandomLocationAroundPlayer))))

(event Custom|Get%20Random%20Location%20Around%20Player
  (bind _playerref (Variables|Default|GetPlayerRef))
  ;[1 1 1] Get Random Location
  (if (AI|Components|NavMovement|IsFalling (Variables|/Script/Engine.Character|GetCharacterMovement (Variables|Default|GetPlayerRef)))
    (bind _output_get (Variables|Default|SetPlayer%20Location (Transformation|GetActorLocation _playerref)))
    (Variables|Default|SetNew%20Enemy%20Location (Math|Vector|MakeVector (+ (Math|Random|RandomFloatinRange -1e+03 1e+03) (.x _output_get)) (+ (Math|Random|RandomFloatinRange -1e+03 1e+03) (.y _output_get)) (.z (Transformation|GetActorLocation self))))
    (CallFunction|CheckLocationAvaliable)
    (else
      (bind _output_get_2 (Variables|Default|SetPlayer%20Location (Transformation|GetActorLocation _playerref)))
      (Variables|Default|SetNew%20Enemy%20Location (Math|Vector|MakeVector (+ (Math|Random|RandomFloatinRange -1e+03 1e+03) (.x _output_get_2)) (+ (Math|Random|RandomFloatinRange -1e+03 1e+03) (.y _output_get_2)) (.z _output_get_2)))
      (CallFunction|CheckLocationAvaliable))))

(event Custom|MeleeDamgeTakenEvent
  ;[1 1 1] MeleeDamge Event
  (Animation|PlayAnimMontage (Variables|Default|GetHit%20Animation) 2.0 "None")
  (CallFunction|UpdateHealth)
  (CallFunction|CheckDeath))

(event Custom|StunDamageEvent
  ;[1 1 1] Grapple Damge Event
  (Variables|Default|SetConfused? true)
  (Effects|SpawnEmitteratLocation "/Game/Reign_Assets/EnemyObjects/Worm_Enemy/Worm_FX/Worm_Confused_FX.Worm_Confused_FX" (+ (Transformation|GetWorldLocation (Variables|Default|GetCapsuleComponent)) "0, 0,250.000000"))
  (CallFunction|UpdateHealth)
  (CallFunction|CheckDeath)
  (Utilities|FlowControl|RetriggerableDelay 2.0)
  (Variables|Default|SetConfused? false)
  (CallFunction|WaitforNextAtk))

(event Custom|PullToDamageEvent
  (bind _capsulecomponent (Variables|Default|GetCapsuleComponent))
  (bind _returnvalue (Transformation|GetWorldLocation _capsulecomponent))
  ;[1 1 1] PullTo Damage Event
  (Variables|Default|SetPlayerLastLoc (Transformation|GetActorLocation (Variables|Default|GetPlayerRef)))
  (bind _newtrack_0 (Timeline|Timeline_0 PlayFromStart)
    (:Update
      (Class|ParticleSystemComponent|SetBeamEndPoint (Variables|/Game/Reign_Assets/Weapon_BP/Master_Weapon_BP.Master_Weapon_BP_C|GetChainParticle (Variables|/Game/Reign_Assets/Player_Character/Blueprints/MC_Prototype_BP.MC_Prototype_BP_C|GetEquippedWeapon (Variables|Default|GetPlayerRef))) 0 (Transformation|GetWorldLocation (Variables|Default|GetChokePoint)))
      (Transformation|SetActorLocation (Variables|Default|GetPlayerRef) (Math|Vector|Lerp(Vector) (Math|Vector|MakeVector (.X (Math|Vector|BreakVector (Variables|Default|GetPlayerLastLoc))) (.Y (Math|Vector|BreakVector (Variables|Default|GetPlayerLastLoc))) (.Z (Math|Vector|BreakVector (Variables|Default|GetPlayerLastLoc)))) (+ (* (Math|Vector|MakeVector (.x _returnvalue) (.y _returnvalue) (+ (.z _returnvalue) 1.5e+02)) (/ 3.0 4.0)) (* (Math|Vector|MakeVector (.X (Math|Vector|BreakVector (Variables|Default|GetPlayerLastLoc))) (.Y (Math|Vector|BreakVector (Variables|Default|GetPlayerLastLoc))) (.Z (Math|Vector|BreakVector (Variables|Default|GetPlayerLastLoc)))) (/ 1.0 4.0))) _newtrack_0) false false)
      (CallFunction|UpdateHealth)
      (CallFunction|CheckDeath))
    (:Finished
      (Default|WeaponReset (Variables|/Game/Reign_Assets/Player_Character/Blueprints/MC_Prototype_BP.MC_Prototype_BP_C|GetEquippedWeapon (Variables|Default|GetPlayerRef))))))

(event Custom|Trigger%20Fire
  ;[1 1 1] Go To The Random Location
  (Variables|Default|SetAttacking? true))

(event EventBeginPlay
  (|CallParentFunction)
  (Variables|Default|SetOriginal%20Location (Transformation|GetActorLocation self))
  (Variables|Default|SetEnter? false)
  (Variables|Default|SetCanBeLockedOn? false)
  (CallFunction|DisableCollision))

(event Collision|EventHit
  (params (MyComp :type Primitive%20Component%20Object%20Reference) (Other :type Actor%20Object%20Reference) (OtherComp :type Primitive%20Component%20Object%20Reference) (bSelfMoved :type Boolean) (HitLocation :type Vector :default "0, 0, 0") (HitNormal :type Vector :default "0, 0, 0") (NormalImpulse :type Vector :default "0, 0, 0") (Hit :type Hit%20Result%20Structure%20%28by%20ref%29))
  ;[1 1 1] Meteor
)

(event EventTick
  (params (DeltaSeconds :type Float%20%28single-precision%29))
  (bind _capsulecomponent (Variables|Default|GetCapsuleComponent))
  (bind _shoot_point (Variables|Default|GetShoot%20Point))
  (bind _returnvalue (Transformation|GetWorldRotation _capsulecomponent))
  (|CallParentFunction DeltaSeconds)
  (Transformation|SetActorRotation (Math|Rotator|MakeRotator (.roll _returnvalue) (.pitch _returnvalue) (.yaw (Math|Rotator|FindLookatRotation (Transformation|GetWorldLocation _capsulecomponent) (Transformation|GetActorLocation (Variables|Default|GetPlayerRef))))))
  (Transformation|SetWorldRotation _shoot_point (Math|Rotator|FindLookatRotation (Transformation|GetWorldLocation _shoot_point) (Transformation|GetActorLocation (Variables|Default|GetPlayerRef))) false false))

(event EventDealingDamage
  (params (Sent%20Damage :type Integer) (Sender :type Actor%20Object%20Reference) (DamageType :type Name :default "None"))
  ;[1 1 1] Damage Solver
  (if (Variables|Default|GetCanBeLockedOn?)
    (CallFunction|PlayImpactSound)
    (bind _returnvalue (Animation|GetCurrentMontage :!class /Script/Engine.Character))
    (Animation|StopAnimMontage _returnvalue)
    (Variables|Default|SetTakenDamage Sent%20Damage)
    (CallFunction|ShowHealthbar)
    (Variables|Default|SetCurrentHealth (- (Variables|Default|GetCurrentHealth) 25))
    (CallFunction|CheckDeath)
    (switch name DamageType
      (:Melee
        (CallFunction|MeleeDamgeTakenEvent))
      (:Special
        (CallFunction|WormAirCombat)
        (CallFunction|StunDamageEvent))
      (:AIR
        (CallFunction|WormAirCombat))
      (:Grapple
        (CallFunction|PulltoDamageEvent))
      (:PullTo
        (CallFunction|StunDamageEvent))
      (:Meteor
        (CallFunction|Meteor)
        (CallFunction|StunDamageEvent)))))

(fn ConstructionScript
  (|CallParentFunction))