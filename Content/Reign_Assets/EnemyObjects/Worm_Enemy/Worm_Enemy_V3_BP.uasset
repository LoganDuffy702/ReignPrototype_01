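; Worm enemy character that roams until something overlaps its sphere, then turns toward the player and plays an attack montage.
; A looping event picks a new roam vector every four seconds around the player's starting location, and Tick feeds it into movement input until aggroed.
; FireProjectile aims Firepoint at the player and spawns a worm projectile, with no caller in this graph.
; DealingDamage delegates to LogansDamageComponent; the HP-decrement chain is disconnected.
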(event OnComponentBeginOverlap(Sphere)
  (params (OverlappedComponent :type Primitive%20Component%20Object%20Reference) (OtherActor :type Actor%20Object%20Reference) (OtherComp :type Primitive%20Component%20Object%20Reference) (OtherBodyIndex :type Integer) (bFromSweep :type Boolean) (SweepResult :type Hit%20Result%20Structure%20%28by%20ref%29))
  (Variables|Default|SetAgroed? true)
  (Variables|Default|SetLast%20Rot (.yaw (Transformation|GetWorldRotation (Variables|Collision|GetCapsuleComponent))))
  (bind _newtrack_0 (Timeline|Timeline_0 PlayFromStart)
    (:Update
      (Transformation|SetWorldRotation (Variables|Collision|GetCapsuleComponent) (Math|Rotator|MakeRotator 0.0 0.0 (Math|Float|Lerp (Variables|Default|GetLast%20Rot) (.yaw (Math|Rotator|FindLookatRotation (Transformation|GetWorldLocation (Variables|Collision|GetCapsuleComponent)) (Transformation|GetActorLocation (Variables|Default|GetPlayer%20Ref)))) _newtrack_0)) false false))
    (:Finished
      (Animation|PlayAnimMontage "/Game/Reign_Assets/EnemyObjects/Worm_Enemy/Mesh/Worm_Animations/Worm_Attack_1_Montage.Worm_Attack_1_Montage" 1.0 "None"))))

(event Custom|CheckHealth
  (if (<= (Variables|Default|GetCurrent%20HP) 0.0)
    (Variables|Default|SetAlive? false)))

(event Custom|Find%20Random%20Loc%20Event
  (bind _direction_vector (CallFunction|RoamFunction (Variables|Default|GetOrigin) -1e+03 1e+03 :!label _label))
  (Variables|Default|SetDirection%20Vector _direction_vector)
  (Utilities|FlowControl|Delay 4.0)
  (goto _label))

(event EventBeginPlay
  (bind _asmc_prototype_bp (Utilities|Casting|CastToMC_Prototype_BP (Game|GetPlayerCharacter 0)))
  (bind _output_get (Variables|Default|SetPlayer%20Ref _asmc_prototype_bp))
  (Variables|Default|SetOrigin (Transformation|GetActorLocation _output_get))
  (CallFunction|FindRandomLocEvent))

(event EventTick
  (params (DeltaSeconds :type Float%20%28single-precision%29))
  (if (not (Variables|Default|GetAgroed?))
    (Pawn|Input|AddMovementInput (Variables|Default|GetDirection%20Vector) 1.0 false)))

(event EventDealingDamage
  (params (Sent%20Damage :type Integer) (Sender :type Actor%20Object%20Reference) (DamageType :type Name :default "None"))
  (Default|LogansDmgSolver (Variables|Default|GetLogans_Damage_Component) DamageType 1.0 self 0.0 0.0))

(fn ConstructionScript)

(fn FireProjectile
  (bind _firepoint (Variables|Default|GetFirepoint))
  (bind _returnvalue (Transformation|GetWorldTransform _firepoint))
  (Transformation|SetWorldRotation (Variables|Default|GetFirepoint) (Math|Rotator|MakeRotator 0.0 0.0 (.yaw (Math|Rotator|FindLookatRotation (Transformation|GetWorldLocation (Variables|Default|GetFirepoint)) (Transformation|GetActorLocation (Variables|Default|GetPlayer%20Ref))))) false false)
  (Game|SpawnActorfromClass "/Game/Reign_Assets/EnemyObjects/Worm_Enemy/Worm_Projectile_BP.Worm_Projectile_BP_C" (Math|Transform|MakeTransform (.location _returnvalue) (.rotation _returnvalue) "0.700000,0.700000,0.700000") "Undefined" 0 0))

(fn FindNewLoc)