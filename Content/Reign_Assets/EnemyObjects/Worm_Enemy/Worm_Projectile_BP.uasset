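; Projectile fired by the Worm enemy that damages the player character on contact.
; On BeginPlay it caches the player reference and destroys itself after a five-second lifetime.
; Sphere overlap with the player spawns an impact effect and deals damage, while any blocking hit only spawns the effect.
; Both cases stop movement, hide the mesh, disable collision and destroy the actor immediately.
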(event OnComponentHit(Sphere)
  (params (HitComponent :type Primitive%20Component%20Object%20Reference) (OtherActor :type Actor%20Object%20Reference) (OtherComp :type Primitive%20Component%20Object%20Reference) (NormalImpulse :type Vector :default "0, 0, 0") (Hit :type Hit%20Result%20Structure%20%28by%20ref%29))
  (Effects|SpawnEmitteratLocation "/Game/Reign_Assets/FX/Impacts/Impact1/Impact_1_FX.Impact_1_FX" (.ImpactPoint (Collision|BreakHitResult Hit)))
  (Components|Movement|StopMovementImmediately (Variables|Default|GetProjectileMovement))
  (Rendering|SetVisibility (Variables|Default|GetCylinder1) false false)
  (Collision|SetCollisionEnabled (Variables|Default|GetSphere) "NoCollision")
  (Actor|DestroyActor))

(event OnComponentBeginOverlap(Sphere)
  (params (OverlappedComponent :type Primitive%20Component%20Object%20Reference) (OtherActor :type Actor%20Object%20Reference) (OtherComp :type Primitive%20Component%20Object%20Reference) (OtherBodyIndex :type Integer) (bFromSweep :type Boolean) (SweepResult :type Hit%20Result%20Structure%20%28by%20ref%29))
  (if (== (Variables|Default|GetPlayerRef) OtherActor)
    (Effects|SpawnEmitteratLocation "/Game/Reign_Assets/FX/Impacts/Impact1/Impact_1_FX.Impact_1_FX" (.ImpactPoint (Collision|BreakHitResult SweepResult)))
    (Default|DealingDamage (Variables|Default|GetPlayerRef) (Variables|Default|GetDamage) 0 "None")
    (Components|Movement|StopMovementImmediately (Variables|Default|GetProjectileMovement))
    (Rendering|SetVisibility (Variables|Default|GetCylinder1) false false)
    (Collision|SetCollisionEnabled (Variables|Default|GetSphere) "NoCollision")
    (Actor|DestroyActor)))

(event Custom|killme
  (Actor|DestroyActor))

(event EventBeginPlay
  (bind _asmc_prototype_bp (Utilities|Casting|CastToMC_Prototype_BP (Game|GetPlayerCharacter 0)))
  (Variables|Default|SetPlayerRef _asmc_prototype_bp)
  (Utilities|FlowControl|Delay 5.0)
  (CallFunction|Killme))

(event Collision|EventActorBeginOverlap
  (params (OtherActor :type Actor%20Object%20Reference)))

(event EventTick
  (params (DeltaSeconds :type Float%20%28single-precision%29)))

(fn ConstructionScript)