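; BossMaster is a Wrath boss Blueprint, apparently a base class, that sets health and deals contact damage to the player.
; BeginPlay caches the player character and sets Health to MaxHealth.
; Right arm overlap with the player sends a fixed damage message, while the left arm overlap event is empty.
; A helper function returns the boss's distance to the player, and Tick does nothing.
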(event OnComponentBeginOverlap(RightArm)
  (params (OverlappedComponent :type Primitive%20Component%20Object%20Reference) (OtherActor :type Actor%20Object%20Reference) (OtherComp :type Primitive%20Component%20Object%20Reference) (OtherBodyIndex :type Integer) (bFromSweep :type Boolean) (SweepResult :type Hit%20Result%20Structure%20%28by%20ref%29))
  (if (or (== OtherActor (Variables|Default|GetPlayer)) (== (stale OnComponentBeginOverlap(LeftArm) OtherActor) (Variables|Default|GetPlayer)))
    (Class|HealthDamageInterface|DealingDamage(Message) (Variables|Default|GetPlayer) 10 0 "None")))

(event OnComponentBeginOverlap(LeftArm)
  (params (OverlappedComponent :type Primitive%20Component%20Object%20Reference) (OtherActor :type Actor%20Object%20Reference) (OtherComp :type Primitive%20Component%20Object%20Reference) (OtherBodyIndex :type Integer) (bFromSweep :type Boolean) (SweepResult :type Hit%20Result%20Structure%20%28by%20ref%29)))

(event EventBeginPlay
  (Variables|Default|SetPlayer (Game|GetPlayerCharacter 0))
  (Variables|Default|SetHealth (Variables|Default|GetMaxHealth)))

(event Collision|EventActorBeginOverlap
  (params (OtherActor :type Actor%20Object%20Reference)))

(event EventTick
  (params (DeltaSeconds :type Float%20%28single-precision%29)))

(fn ConstructionScript)

(fn GetDistancetoPlayer
  (return (Math|Float|Absolute(Float) (Math|Vector|VectorLength (- (Transformation|GetActorLocation) (Transformation|GetActorLocation (Variables|Default|GetPlayer)))))))