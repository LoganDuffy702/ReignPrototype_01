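; Handler for the Wrath boss that triggers timed enemy spawns through the level's BossEnemySpawner actors.
; On BeginPlay it caches all spawners, and SpawnEnemies sets a target count and starts a looping timer at the given rate.
; Each tick calls SpawnEnemy on a random spawner until EnemiesSpawned, which is not updated here, equals the target, then clears the timer and sets IsFinished.
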(event Custom|SpawnEnemies
  (params (NumOfEnemies :type Integer) (Spawn%20Rate :type Float%20%28single-precision%29))
  (Variables|Default|SetNumOfEnemies NumOfEnemies)
  (Variables|Default|SetIsFinished false)
  (bind _returnvalue (Utilities|Time|SetTimerbyEvent (delegate Custom|StartToSpawnEnemy) Spawn%20Rate true))
  (Variables|Default|SetTimer%20Hamdler _returnvalue))

(event Custom|StartToSpawnEnemy
  ;[1 1 1] Spawns in an enemy
  (if (== (Variables|Default|GetNumOfEnemies) (Variables|Default|GetEnemiesSpawned))
    (Variables|Default|SetIsFinished true)
    (Utilities|Time|ClearandInvalidateTimerbyHandle (Variables|Default|GetTimer%20Hamdler))
    (else
      (bind _result (Math|Integer|DecrementInt (Utilities|Array|Length (Variables|Default|GetSpawners)))
        (:%20%20
          (Default|SpawnEnemy (Utilities|Array|Get(acopy) (Variables|Default|GetSpawners) (Math|Random|RandomIntegerinRange 0 _result))))))))

(event EventBeginPlay
  (bind _outactors (Actor|GetAllActorsOfClass "/Game/Reign_Assets/EnemyObjects/Wrath_Boss/Blueprints/BossEnemySpawner.BossEnemySpawner_C"))
  (Variables|Default|SetSpawners _outactors))

(fn ConstructionScript)