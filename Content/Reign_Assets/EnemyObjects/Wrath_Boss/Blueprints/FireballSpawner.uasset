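; Wrath boss spawner actor that emits a row of Fireball actors one at a time, starting on BeginPlay.
; SpawnFireballs stores the count and start position, then runs a looping timer on SpawnFireball.
; Each tick steps the position along world Y and spawns a Fireball with the spawner's rotation and scale.
; Once the count is reached, it clears the timer, resets the counter and flags spawning as finished.
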(event Custom|SpawnFireballs
  (params (NumOfFireballs :type Integer) (SpawnRate :type Float%20%28single-precision%29) (StartingPosition :type Vector))
  ;[1 1 1] Loop Event to Spawn Fireballs
  (Variables|Default|SetisFinishedWithSpawning false)
  (Variables|Default|SetStartingPosition StartingPosition)
  (Variables|Default|SetNumOfFireballs NumOfFireballs)
  (bind _returnvalue (Utilities|Time|SetTimerbyEvent (delegate Custom|SpawnFireball) SpawnRate true))
  (Variables|Default|SetTimerHandle _returnvalue))

(event Custom|SpawnFireball
  (bind _returnvalue (Transformation|GetActorTransform))
  ;[1 1 1] Spawning Fireball Event
  (if (== (Variables|Default|GetFireballsSpawned) (Variables|Default|GetNumOfFireballs))
    (Utilities|Time|ClearandInvalidateTimerbyHandle (Variables|Default|GetTimerHandle)) ; If All balls spawned end and set finished spawning to true
    (Variables|Default|SetisFinishedWithSpawning true)
    (Variables|Default|SetFireballsSpawned 0)
    (Development|PrintString "Done")
    (else
      (bind _output_get (Variables|Default|SetStartingPosition (Math|Vector|MakeVector (.x (Variables|Default|GetStartingPosition)) (+ (.y (Variables|Default|GetStartingPosition)) 5e+02) (.z (Variables|Default|GetStartingPosition)))))
      (Development|PrintString (Utilities|String|ToString(Transform) (Math|Transform|MakeTransform _output_get (.rotation _returnvalue) (.scale _returnvalue))))
      (Game|SpawnActorfromClass "/Game/Reign_Assets/EnemyObjects/Wrath_Boss/Blueprints/Fireball.Fireball_C" (Math|Transform|MakeTransform _output_get (.rotation _returnvalue) (.scale _returnvalue)) "Undefined" 0 "-2000.000000,0.000000,6000.000000" "0.000000,0.000000,0.000000" "5.000000,5.000000,0.000000" 0)
      (Variables|Default|SetFireballsSpawned (+ (Variables|Default|GetFireballsSpawned) 1))
      (Development|PrintString "Spawn Fireball"))))

(event EventBeginPlay
  (CallFunction|SpawnFireballs 5 2.0 (.location (Transformation|GetActorTransform))))

(fn ConstructionScript)