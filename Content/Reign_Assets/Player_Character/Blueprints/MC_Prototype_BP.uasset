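; Prototype player character for third-person melee combat, with sprint, weapon pickup and sheathing, harpoon aiming, grappling and a health/stamina HUD.
; Input events gate actions through state flags, and the equipped weapon actor supplies equip montages and light, heavy, air-dash and harpoon attacks.
; Attacks pressed mid-swing queue a chain for ChainAttacks, which checks stamina before firing.
; Timer-driven regen refills stats, but the sprint-drain timer is never started.
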(event Custom|PickUpEvent
  (bind _attachedweapon (Variables|Default|GetAttachedWeapon))
  ;[1 1 1] Picking Up Weapons
  (if (Utilities|IsValidClass (Variables|Default|GetAttachedWeapon))
    (Utilities|IsValid (Variables|Default|GetEquippedWeapon)
      (:Is%20Not%20Valid
        (bind _returnvalue (Game|SpawnActorfromClass _attachedweapon (Transformation|GetSocketTransform (Variables|Character|GetMesh) (.EquipSocket (Utilities|GetClassDefaults _attachedweapon)) "RTS_World") "Undefined" 0 0))
        (Variables|Default|SetEquippedWeapon _returnvalue)
        (CallFunction|GrabWeapon)
        (Variables|Default|SetIsWeaponSet? true)))
    (else
      (Development|PrintString "Nothing To Pick up"))))

(event Custom|Draw/Sheath%20Weapon
  ;[1 1 1] Draw/Sheath Sword
  (if (or (not (Variables|Default|GetIsWeaponSet?)) (Variables|Default|GetPlayingAnimation?))
    (Development|PrintString "Playing Animation/no Set weapon")
    (elif (Variables|Default|GetIsWeaponEquipped?)
      (Variables|Default|SetCannot%20Attack true)
      (Variables|Default|SetPlayingAnimation? true)
      (bind _returnvalue (Animation|PlayAnimMontage (Variables|/Game/Reign_Assets/Weapon_BP/Master_Weapon_BP.Master_Weapon_BP_C|GetUnequipAnimation (Variables|Default|GetEquippedWeapon)) 1.0 "None"))
      (Utilities|FlowControl|Delay _returnvalue)
      (Variables|Default|SetPlayingAnimation? false)
      (Variables|Default|SetCannot%20Attack false)
      (else
        (Variables|Default|SetCannot%20Attack true)
        (Variables|Default|SetPlayingAnimation? true)
        (bind _returnvalue_2 (Animation|PlayAnimMontage (Variables|/Game/Reign_Assets/Weapon_BP/Master_Weapon_BP.Master_Weapon_BP_C|GetEquipAnimation (Variables|Default|GetEquippedWeapon)) 1.0 "None"))
        (Utilities|FlowControl|Delay _returnvalue_2)
        (Variables|Default|SetPlayingAnimation? false)
        (Variables|Default|SetCannot%20Attack false)))))

(event Custom|Start/Stop%20Stamina%20Regen
  ;[1 1 1] Health and Stamina Regen
  (Class|KismetSystemLibrary|PauseTimer self "StaminaRegen")
  (Utilities|FlowControl|Delay 1.0)
  (Utilities|Time|SetTimerbyFunctionName self "StaminaRegen" 0.1 true))

(event Custom|Start/Stop%20Health%20Regen
  ;[1 1 1] Health and Stamina Regen
  (Class|KismetSystemLibrary|PauseTimer self "HealthRegen")
  (Utilities|FlowControl|Delay 1.0)
  (Utilities|Time|SetTimerbyFunctionName self "HealthRegen" 0.1 true))

(event Custom|Attack
  ;[1 1 1] Melee Attack System
  ;;[1 1 1] Attack Solver
  (Variables|Default|SetPlayingAnimation? true)
  (if (not (Variables|Default|GetLastAttack))
    (if (Variables|Default|GetLightAttack)
      (if (>= (Variables|Default|GetCurrentStamina) 5.0)
        (CallFunction|StaminaCustomDecrease 1.0)
        (Default|LightAttack (Variables|Default|GetEquippedWeapon))
        (else
          (CallFunction|ResetAttack :!label _label)))
      (elif (Variables|Default|GetHeavyAttack)
        (if (>= (Variables|Default|GetCurrentStamina) 2e+01)
          (CallFunction|StaminaCustomDecrease 1.0)
          (Default|HeavyAttack (Variables|Default|GetEquippedWeapon))
          (else
            (goto _label)))
        (elif (Variables|Default|GetAirDash)
          (if (>= (Variables|Default|GetCurrentStamina) 1e+01)
            (CallFunction|StaminaCustomDecrease 1.0)
            (Default|AirDash (Variables|Default|GetEquippedWeapon))
            (CallFunction|AmIFalling?)
            (else
              (CallFunction|ResetAttack)
              (CallFunction|ResetShooting))))))))

(event Custom|ResetAttack
  ;[1 1 1] Melee Attack System
  ;;[1 1 1] Resets almost everyting
  (Variables|Default|SetLightAttack false)
  (Variables|Default|SetHeavyAttack false)
  (Variables|Default|SetChainAttack false)
  (Variables|Default|SetLastAttack false)
  (Variables|Default|SetChainHeavyAttack 0)
  (Variables|Default|SetChainLightAttack 0)
  (Variables|Default|SetPlayingAnimation? false))

(event Custom|Chain%20Attacks
  ;[1 1 1] Melee Attack System
  ;;[1 1 1] Attack Solver
  (if (Variables|Default|GetChainAttack)
    (Variables|Default|SetChainAttack false)
    (Variables|Default|SetPlayingAnimation? true)
    (if (not (Variables|Default|GetLastAttack))
      (if (Variables|Default|GetLightAttack)
        (if (>= (Variables|Default|GetCurrentStamina) 5.0)
          (CallFunction|StaminaCustomDecrease 1.0)
          (Default|LightAttack (Variables|Default|GetEquippedWeapon))
          (else
            (CallFunction|ResetAttack :!label _label)))
        (elif (Variables|Default|GetHeavyAttack)
          (if (>= (Variables|Default|GetCurrentStamina) 2e+01)
            (CallFunction|StaminaCustomDecrease 1.0)
            (Default|HeavyAttack (Variables|Default|GetEquippedWeapon))
            (else
              (goto _label)))
          (elif (Variables|Default|GetAirDash)
            (if (>= (Variables|Default|GetCurrentStamina) 1e+01)
              (CallFunction|StaminaCustomDecrease 1.0)
              (Default|AirDash (Variables|Default|GetEquippedWeapon))
              (CallFunction|AmIFalling?)
              (else
                (CallFunction|ResetAttack)
                (CallFunction|ResetShooting)))))))))

(event Custom|Am%20I%20Falling?
  ;[1 1 1] Melee Attack System
  ;;[1 1 1] Attack Event
  ;;;[1 1 1] Air Attack
  (if (AI|Components|NavMovement|IsFalling (Variables|Character|GetCharacterMovement))
    (Utilities|Time|SetTimerbyFunctionName 0 "Am I Falling?" 0.01 true)
    (else
      (Class|KismetSystemLibrary|PauseTimer 0 "Am I Falling?")
      (Utilities|FlowControl|DoOnce false) ; enters at Reset
    )))

(event Custom|ResetShooting
  ;[1 1 1] Shooting
  (Variables|Default|SetCannot%20Attack false)
  (Variables|Default|SetIsShooting? false)
  (Variables|Default|SetPlayingAnimation? false)
  (Development|SetHiddeninGame (Variables|Default|GetAiming%20Arrow) true false)
  (Utilities|FlowControl|DoOnce false) ; enters at Reset
)

(event EventBeginPlay
  ;[1 1 1] On Begin
  (Variables|/Script/Engine.CharacterMovementComponent|SetMaxWalkSpeed (Variables|Character|GetCharacterMovement) 5e+02)
  (bind _returnvalue (UserInterface|CreateWidget "/Game/Reign_Assets/Player_Character/Player_Widgets_UI/PlayerHealthStamina.PlayerHealthStamina_C"))
  (bind _output_get (Variables|Default|SetHealthStaminaWidget _returnvalue))
  (UserInterface|Viewport|AddtoViewport _output_get 0)
  (CallFunction|UpdateHealth)
  (CallFunction|UpdateStamina))

(event Input|ActionEvents|InputActionRight_DownPad
  (params (Key :type Key%20Structure))
  ;[1 1 1] Camera Controls and FX
)

(event Input|ActionEvents|InputActionYButton
  (params (Key :type Key%20Structure))
  ;[1 1 1] HotKeys
  (:Pressed
    (CallFunction|PickUpEvent)))

(event Input|ActionEvents|InputActionAButton
  (params (Key :type Key%20Structure))
  ;[1 1 1] Jumping.....
  (:Pressed
    (Character|Jump))
  (:Released
    (Character|StopJumping)))

(event Input|ActionEvents|InputActionXButton
  (params (Key :type Key%20Structure))
  ;[1 1 1] HotKeys
  (:Pressed
    (CallFunction|Draw/SheathWeapon)))

(event Input|ActionEvents|InputActionRight_DownPad
  (params (Key :type Key%20Structure))
  ;[1 1 1] Shooting
  (:Pressed
    (Utilities|IsValid (Variables|Default|GetGrappleObject)
      (:Is%20Valid
        (Development|PrintString "Can Grapple")
        (if (>= (Variables|Default|GetCurrentStamina) 5e+01)
          (Transformation|SetWorldLocation (Variables|Collision|GetCapsuleComponent) (Math|Interpolation|VInterpTo (Transformation|GetWorldLocation (Variables|Collision|GetCapsuleComponent)) (+ (Transformation|GetWorldLocation (Variables|/Game/Reign_Assets/World_Objects/GrappleObjects/Master_Grapple_Object.Master_Grapple_Object_C|GetGrapple%20Point (Variables|Default|GetGrappleObject))) "0, 0,100.000000") (Utilities|Time|GetWorldDeltaSeconds) 7e+01) false false)
          (CallFunction|StaminaCustomDecrease 5e+01)
          (else
            (Development|PrintString "Not Enough Stamina"))))
      (:Is%20Not%20Valid
        (Development|PrintString "Cant Grapple")))))

(event Input|ActionEvents|InputActionJump
  (params (Key :type Key%20Structure))
  ;[1 1 1] Melee Attack System
  ;;[1 1 1] Attack Event
  (:Pressed
    (Utilities|IsValid (Variables|Default|GetEquippedWeapon)
      (:Is%20Valid
        (if (not (Variables|Default|GetCannot%20Attack))
          (if (Variables|Default|GetIsWeaponEquipped?)
            (if (Variables|/Game/Reign_Assets/Weapon_BP/Master_Weapon_BP.Master_Weapon_BP_C|GetIsBladeAttached? (Variables|Default|GetEquippedWeapon))
              (if (AI|Components|NavMovement|IsFalling (Variables|Character|GetCharacterMovement))
                ;;;[1 1 1] Air Attack
                (Utilities|FlowControl|DoOnce false
                  (:Completed
                    (Variables|Default|SetAirDash true)
                    (Variables|Default|SetLightAttack false)
                    (Variables|Default|SetHeavyAttack false)
                    (Collision|SetCollisionResponsetoChannel (Variables|Collision|GetCapsuleComponent) "ECC_GameTraceChannel1" "ECR_Ignore")
                    (CallFunction|Attack)))
                (else
                  ;;[1 1 1] Ground Light Attack
                  (if (Variables|Default|GetHoldingSprint?)
                    ;;[1 1 1] Dash HeavyAttack
                    (if (or (Variables|Default|GetLightAttack) (Variables|Default|GetHeavyAttack))
                      (Variables|Default|SetChainAttack true)
                      (Variables|Default|SetLightAttack false)
                      (Variables|Default|SetHeavyAttack true)
                      (Variables|Default|SetAirDash false)
                      (else
                        (Variables|Default|SetLightAttack false)
                        (Variables|Default|SetHeavyAttack true)
                        (Variables|Default|SetAirDash false)
                        (Collision|SetCollisionResponsetoChannel (Variables|Collision|GetCapsuleComponent) "ECC_GameTraceChannel1" "ECR_Ignore")
                        (CallFunction|Attack)))
                    (elif (or (Variables|Default|GetLightAttack) (Variables|Default|GetHeavyAttack))
                      (Variables|Default|SetChainAttack true)
                      (Variables|Default|SetLightAttack true)
                      (Variables|Default|SetHeavyAttack false)
                      (Variables|Default|SetAirDash false)
                      (else
                        (Variables|Default|SetLightAttack true)
                        (Variables|Default|SetHeavyAttack false)
                        (Variables|Default|SetAirDash false)
                        (CallFunction|Attack))))))
              (else
                (Development|PrintString "Blade not attached")))
            (else
              (CallFunction|Draw/SheathWeapon))))))))

(event Input|AxisEvents|InputAxisTurn
  (params (AxisValue :type Float%20%28single-precision%29))
  ;[1 1 1] Aiming Controls
  (if (Variables|Default|GetIsShooting?)
    (Transformation|SetWorldRotation (Variables|Collision|GetCapsuleComponent) (Math|Rotator|MakeRotator 0.0 0.0 (+ (* (stale Input|AxisEvents|InputAxisTurnRate AxisValue) 2.0) (.Yaw (Math|Rotator|BreakRotator (Transformation|GetWorldRotation (Variables|Collision|GetCapsuleComponent)))))) false false)))

(event Input|AxisEvents|InputAxisRightTriggerAxis
  (params (AxisValue :type Float%20%28single-precision%29))
  ;[1 1 1] Controls
  ;;[1 1 1] Movement
  (if (>= AxisValue 0.1)
    (Variables|Default|SetHoldingSprint? true)
    (if (!= (Math|Vector|VectorLength (Transformation|GetVelocity)) 0.0)
      (if (and (> (Variables|Default|GetCurrentStamina) 1.0) (not (Variables|Default|GetPlayingAnimation?)))
        (Variables|/Script/Engine.CharacterMovementComponent|SetMaxWalkSpeed (Variables|Character|GetCharacterMovement) 1e+03)))
    (else
      (Variables|Default|SetHoldingSprint? false)
      (Variables|/Script/Engine.CharacterMovementComponent|SetMaxWalkSpeed (Variables|Character|GetCharacterMovement) 5e+02)
      (Class|KismetSystemLibrary|PauseTimer self "StaminaSprintDecrease"))))

(event Input|AxisEvents|InputAxisTurnRate
  (params (AxisValue :type Float%20%28single-precision%29)))

(event Input|AxisEvents|InputAxisLeftTriggerAxis
  (params (AxisValue :type Float%20%28single-precision%29))
  ;[1 1 1] Shooting
  (if (>= AxisValue 0.1)
    (Utilities|IsValid (Variables|Default|GetEquippedWeapon)
      (:Is%20Valid
        (if (not (Variables|Default|GetCannot%20Attack))
          (if (Variables|Default|GetIsWeaponEquipped?)
            (if (not (Variables|Default|GetPlayingAnimation?))
              (Variables|Default|SetPlayingAnimation? true)
              (Variables|Default|SetICanAim? true)
              (Variables|Default|SetIsShooting? true)
              (Variables|Default|SetCannot%20Attack true)
              (Development|SetHiddeninGame (Variables|Default|GetAiming%20Arrow) false false))
            (else
              (CallFunction|Draw/SheathWeapon))))))
    (elif (Variables|Default|GetIsShooting?)
      (Utilities|FlowControl|DoOnce false
        (:Completed
          (Utilities|IsValid (Variables|Default|GetEquippedWeapon)
            (:Is%20Valid
              (if (Variables|Default|GetIsWeaponEquipped?)
                (Variables|Default|SetICanAim? false)
                (Default|HarpoonEvent (Variables|Default|GetEquippedWeapon))))))))))

(event Input|AxisEvents|InputAxisMoveForward
  (params (AxisValue :type Float%20%28single-precision%29))
  (bind _returnvalue (Pawn|GetControlRotation :!class /Script/Engine.Pawn))
  (bind _yaw (Math|Rotator|BreakRotator _returnvalue))
  (bind _returnvalue_2 (Math|Rotator|MakeRotator 0.0 0.0 _yaw))
  ;[1 1 1] Controls
  ;;[1 1 1] Movement
  (if (not (Variables|Default|GetIsShooting?))
    (if (not (Variables|Default|GetPlayingAnimation?))
      (Pawn|Input|AddMovementInput (Math|Vector|GetForwardVector _returnvalue_2) AxisValue false)
      (Pawn|Input|AddMovementInput (Math|Vector|GetRightVector _returnvalue_2) (* AxisValue -1.0) false))))

(event Input|AxisEvents|InputAxisMoveRight
  (params (AxisValue :type Float%20%28single-precision%29))
  (bind _returnvalue (Pawn|GetControlRotation :!class /Script/Engine.Pawn))
  (bind _yaw (Math|Rotator|BreakRotator _returnvalue))
  (bind _returnvalue_2 (Math|Rotator|MakeRotator 0.0 0.0 _yaw))
  ;[1 1 1] Controls
  ;;[1 1 1] Movement
  (if (not (Variables|Default|GetIsShooting?))
    (if (not (Variables|Default|GetPlayingAnimation?))
      (Pawn|Input|AddMovementInput (Math|Vector|GetRightVector _returnvalue_2) AxisValue false)
      (Pawn|Input|AddMovementInput (Math|Vector|GetForwardVector _returnvalue_2) AxisValue false))
    (else
      ;;;[1 1 1] PlayerAimingRotation
      (if (Variables|Default|GetICanAim?)
        (Transformation|SetWorldRotation (Variables|Collision|GetCapsuleComponent) (Math|Rotator|MakeRotator 0.0 0.0 (+ (* AxisValue 1e+01) (.Yaw (Math|Rotator|BreakRotator (Transformation|GetWorldRotation (Variables|Collision|GetCapsuleComponent)))))) false false)))))

(event Input|KeyboardEvents|F
  (params (Key :type Key%20Structure))
  ;[1 1 1] Shooting
)

(event Input|KeyboardEvents|E
  (params (Key :type Key%20Structure))
  ;[1 1 1] HotKeys
  (:Pressed
    (CallFunction|PickUpEvent)))

(event Input|KeyboardEvents|Q
  (params (Key :type Key%20Structure))
  ;[1 1 1] HotKeys
  (:Pressed
    (CallFunction|Draw/SheathWeapon)))

(event Input|MouseEvents|LeftMouseButton
  (params (Key :type Key%20Structure))
  ;[1 1 1] Melee Attack System
  ;;[1 1 1] Attack Event
)

(event Input|MouseEvents|RightMouseButton
  (params (Key :type Key%20Structure))
  ;[1 1 1] Controls
  ;;[1 1 1] Movement
  (:Pressed
    (Variables|Default|SetHoldingSprint? true)
    (if (!= (Math|Vector|VectorLength (Transformation|GetVelocity)) 0.0)
      (if (and (> (Variables|Default|GetCurrentStamina) 1.0) (not (Variables|Default|GetPlayingAnimation?)))
        (Variables|/Script/Engine.CharacterMovementComponent|SetMaxWalkSpeed (Variables|Character|GetCharacterMovement) 1e+03))))
  (:Released
    (Variables|Default|SetHoldingSprint? false)
    (Variables|/Script/Engine.CharacterMovementComponent|SetMaxWalkSpeed (Variables|Character|GetCharacterMovement) 5e+02)
    (Class|KismetSystemLibrary|PauseTimer self "StaminaSprintDecrease")))

(event Input|KeyboardEvents|Z
  (params (Key :type Key%20Structure))
  (bind _springarm (Variables|Default|GetSpringArm))
  ;[1 1 1] Camera Controls and FX
  (:Pressed
    (Variables|/Script/Engine.SpringArmComponent|SetTargetArmLength _springarm 7e+02))
  (:Released
    (Variables|/Script/Engine.SpringArmComponent|SetTargetArmLength _springarm 1.3e+03)))

(fn ConstructionScript)

(fn GrabWeapon
  (bind _equippedweapon (Variables|Default|GetEquippedWeapon))
  (Transformation|AttachComponentToComponent _equippedweapon (Variables|Character|GetMesh) (Variables|/Game/Reign_Assets/Weapon_BP/Master_Weapon_BP.Master_Weapon_BP_C|GetUnequipSocket _equippedweapon) "SnapToTarget" "SnapToTarget" "SnapToTarget" true)
  (Variables|Default|SetIsWeaponEquipped? false)
  (return))

(fn EquipWeapon
  (bind _equippedweapon (Variables|Default|GetEquippedWeapon))
  (Transformation|AttachComponentToComponent _equippedweapon (Variables|Character|GetMesh) (Variables|/Game/Reign_Assets/Weapon_BP/Master_Weapon_BP.Master_Weapon_BP_C|GetEquipSocket _equippedweapon) "SnapToTarget" "SnapToTarget" "SnapToTarget" true)
  (Variables|Default|SetIsWeaponEquipped? true))

(fn UnequipWeapon
  (bind _equippedweapon (Variables|Default|GetEquippedWeapon))
  (Transformation|AttachComponentToComponent _equippedweapon (Variables|Character|GetMesh) (Variables|/Game/Reign_Assets/Weapon_BP/Master_Weapon_BP.Master_Weapon_BP_C|GetUnequipSocket _equippedweapon) "SnapToTarget" "SnapToTarget" "SnapToTarget" true)
  (Variables|Default|SetIsWeaponEquipped? false))

(fn UpdateHealth
  (Progress|SetPercent (Variables|/Game/Reign_Assets/Player_Character/Player_Widgets_UI/PlayerHealthStamina.PlayerHealthStamina_C|GetHealth (Variables|Default|GetHealthStaminaWidget)) (/ (Variables|Default|GetCurrentHealth) (Variables|Default|GetMaxHealth)))
  (return))

(fn UpdateStamina
  (Progress|SetPercent (Variables|/Game/Reign_Assets/Player_Character/Player_Widgets_UI/PlayerHealthStamina.PlayerHealthStamina_C|GetStamina (Variables|Default|GetHealthStaminaWidget)) (/ (Variables|Default|GetCurrentStamina) (Variables|Default|GetMaxStamina)))
  (return))

(fn HealthRegen
  (if (>= (Variables|Default|GetCurrentHealth) (Variables|Default|GetMaxHealth))
    (Class|KismetSystemLibrary|PauseTimer self "Health Regen")
    (Variables|Default|SetCurrentHealth (Variables|Default|GetMaxHealth))
    (else
      (Variables|Default|SetCurrentHealth (+ (Variables|Default|GetCurrentHealth) (Variables|Default|GetHealthRegenRate)))
      (CallFunction|UpdateHealth)
      (return))))

(fn StaminaSprintDecrease
  (if (!= (Math|Vector|VectorLength (Transformation|GetVelocity)) 0.0)
    (if (and (> (Variables|Default|GetCurrentStamina) 1.0) (not (Variables|Default|GetPlayingAnimation?)))
      (Variables|Default|SetCurrentStamina (- (Variables|Default|GetCurrentStamina) 1.0))
      (CallFunction|UpdateStamina)
      (CallFunction|Start/StopStaminaRegen)
      (return)
      (else
        (Class|KismetSystemLibrary|PauseTimer self "StaminaDecrease")
        (Variables|/Script/Engine.CharacterMovementComponent|SetMaxWalkSpeed (Variables|Character|GetCharacterMovement) 5e+02)))))

(fn StaminaRegen
  (if (>= (Variables|Default|GetCurrentStamina) (Variables|Default|GetMaxStamina))
    (Class|KismetSystemLibrary|PauseTimer self "StaminaRegen")
    (Variables|Default|SetCurrentStamina (Variables|Default|GetMaxStamina))
    (else
      (Variables|Default|SetCurrentStamina (+ (Variables|Default|GetCurrentStamina) (Variables|Default|GetStaminaRegenRate)))
      (CallFunction|UpdateStamina)
      (return))))

(fn HealthDecrease
  (params (DecreaseAmount :type Float%20%28single-precision%29))
  (if true
    (if (> (Variables|Default|GetCurrentHealth) 1.0)
      (Variables|Default|SetCurrentHealth (- (Variables|Default|GetCurrentHealth) DecreaseAmount))
      (CallFunction|UpdateHealth)
      (CallFunction|Start/StopHealthRegen)
      (return))))

(fn StaminaCustomDecrease
  (params (DecreaseAmount :type Float%20%28single-precision%29))
  (Variables|Default|SetCurrentStamina (- (Variables|Default|GetCurrentStamina) DecreaseAmount))
  (CallFunction|UpdateStamina)
  (CallFunction|Start/StopStaminaRegen)
  (return))

(fn StopMontage
  (bind _returnvalue (Animation|GetCurrentMontage :!class /Script/Engine.Character))
  (Animation|StopAnimMontage _returnvalue)
  (return))

(fn CMove
  (bind _mesh (Variables|Character|GetMesh))
  (if (Variables|Default|GetBoosting?)
    (if (Variables|Default|GetBoostingUp?)
      (Character|LaunchCharacter (* (Math|Vector|GetUpVector (Transformation|GetWorldRotation (Variables|Character|GetMesh))) 1.5e+03) false false)
      (Variables|Default|SetBoosting? false)
      (Variables|Default|SetBoostingUp? false)
      (else
        (Character|LaunchCharacter (* (Math|Vector|GetRightVector (Transformation|GetWorldRotation (Variables|Character|GetMesh))) (Variables|Default|GetBoostValue)) false false)
        (Variables|Default|SetBoosting? false)))
    (elif (Variables|Default|GetLeft/Right?)
      (Pawn|Input|AddMovementInput (Math|Vector|GetForwardVector _mesh) (Variables|Default|GetMovementValue) false)
      (return)
      (else
        (Pawn|Input|AddMovementInput (Math|Vector|GetRightVector _mesh) (Variables|Default|GetMovementValue) false)
        (return)))))

(fn CBoost
  (if (Variables|Default|GetBoosting?)
    ;[1 1 1] Forward Boost
    (Character|LaunchCharacter (* (Math|Vector|GetRightVector (Transformation|GetWorldRotation (Variables|Character|GetMesh))) (Variables|Default|GetBoostValue)) false false)
    (Variables|Default|SetBoosting? false)
    (elif (Variables|Default|GetBoostingUp?)
      ;[1 1 1] Upward Boost
      (Character|LaunchCharacter (* (Math|Vector|GetUpVector (Transformation|GetWorldRotation (Variables|Character|GetMesh))) (Variables|Default|GetBoostValue)) false false)
      (Variables|Default|SetBoostingUp? false))))