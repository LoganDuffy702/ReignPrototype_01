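; Mouse companion controller that positions a companion effect near the player or at a lock-on target.
; Each tick it places the effect a fixed distance along the player locator's rotation actor, or interpolates toward the lock-on marker when EnemyElement is valid.
; The older cursor-follow and cursor-trace targeting logic is disconnected, so FollowMouse and CheckTarget do nothing and nothing live assigns EnemyElement.
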(event Custom|Follow%20Mouse
  ;[1 1 1] Mouse Movement
)

(event Custom|Companion%20Movement
  (bind _enemyelement (Variables|Default|GetEnemyElement))
  (bind _playerlocatorbp_ref (Variables|Default|GetPlayerLocatorBP_Ref))
  (bind _companionrotactor (Variables|/Game/Reign_Assets/World_Objects/PlayerLocation_Actor/PlayerLocation_Actor_BP.PlayerLocation_Actor_BP_C|GetCompanionRotActor _playerlocatorbp_ref))
  ;[1 1 1] Companion
  (Utilities|IsValid _enemyelement
    (:Is%20Valid
      (Transformation|SetWorldLocation (Variables|Default|GetCompanion_FX) (Math|Interpolation|VInterptoConstant (Variables|Default|GetComp%20Last%20Loc) (Transformation|GetWorldLocation (Variables|/Game/Reign_Assets/EnemyObjects/Master_LockOn_BP/Master_LockOn_Object_BP.Master_LockOn_Object_BP_C|GetLockOnMarker _enemyelement)) 0.1 5e+02) false false))
    (:Is%20Not%20Valid
      (bind _outpoint (CallFunction|RotateAround (Transformation|GetWorldLocation _companionrotactor) (Transformation|GetWorldRotation _companionrotactor) 2e+02))
      (Transformation|SetWorldLocation (Variables|Default|GetCompanion_FX) _outpoint false false))))

(event Custom|CheckTarget
  ;[1 1 1] Lock on Mouse Version (old)
)

(event Custom|TargetFound
  (bind _enemyelement (Variables|Default|GetEnemyElement))
  ;[1 1 1] Lock on Mouse Version (old)
  (Utilities|IsValid _enemyelement
    (:Is%20Valid
      (bind _output_get (Variables|Default|SetTargetedEnemy _enemyelement))
      (Variables|/Game/Reign_Assets/EnemyObjects/Master_LockOn_BP/Master_LockOn_Object_BP.Master_LockOn_Object_BP_C|SetIsLinked? _output_get true)
      (Variables|/Game/Reign_Assets/Player_Character/Blueprints/MC_Prototype_BP.MC_Prototype_BP_C|SetNearestTarget (Variables|Default|GetPlayerRef) _output_get))))

(event Custom|SetTargetedObject
  (bind _enemyelement (Variables|Default|GetEnemyElement))
  ;[1 1 1] Lock on Mouse Version (old)
  (Utilities|IsValid _enemyelement
    (:Is%20Valid
      (Class|LockonSystem|Lockon(Message) _enemyelement)
      (Variables|Default|SetComp%20Last%20Loc (Transformation|GetWorldLocation (Variables|Default|GetCompanion_FX))))))

(event Custom|CheckDistance
  ;[1 1 1] Lock on Mouse Version (old)
  (Utilities|IsValid (Variables|Default|GetEnemyElement)
    (:Is%20Valid
      (if (not (Variables|/Game/Reign_Assets/EnemyObjects/Master_LockOn_BP/Master_LockOn_Object_BP.Master_LockOn_Object_BP_C|GetCanBeTargeted (Variables|Default|GetEnemyElement)))
        (Variables|Default|SetEnemyElement 0)
        (Variables|Default|SetComp%20Last%20Loc (Transformation|GetWorldLocation (Variables|Default|GetCompanion_FX)))))))

(event EventBeginPlay
  (bind _asmc_prototype_bp (Utilities|Casting|CastToMC_Prototype_BP (Game|GetPlayerCharacter 0)))
  (Variables|Default|SetPlayerRef _asmc_prototype_bp)
  (bind _outactors (Actor|GetAllActorsOfClass "/Game/Reign_Assets/World_Objects/PlayerLocation_Actor/PlayerLocation_Actor_BP.PlayerLocation_Actor_BP_C"))
  (Variables|Default|SetPlayerLocatorBP_Ref (Utilities|Array|Get(acopy) _outactors)))

(event Collision|EventActorBeginOverlap
  (params (OtherActor :type Actor%20Object%20Reference)))

(event EventTick
  (params (DeltaSeconds :type Float%20%28single-precision%29))
  (Variables|Default|SetDeltaTime DeltaSeconds)
  (CallFunction|FollowMouse)
  (CallFunction|CompanionMovement)
  (CallFunction|CheckTarget))

(fn ConstructionScript)

(fn RotateAround
  (params (Center :type Vector) (Rotation :type Rotator) (Distance :type Float%20%28single-precision%29))
  (return (+ Center (* (Math|Vector|GetForwardVector Rotation) Distance))))