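; Player companion actor, formerly a mouse-driven lock-on cursor, that trails the player character.
; Each tick it turns its Parent component toward the player and applies forward force when over 1000 units away.
; Movement is skipped while a Phase1_Boss exists and MoveCompanion is set.
; Mouse following and CheckTarget are empty stubs; cursor-trace lock-on and orbit positioning around PlayerLocation_Actor_BP remain as disconnected legacy logic.
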(event Custom|Follow%20Mouse
  ;[1 1 1] Mouse Movement
)

(event Custom|Companion%20Movement
  (bind _playerref (Variables|Default|GetPlayerRef))
  (bind _parent (Variables|Default|GetParent))
  (bind _parent_2 (Variables|Default|GetParent))
  (bind _returnvalue (Transformation|GetWorldLocation _parent))
  (bind _capsulecomponent (Variables|/Script/Engine.Character|GetCapsuleComponent _playerref))
  (bind _returnvalue_2 (Transformation|GetWorldLocation _capsulecomponent))
  (bind _returnvalue_3 (Math|Rotator|FindLookatRotation _returnvalue _returnvalue_2))
  (bind _returnvalue_4 (Math|Rotator|MakeRotator (.roll _returnvalue_3) (.pitch _returnvalue_3) (.yaw _returnvalue_3)))
  (Transformation|SetWorldRotation (Variables|Default|GetParent) (Math|Rotator|MakeRotator 0.0 (.pitch _returnvalue_4) (.yaw _returnvalue_4)) false false)
  (if (not (<= (Math|Vector|VectorLength (- (Transformation|GetWorldLocation (Variables|Default|GetParent)) (Transformation|GetWorldLocation (Variables|/Script/Engine.Character|GetCapsuleComponent (Variables|Default|GetPlayerRef))))) 1e+03))
    (Physics|AddForce _parent_2 (* (Math|Vector|GetForwardVector _parent_2) 130000) "None" false)))

(event Custom|CheckTarget
  ;[1 1 1] Lock on Mouse Version (old)
)

(event Custom|TargetFound
  (bind _enemyelement (Variables|Default|GetEnemyElement))
  ;[1 1 1] Lock on Mouse Version (old)
  (Utilities|IsValid _enemyelement
    (:Is%20Valid
      (bind _output_get (Variables|Default|SetTargetedEnemy _enemyelement))
      (Variables|/Game/Reign_Assets/EnemyObjects/Master_LockOn_BP/Master_LockOn_Object_BP.Master_LockOn_Object_BP_C|SetIsLinked? _output_get true)
      (Variables|/Game/Reign_Assets/Player_Character/Blueprints/MC_Prototype_BP.MC_Prototype_BP_C|SetNearestTarget (Variables|Default|GetPlayerRef) _output_get))))

(event Custom|SetTargetedObject
  (bind _enemyelement (Variables|Default|GetEnemyElement))
  ;[1 1 1] Lock on Mouse Version (old)
  (Utilities|IsValid _enemyelement
    (:Is%20Valid
      (Class|LockonSystem|Lockon(Message) _enemyelement)
      (Variables|Default|SetComp%20Last%20Loc (Transformation|GetWorldLocation (Variables|Default|GetCompanion_FX))))))

(event Custom|CheckDistance
  ;[1 1 1] Lock on Mouse Version (old)
  (Utilities|IsValid (Variables|Default|GetEnemyElement)
    (:Is%20Valid
      (if (not (Variables|/Game/Reign_Assets/EnemyObjects/Master_LockOn_BP/Master_LockOn_Object_BP.Master_LockOn_Object_BP_C|GetDistanceToPlayerActive? (Variables|Default|GetEnemyElement)))
        (Variables|Default|SetEnemyElement 0)
        (Variables|Default|SetComp%20Last%20Loc (Transformation|GetWorldLocation (Variables|Default|GetCompanion_FX)))))))

(event EventBeginPlay
  (bind _asmc_prototype_bp (Utilities|Casting|CastToMC_Prototype_BP (Game|GetPlayerCharacter 0)))
  (Variables|Default|SetPlayerRef _asmc_prototype_bp)
  (bind _outactors (Actor|GetAllActorsOfClass "/Game/Reign_Assets/World_Objects/PlayerLocation_Actor/PlayerLocation_Actor_BP.PlayerLocation_Actor_BP_C"))
  (Variables|Default|SetPlayerLocatorBP_Ref (Utilities|Array|Get(acopy) _outactors)))

(event Collision|EventActorBeginOverlap
  (params (OtherActor :type Actor%20Object%20Reference)))

(event EventTick
  (params (DeltaSeconds :type Float%20%28single-precision%29))
  (Variables|Default|SetDeltaTime DeltaSeconds)
  (bind _outactors (Actor|GetAllActorsOfClass "/Game/Final_Boss/Phase1/Phase1_Boss.Phase1_Boss_C"))
  (if (and (Utilities|Array|IsValidIndex _outactors) (Variables|Default|GetMoveCompanion))
    (Utilities|FlowControl|DoOnce false)
    (else
      (CallFunction|FollowMouse)
      (CallFunction|CompanionMovement))))

(fn ConstructionScript)

(fn RotateAround
  (params (Center :type Vector) (Rotation :type Rotator) (Distance :type Float%20%28single-precision%29))
  (return (+ Center (* (Math|Vector|GetForwardVector Rotation) Distance))))