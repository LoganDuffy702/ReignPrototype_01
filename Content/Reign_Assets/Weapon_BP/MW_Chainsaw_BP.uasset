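; Chainsaw weapon Blueprint, a child class that adds detachable-blade effects on top of its parent's behavior.
; LaunchBladeFX attaches the Blade to the damaged enemy's ChokePoint and spawns a flying aggro emitter there.
; ReturnBladeFX detaches the Blade and reattaches it to the Weapon component, snapping its rotation back.
; A separate event turns off the Blade's custom depth rendering, and nothing in this graph calls these three events.
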(event EventBeginPlay
  (|CallParentFunction))

(event Collision|EventActorBeginOverlap
  (params (OtherActor :type Actor%20Object%20Reference))
  (|CallParentFunction OtherActor) ; This node is disabled and will not be called.\nDrag off pins to build functionality.
)

(event EventTick
  (params (DeltaSeconds :type Float%20%28single-precision%29))
  (|CallParentFunction DeltaSeconds) ; This node is disabled and will not be called.\nDrag off pins to build functionality.
)

(event EventLaunchBladeFX
  (bind _damagedenemy (Variables|Default|GetDamagedEnemy))
  (bind _chokepoint (Variables|/Game/Reign_Assets/EnemyObjects/Master_LockOn_BP/Master_LockOn_Object_BP.Master_LockOn_Object_BP_C|GetChokePoint _damagedenemy))
  (Transformation|AttachComponentToComponent (Variables|Default|GetBlade) _chokepoint "" "KeepRelative" "KeepWorld" "KeepWorld" true)
  (Effects|SpawnEmitteratLocation "/Game/Reign_Assets/EnemyObjects/Flying_Enemy/FlyingFX/FlyingAggro_FX.FlyingAggro_FX" (Transformation|GetWorldLocation _chokepoint)))

(event EventReturnBladeFX
  (Transformation|DetachFromComponent (Variables|Default|GetBlade) "KeepRelative" "KeepRelative" "KeepWorld" true)
  (Transformation|AttachComponentToComponent (Variables|Default|GetBlade) (Variables|Default|GetWeapon) "" "KeepRelative" "SnapToTarget" "KeepWorld" true))

(event EventTurnOffCustomDepth
  (Rendering|SetRenderCustomDepth (Variables|Default|GetBlade) false))

(fn ConstructionScript
  (|CallParentFunction))