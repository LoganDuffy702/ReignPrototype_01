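; Base weapon Blueprint for the player character, handling melee combos, air attacks and a harpoon grapple.
; X/Y combo strings select attack montages, while sphere traces damage unhit lock-on objects and restore stamina.
; The harpoon plays a montage on the nearest target, FireWeapon links and damages it with a beam-particle chain, and re-triggering releases it.
; Older cable, launch-trace, chain-combo and tower-damage logic remains disconnected.
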(event Custom|WeaponAttack
  (params (DamageType :type Name) (ComboString :type String))
  (bind _atkspeed (Variables|Default|GetAtkSpeed))
  (bind _characterref (Variables|Default|GetCharacterRef))
  (bind _characterref_2 (Variables|Default|GetCharacterRef))
  (bind _characterref_3 (Variables|Default|GetCharacterRef))
  (bind _charactermovement (Variables|/Script/Engine.Character|GetCharacterMovement _characterref_3))
  ;[1 1 1] Standard Attack Event
  ;;[1 1 1] New Combo system
  (Variables|Default|SetDamageType DamageType)
  (Variables|/Game/Reign_Assets/Player_Character/Blueprints/MC_Prototype_BP.MC_Prototype_BP_C|SetPlayingAnimation? _characterref_2 true)
  (if (AI|Components|NavMovement|IsFalling (Variables|/Script/Engine.Character|GetCharacterMovement _characterref_2))
    (Variables|/Script/Engine.MovementComponent|SetVelocity _charactermovement "0, 0, 0")
    (Variables|/Script/Engine.CharacterMovementComponent|SetGravityScale _charactermovement 0.0)
    (Animation|PlayAnimMontage (Variables|Default|GetCharacterRef) (Variables|Default|GetAirAttacks) 2.2 "None")
    (Utilities|FlowControl|RetriggerableDelay 1.0)
    (Variables|/Script/Engine.CharacterMovementComponent|SetGravityScale (Variables|/Script/Engine.Character|GetCharacterMovement (Variables|Default|GetCharacterRef)) 2.0)
    (else
      (Development|PrintString ComboString)
      (switch string ComboString
        (:X
          (bind _output_get (Variables|Default|SetAttackNumber 0))
          (Animation|PlayAnimMontage _characterref (Utilities|Array|Get(acopy) (Variables|Default|GetLightAttacks) _output_get) _atkspeed "None"))
        (:XX
          (bind _output_get_2 (Variables|Default|SetAttackNumber 1))
          (Animation|PlayAnimMontage _characterref (Utilities|Array|Get(acopy) (Variables|Default|GetLightAttacks) _output_get_2) _atkspeed "None"))
        (:XXX
          (bind _output_get_3 (Variables|Default|SetAttackNumber 0))
          (Animation|PlayAnimMontage (Variables|Default|GetCharacterRef) (Utilities|Array|Get(acopy) (Variables|Default|GetLightAttacks) _output_get_3) _atkspeed "None")
          (Variables|/Game/Reign_Assets/Player_Character/Blueprints/MC_Prototype_BP.MC_Prototype_BP_C|SetComboString (Variables|Default|GetCharacterRef) ""))
        (:XXY
          (bind _output_get_4 (Variables|Default|SetAttackNumber 1))
          (Animation|PlayAnimMontage _characterref (Utilities|Array|Get(acopy) (Variables|Default|GetHeavyAttacks) _output_get_4) 1.0 "None"))
        (:YXX
          (bind _output_get_5 (Variables|Default|SetAttackNumber 0))
          (Animation|PlayAnimMontage _characterref (Utilities|Array|Get(acopy) (Variables|Default|GetHeavyAttacks) _output_get_5) 1.0 "None")
          (Variables|/Game/Reign_Assets/Player_Character/Blueprints/MC_Prototype_BP.MC_Prototype_BP_C|SetComboString (Variables|Default|GetCharacterRef) ""))
        (:XYX
          (bind _output_get_6 (Variables|Default|SetAttackNumber 3))
          (Animation|PlayAnimMontage _characterref (Utilities|Array|Get(acopy) (Variables|Default|GetLightAttacks) _output_get_6) _atkspeed "None"))
        (:Y
          (bind _output_get_7 (Variables|Default|SetAttackNumber 1))
          (Animation|PlayAnimMontage _characterref (Utilities|Array|Get(acopy) (Variables|Default|GetLightAttacks) _output_get_7) _atkspeed "None"))
        (:YYY
          (bind _output_get_8 (Variables|Default|SetAttackNumber 2))
          (Animation|PlayAnimMontage _characterref (Utilities|Array|Get(acopy) (Variables|Default|GetLightAttacks) _output_get_8) _atkspeed "None"))))))

(event Custom|SpecialAttack
  (params (DamageType :type Name))
  ;[1 1 1] Standard Attack Event
  ;;[1 1 1] Heavy/Dash Attack Event?(old)
  (Variables|Default|SetDamageType DamageType)
  (Animation|PlayAnimMontage (Variables|Default|GetCharacterRef) (Utilities|Array|Get(acopy) (Variables|Default|GetHeavyAttacks) (Variables|/Game/Reign_Assets/Player_Character/Blueprints/MC_Prototype_BP.MC_Prototype_BP_C|GetSpecialSlot%20Number (Variables|Default|GetCharacterRef))) 1.0 "None"))

(event Custom|Harpoon%20Event
  (params (DamageName :type Name))
  (bind _characterref (Variables|Default|GetCharacterRef))
  ;[1 1 1] Harpoon Event
  (Variables|Default|SetDamageType DamageName)
  (Utilities|Time|SetGlobalTimeDilation 1.0)
  (if (not (Variables|Default|GetGrappleActive?))
    (bind _asmc_prototype_bp (Utilities|Casting|CastToMC_Prototype_BP (Game|GetPlayerCharacter 0)))
    (bind _output_get (Variables|Default|SetDamagedEnemy (Variables|/Game/Reign_Assets/Player_Character/Blueprints/MC_Prototype_BP.MC_Prototype_BP_C|GetNearestTarget _asmc_prototype_bp)))
    (Utilities|IsValid _output_get
      (:Is%20Valid
        (Animation|PlayAnimMontage (Variables|Default|GetCharacterRef) (Variables|Default|GetGrappleAttack) 2.0 "None"))
      (:Is%20Not%20Valid
        (CallFunction|WeaponReset)
        (Variables|Default|SetDamagedEnemy 0)))
    (else
      (Default|StopPullEvent (Variables|Default|GetDamagedEnemy))
      (Rendering|SetVisibility (Variables|Default|GetChainParticle) false false)
      (Default|ResetShooting _characterref)
      (Variables|/Game/Reign_Assets/Player_Character/Blueprints/MC_Prototype_BP.MC_Prototype_BP_C|SetCannot%20Attack _characterref false)
      (Variables|/Game/Reign_Assets/Player_Character/Blueprints/MC_Prototype_BP.MC_Prototype_BP_C|SetPlayingAnimation? _characterref false)
      (Variables|Default|SetGrappleActive? false)
      (Variables|Default|SetIsBladeAttached? true))))

(event Custom|FireWeapon
  ;[1 1 1] Harpoon Event
  (CallFunction|CableMechanicsEnemy)
  (CallFunction|GrappleDmgEvent))

(event Custom|WeaponReset
  (bind _characterref (Variables|Default|GetCharacterRef))
  ;[1 1 1] Harpoon Event
  (Rendering|SetVisibility (Variables|Default|GetChainParticle) false false)
  (Default|ResetShooting _characterref)
  (Variables|/Game/Reign_Assets/Player_Character/Blueprints/MC_Prototype_BP.MC_Prototype_BP_C|SetCannot%20Attack _characterref false)
  (Variables|/Game/Reign_Assets/Player_Character/Blueprints/MC_Prototype_BP.MC_Prototype_BP_C|SetPlayingAnimation? _characterref false)
  (Variables|Default|SetGrappleActive? false)
  (Variables|Default|SetIsBladeAttached? true))

(event Custom|Grapple%20Dmg%20Event
  (params (Hit%20Result :type Hit%20Result%20Structure))
  ;[1 1 1] Hit Event
  ;;[1 1 1] Grapple
  (Utilities|IsValid (Variables|Default|GetDamagedEnemy)
    (:Is%20Valid
      (Default|DealingDamage (Variables|Default|GetDamagedEnemy) 50 (Variables|Default|GetCharacterRef) (Variables|Default|GetDamageType)))))

(event Custom|AirDash
  (params (DamageType :type Name))
  ;[1 1 1] Standard Attack Event
  ;;[1 1 1] Heavy/Dash Attack Event?(old)
  (Variables|Default|SetDamageType DamageType)
  (Animation|PlayAnimMontage (Variables|Default|GetCharacterRef) (Variables|Default|GetAirAttacks) 2.0 "None"))

(event Custom|Multi%20Hit%20Event
  (params (Hit%20Result :type Array%20of%20Hit%20Result%20Structures))
  ;[1 1 1] Hit Event
  ;;[1 1 1] This is the melee attacks (This will not be active anymore)
  (for _array_element Hit%20Result
    (|CheckIfDynamicEnemy _array_element)))

(event Custom|Attack%20Now
  (bind _characterref (Variables|Default|GetCharacterRef))
  (bind _aoe_point (Variables|/Game/Reign_Assets/Player_Character/Blueprints/MC_Prototype_BP.MC_Prototype_BP_C|GetAoE%20Point _characterref))
  (bind _returnvalue (Transformation|GetWorldLocation _aoe_point))
  ;[1 1 1] Hit Event
  ;;[1 1 1] Traces
  (bind (_outhits _returnvalue_2) (Collision|MultiSphereTraceForObjects _returnvalue _returnvalue (Variables|Default|GetAttackRadius) (Utilities|Array|MakeArray "ObjectTypeQuery7" "ObjectTypeQuery9") false (Utilities|Array|MakeArray (Variables|Default|GetCharacterRef)) "None" true "(R=1.000000,G=0.000000,B=0.086574,A=1.000000)" "(R=0.000000,G=1.000000,B=0.053862,A=1.000000)" 1.0))
  (if _returnvalue_2
    (CallFunction|MultiHitEvent _outhits)))

(event Custom|Dash%20Attack
  (bind _characterref (Variables|Default|GetCharacterRef))
  (bind _aoe_point (Variables|/Game/Reign_Assets/Player_Character/Blueprints/MC_Prototype_BP.MC_Prototype_BP_C|GetAoE%20Point _characterref))
  (bind _returnvalue (Transformation|GetWorldLocation _aoe_point))
  ;[1 1 1] Hit Event
  ;;[1 1 1] Traces
  (bind (_outhits _returnvalue_2) (Collision|MultiSphereTraceForObjects _returnvalue _returnvalue (Variables|Default|GetAttackRadius) (Utilities|Array|MakeArray "ObjectTypeQuery7" "ObjectTypeQuery9") false (Utilities|Array|MakeArray (Variables|Default|GetCharacterRef)) "None" true "(R=1.000000,G=0.000000,B=0.086574,A=1.000000)" "(R=0.000000,G=1.000000,B=0.053862,A=1.000000)" 4.0))
  (if _returnvalue_2
    (CallFunction|MultiHitEvent _outhits)))

(event EventBeginPlay
  ;[1 1 1] Get Character referance on Beginning of Spawn
  (bind _asmc_prototype_bp (Utilities|Casting|CastToMC_Prototype_BP (Game|GetPlayerCharacter 0)))
  (Variables|Default|SetCharacterRef _asmc_prototype_bp))

(event EventTick
  (params (DeltaSeconds :type Float%20%28single-precision%29))
  (Class|ParticleSystemComponent|SetBeamSourcePoint (Variables|Default|GetChainParticle) 0 (Transformation|GetWorldLocation (Variables|Default|GetChainOrigin))))

(fn ConstructionScript)

(fn CableMechanicsEnemy
  (bind _chainparticle (Variables|Default|GetChainParticle))
  (bind _damagedenemy (Variables|Default|GetDamagedEnemy))
  (Utilities|IsValid _damagedenemy
    (:Is%20Valid
      (Variables|/Game/Reign_Assets/EnemyObjects/Master_LockOn_BP/Master_LockOn_Object_BP.Master_LockOn_Object_BP_C|SetIsLinked? _damagedenemy true)
      (Effects|SpawnEmitteratLocation "/Game/StarterContent/Particles/P_Explosion.P_Explosion" (Transformation|GetActorLocation _damagedenemy))
      (Class|ParticleSystemComponent|SetBeamTargetPoint _chainparticle 0 (Transformation|GetWorldLocation (Variables|/Game/Reign_Assets/EnemyObjects/Master_LockOn_BP/Master_LockOn_Object_BP.Master_LockOn_Object_BP_C|GetChokePoint (Variables|Default|GetDamagedEnemy))))
      (Rendering|SetVisibility _chainparticle true false)
      (Variables|Default|SetGrappleActive? true)
      (return))))

(fn CableMechanicsWorldObjects
  (params (Actor :type Actor%20Object%20Reference))
  (Effects|SpawnEmitteratLocation "/Game/StarterContent/Particles/P_Explosion.P_Explosion" (Variables|Default|GetCable%20Hit%20Location))
  (bind _returnvalue (AddComponent|AddCableComponent false (Transformation|GetRelativeTransform (Variables|Default|GetChainOrigin))))
  (bind _output_get (Variables|Default|SetCurrentCable _returnvalue))
  (Class|CableComponent|SetAttachEndto _output_get Actor "Grapple Point" "None")
  (Variables|/Script/CableComponent.CableComponent|SetEndLocation (Variables|Default|GetCurrentCable) "0, 0, 0")
  (return))