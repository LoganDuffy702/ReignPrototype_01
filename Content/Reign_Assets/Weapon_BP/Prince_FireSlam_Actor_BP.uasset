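; Prince fire slam projectile that turns into a short-lived damaging fire area when its sphere first overlaps something.
; The overlap stops ProjectileMovement, enlarges the flame particle and calls StartFire, which repeats on a looping timer it sets itself.
; Each pulse plays fire effects and sphere-traces nearby objects, sending melee damage through DealingDamageMessage.
; After a few seconds the timer pauses, the particles deactivate and the actor destroys itself.
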(event OnComponentBeginOverlap(Sphere)
  (params (OverlappedComponent :type Primitive%20Component%20Object%20Reference) (OtherActor :type Actor%20Object%20Reference) (OtherComp :type Primitive%20Component%20Object%20Reference) (OtherBodyIndex :type Integer) (bFromSweep :type Boolean) (SweepResult :type Hit%20Result%20Structure%20%28by%20ref%29))
  (Game|Components|ProjectileMovement|StopSimulating (Variables|Default|GetProjectileMovement) SweepResult)
  (Utilities|FlowControl|DoOnce false
    (:Completed
      (Effects|Components|ParticleSystem|SetFloatParameter (Variables|Default|GetParticleSystem) "FlameSize" 2e+02)
      (CallFunction|StartFire)
      (Utilities|FlowControl|Delay 5.0)
      (Class|KismetSystemLibrary|PauseTimer 0 "StartFire")
      (Components|Activation|Deactivate (Variables|Default|GetParticleSystem))
      (Utilities|FlowControl|Delay 1.0)
      (Actor|DestroyActor))))

(event Custom|StartFire
  (bind _returnvalue (Transformation|GetActorLocation))
  (bind _returnvalue_2 (Transformation|GetActorLocation))
  (bind _returnvalue_3 (+ _returnvalue_2 "0, 0,100.000000"))
  (Effects|SpawnEmitteratLocation "/Game/Reign_Assets/Weapon_BP/WeaponFX/SpecialFire_P.SpecialFire_P" _returnvalue_3)
  (Audio|PlaySoundatLocation "/Game/Reign_Assets/Sounds/Random_FX_Sounds/Lighter_Cue.Lighter_Cue" _returnvalue_3 "0, 0, 0" 1.0 1.0 0.0 0 0 0)
  (bind (_outhits _returnvalue_4) (Collision|MultiSphereTraceForObjects _returnvalue _returnvalue 6e+02 (Utilities|Array|MakeArray "ObjectTypeQuery7" "ObjectTypeQuery9") true 0 "None" true "(R=1.000000,G=0.000000,B=0.000000,A=1.000000)" "(R=0.000000,G=1.000000,B=0.000000,A=1.000000)" 1.0))
  (if _returnvalue_4
    (for _array_element _outhits
      (Class|HealthDamageInterface|DealingDamage(Message) (.HitActor (Collision|BreakHitResult _array_element)) 5 0 "Melee")
      (Utilities|Time|SetTimerbyFunctionName 0 "StartFire" 1.0 true))
    (else
      (Utilities|Time|SetTimerbyFunctionName 0 "StartFire" 1.0 true))))

(event EventBeginPlay)

(event Collision|EventActorBeginOverlap
  (params (OtherActor :type Actor%20Object%20Reference)))

(event EventTick
  (params (DeltaSeconds :type Float%20%28single-precision%29)))

(fn ConstructionScript)