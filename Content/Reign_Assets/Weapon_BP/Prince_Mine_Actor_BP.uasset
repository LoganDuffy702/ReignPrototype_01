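; Prince's mine actor, an explosive that arms shortly after spawning and detonates when triggered or when its lifetime runs out.
; BeginPlay sets a timer to enable query collision on the trigger and starts a longer self-detonation delay; an overlap detonates it after a brief fuse.
; Detonation plays sound and particles, sphere-traces two object types, sends fixed melee damage to each hit actor via DealingDamageMessage, then destroys the mine.
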(event OnComponentBeginOverlap(TriggerCol)
  (params (OverlappedComponent :type Primitive%20Component%20Object%20Reference) (OtherActor :type Actor%20Object%20Reference) (OtherComp :type Primitive%20Component%20Object%20Reference) (OtherBodyIndex :type Integer) (bFromSweep :type Boolean) (SweepResult :type Hit%20Result%20Structure%20%28by%20ref%29))
  (Utilities|FlowControl|Delay 0.2)
  (CallFunction|ExplodePlz))

(event Custom|Explode%20Plz
  (bind _returnvalue (Transformation|GetActorLocation))
  (Audio|PlaySoundatLocation "/Game/Reign_Assets/Sounds/AttackSounds/Mine_Explosion_Cue.Mine_Explosion_Cue" (Transformation|GetActorLocation) "0, 0, 0" 1.0 1.0 0.0 0 0 0)
  (Effects|SpawnEmitteratLocation "/Game/Reign_Assets/FX/PlayerBased_Fx/SpecialSlam_P.SpecialSlam_P" (Transformation|GetActorLocation))
  (bind (_outhits _returnvalue_2) (Collision|MultiSphereTraceForObjects _returnvalue _returnvalue 6e+02 (Utilities|Array|MakeArray "ObjectTypeQuery7" "ObjectTypeQuery9") false 0 "None"))
  (if _returnvalue_2
    (for _array_element _outhits
      (Class|HealthDamageInterface|DealingDamage(Message) (.HitActor (Collision|BreakHitResult _array_element)) 30 0 "Melee")))
  (Actor|DestroyActor))

(event Custom|Enable%20Mine
  (Collision|SetCollisionEnabled (Variables|Default|GetTriggerCol) "QueryOnly"))

(event EventBeginPlay
  (Utilities|Time|SetTimerbyFunctionName 0 "Enable Mine" 1.0)
  (Utilities|FlowControl|Delay 1e+01)
  (CallFunction|ExplodePlz))

(fn ConstructionScript)