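; Lightsaber blade trace component that detects hits along the path the blade sweeps during an attack.
; While Attack is set, each Tick line-traces from the previous world location to the current one against a custom object channel, ignoring the owning character.
; It stores the result in HitResult and IHitSomething, and StartNewLoc reseeds the start point for a new swing.
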(event EventTick
  (params (DeltaSeconds :type Float%20%28single-precision%29))
  (bind _returnvalue (Transformation|GetWorldLocation))
  (if (Variables|Default|GetAttack?)
    (if (Variables|Default|GetStartNewLoc)
      (Variables|Default|SetStartNewLoc false)
      (Variables|Default|SetLastLocation (Transformation|GetWorldLocation)))
    (bind (_outhit _returnvalue_2) (Collision|LineTraceForObjects (Variables|Default|GetLastLocation) _returnvalue (Utilities|Array|MakeArray "ObjectTypeQuery7") false (Utilities|Array|MakeArray (Variables|Default|GetCharRef)) "ForDuration"))
    (Variables|Default|SetLastLocation _returnvalue)
    (if _returnvalue_2
      (Variables|Default|SetI%20Hit%20Something? true)
      (Variables|Default|SetHitResult _outhit)
      (else
        (Variables|Default|SetI%20Hit%20Something? false)))))

(event EventBeginPlay)