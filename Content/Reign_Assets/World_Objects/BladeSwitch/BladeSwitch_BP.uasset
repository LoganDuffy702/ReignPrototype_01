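; BladeSwitch is a puzzle object with three overlap switches that remove a wall when all are active at once.
; Each switch's overlap swaps its mesh material, sets its active flag and runs a shared check that destroys the Wall component.
; A one-second retriggerable delay per switch then restores the material and clears the flag, so all three must be triggered within that short window.
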(event OnComponentBeginOverlap(SwitchCollision1)
  (params (OverlappedComponent :type Primitive%20Component%20Object%20Reference) (OtherActor :type Actor%20Object%20Reference) (OtherComp :type Primitive%20Component%20Object%20Reference) (OtherBodyIndex :type Integer) (bFromSweep :type Boolean) (SweepResult :type Hit%20Result%20Structure%20%28by%20ref%29))
  (bind _staticmesh (Variables|Default|GetStaticMesh))
  (Rendering|Material|SetMaterial _staticmesh 0 "/Game/Reign_Assets/EnemyObjects/Grapple_Objects/Grapple_Mats/NonMoving_Grapple_Mat.NonMoving_Grapple_Mat")
  (Variables|Default|SetS1Active? true)
  (CallFunction|Checkforactives)
  (Utilities|FlowControl|RetriggerableDelay 1.0)
  (Rendering|Material|SetMaterial _staticmesh 0 "/Game/Reign_Assets/EnemyObjects/Grapple_Objects/Grapple_Mats/Launch_Grapple_Mat.Launch_Grapple_Mat")
  (Variables|Default|SetS1Active? false))

(event OnComponentBeginOverlap(SwitchCollision2)
  (params (OverlappedComponent :type Primitive%20Component%20Object%20Reference) (OtherActor :type Actor%20Object%20Reference) (OtherComp :type Primitive%20Component%20Object%20Reference) (OtherBodyIndex :type Integer) (bFromSweep :type Boolean) (SweepResult :type Hit%20Result%20Structure%20%28by%20ref%29))
  (Rendering|Material|SetMaterial (Variables|Default|GetStaticMesh1) 0 "/Game/Reign_Assets/EnemyObjects/Grapple_Objects/Grapple_Mats/NonMoving_Grapple_Mat.NonMoving_Grapple_Mat")
  (Variables|Default|SetS2Active? true)
  (CallFunction|Checkforactives)
  (Utilities|FlowControl|RetriggerableDelay 1.0)
  (Rendering|Material|SetMaterial (Variables|Default|GetStaticMesh1) 0 "/Game/Reign_Assets/EnemyObjects/Grapple_Objects/Grapple_Mats/Launch_Grapple_Mat.Launch_Grapple_Mat")
  (Variables|Default|SetS2Active? false))

(event OnComponentBeginOverlap(SwitchCollision3)
  (params (OverlappedComponent :type Primitive%20Component%20Object%20Reference) (OtherActor :type Actor%20Object%20Reference) (OtherComp :type Primitive%20Component%20Object%20Reference) (OtherBodyIndex :type Integer) (bFromSweep :type Boolean) (SweepResult :type Hit%20Result%20Structure%20%28by%20ref%29))
  (bind _staticmesh2 (Variables|Default|GetStaticMesh2))
  (Rendering|Material|SetMaterial _staticmesh2 0 "/Game/Reign_Assets/EnemyObjects/Grapple_Objects/Grapple_Mats/NonMoving_Grapple_Mat.NonMoving_Grapple_Mat")
  (Variables|Default|SetS3Active? true)
  (CallFunction|Checkforactives)
  (Utilities|FlowControl|RetriggerableDelay 1.0)
  (Rendering|Material|SetMaterial _staticmesh2 0 "/Game/Reign_Assets/EnemyObjects/Grapple_Objects/Grapple_Mats/Launch_Grapple_Mat.Launch_Grapple_Mat")
  (Variables|Default|SetS3Active? false))

(event Custom|Checkforactives
  (Utilities|IsValid (Variables|Default|GetWall)
    (:Is%20Valid
      (if (Math|Boolean|ANDBoolean (Variables|Default|GetS1Active?) (Variables|Default|GetS2Active?) (Variables|Default|GetS3Active?))
        (Components|DestroyComponent (Variables|Default|GetWall))))))

(event EventBeginPlay)

(event Collision|EventActorBeginOverlap
  (params (OtherActor :type Actor%20Object%20Reference)))

(event EventTick
  (params (DeltaSeconds :type Float%20%28single-precision%29)))

(event EventDealingDamage
  (params (Sent%20Damage :type Integer) (Sender :type Actor%20Object%20Reference) (DamageType :type Name :default "None")))

(fn ConstructionScript)