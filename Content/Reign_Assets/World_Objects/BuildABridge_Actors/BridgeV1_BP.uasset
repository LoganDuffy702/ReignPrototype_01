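; Bridge actor that builds itself panel by panel at BeginPlay, after a one-second delay.
; PrintCubes runs a DoN and Delay loop, spawning Bridge_Panel_BP along Start's forward vector at SeperationDistance steps, paced by PrintDelay.
; Panel count derives from the Start-to-End distance in fixed 100-unit divisions, minus one, independent of SeperationDistance.
; Panels inherit the actor's rotation and Y/Z scale, with X scale fixed at one.
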(event Custom|PrintCubes
  (bind _returnvalue (Transformation|GetActorTransform))
  (bind _start (Variables|Default|GetStart))
  (Utilities|FlowControl|Delay 1.0)
  (bind _counter (Utilities|FlowControl|DoN (- (.ReturnValue (Math|Float|Division(WholeandRemainder) (Math|Vector|VectorLength (- (Transformation|GetWorldLocation (Variables|Default|GetStart)) (Transformation|GetWorldLocation (Variables|Default|GetEnd)))) 1e+02)) 1) :!label _label)
    (:Exit
      (Variables|Default|SetFinalDistance (* _counter (Variables|Default|GetSeperationDistance)))
      (Game|SpawnActorfromClass "/Game/Reign_Assets/World_Objects/BuildABridge_Actors/Bridge_Panel_BP.Bridge_Panel_BP_C" (Math|Transform|MakeTransform (+ (* (Math|Vector|GetForwardVector (Transformation|GetWorldRotation _start)) (Variables|Default|GetFinalDistance)) (Transformation|GetWorldLocation _start)) (.rotation _returnvalue) (Math|Vector|MakeVector 1.0 (.y (.scale _returnvalue)) (.z (.scale _returnvalue)))) "Undefined" 0 0)
      (Utilities|FlowControl|Delay (Variables|Default|GetPrint%20Delay))
      (goto _label))))

(event EventBeginPlay
  (CallFunction|PrintCubes))

(event Collision|EventActorBeginOverlap
  (params (OtherActor :type Actor%20Object%20Reference)))

(event EventTick
  (params (DeltaSeconds :type Float%20%28single-precision%29)))

(fn ConstructionScript)