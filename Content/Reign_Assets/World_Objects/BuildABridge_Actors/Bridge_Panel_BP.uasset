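; Bridge panel actor for the build-a-bridge world objects, with a randomized material-driven resting offset.
; The construction script gives the Panel a dynamic Limbo test material instance and sets its "Resting Offset" to a random vector bounded partly by SpawnDistance.
; BeginPlay caches the panel's world location and scale.
; The transform logic that would restore or zero-scale the panel is disconnected and never runs.
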(event EventBeginPlay
  (bind _panel (Variables|Default|GetPanel))
  (Variables|Default|SetOriginalScale (Transformation|GetWorldScale _panel))
  (Variables|Default|SetOrgin (Transformation|GetWorldLocation _panel)))

(event Collision|EventActorBeginOverlap
  (params (OtherActor :type Actor%20Object%20Reference)))

(event EventTick
  (params (DeltaSeconds :type Float%20%28single-precision%29)))

(fn ConstructionScript
  (bind _spawndistance (Variables|Default|GetSpawnDistance))
  (bind _returnvalue (* _spawndistance -1.0))
  (bind _returnvalue_2 (Math|Random|RandomFloatinRange _returnvalue 1e+01))
  (for _array_element (Utilities|Array|MakeArray (Variables|Default|GetPanel))
    (Rendering|Material|CreateDynamicMaterialInstance _array_element 0 "/Game/Reign_Assets/Foliage/Limbo_Foliage/Limbo_Test_Mat_Inst.Limbo_Test_Mat_Inst" "None" :!class /Script/Engine.PrimitiveComponent)
    (Rendering|Material|SetVectorParameterValueonMaterials _array_element "Resting Offset" (Math|Vector|MakeVector _returnvalue_2 (Math|Random|RandomFloatinRange _returnvalue _spawndistance) _returnvalue_2))))