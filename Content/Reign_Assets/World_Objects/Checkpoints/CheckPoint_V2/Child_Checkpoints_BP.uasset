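; Child checkpoint obelisk that works under a Mast_Checkpoint_V2 master and becomes active on any box overlap, or shortly after ChildStartUp is called.
; On BeginPlay it caches the master, all child checkpoints and a dynamic obelisk material with glow on.
; Activation calls the master's DeactivateMastCheckPoint with itself, starts the particles, turns glow off and sets Active.
; DeactiveChildCP restores the glow, stops particles and clears Active.
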(event OnComponentBeginOverlap(Box)
  (params (OverlappedComponent :type Primitive%20Component%20Object%20Reference) (OtherActor :type Actor%20Object%20Reference) (OtherComp :type Primitive%20Component%20Object%20Reference) (OtherBodyIndex :type Integer) (bFromSweep :type Boolean) (SweepResult :type Hit%20Result%20Structure%20%28by%20ref%29))
  (Default|DeactivateMastCheckPoint (Variables|Default|GetMasterCheckpoint) self)
  (Components|Activation|Activate (Variables|Default|GetParticleSystem) false)
  (Rendering|Material|SetScalarParameterValue (Variables|Default|GetDyn%20Mat) "Glow" 0.0 :!class /Script/Engine.MaterialInstanceDynamic)
  (Variables|Default|SetActive? true))

(event Custom|Deactive%20Child%20CP
  (Rendering|Material|SetScalarParameterValue (Variables|Default|GetDyn%20Mat) "Glow" 6.0 :!class /Script/Engine.MaterialInstanceDynamic)
  (Components|Activation|Deactivate (Variables|Default|GetParticleSystem))
  (Variables|Default|SetActive? false))

(event Custom|ChildStartUp
  (Utilities|FlowControl|Delay 0.2)
  (Default|DeactivateMastCheckPoint (Variables|Default|GetMasterCheckpoint) self)
  (Components|Activation|Activate (Variables|Default|GetParticleSystem) false)
  (Rendering|Material|SetScalarParameterValue (Variables|Default|GetDyn%20Mat) "Glow" 0.0 :!class /Script/Engine.MaterialInstanceDynamic)
  (Variables|Default|SetActive? true))

(event EventBeginPlay
  (bind _outactors (Actor|GetAllActorsOfClass "/Game/Reign_Assets/World_Objects/Checkpoints/CheckPoint_V2/Mast_Checkpoint_V2.Mast_Checkpoint_V2_C"))
  (Variables|Default|SetMasterCheckpoint (Utilities|Array|Get(acopy) _outactors))
  (bind _returnvalue (Rendering|Material|CreateDynamicMaterialInstance (Variables|Default|GetObelisk) 0 0 "None" :!class /Script/Engine.PrimitiveComponent))
  (bind _output_get (Variables|Default|SetDyn%20Mat _returnvalue))
  (Rendering|Material|SetScalarParameterValue _output_get "Glow" 6.0 :!class /Script/Engine.MaterialInstanceDynamic)
  (bind _outactors_2 (Actor|GetAllActorsOfClass "Child_Checkpoints_BP_C"))
  (Variables|Default|SetChildCp _outactors_2))

(fn ConstructionScript)