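; Test switch actor from the CheckPoint_V2 folder that makes one instance at a time the active one, shown by a hidden sphere.
; Capsule overlap by any actor stores it in PlayerTouched, hides this sphere, then calls ResetSwitch on every other SwitchTest_BP in the level to show theirs again.
; Ending the overlap clears PlayerTouched but leaves the sphere hidden.
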(event OnComponentBeginOverlap(Capsule)
  (params (OverlappedComponent :type Primitive%20Component%20Object%20Reference) (OtherActor :type Actor%20Object%20Reference) (OtherComp :type Primitive%20Component%20Object%20Reference) (OtherBodyIndex :type Integer) (bFromSweep :type Boolean) (SweepResult :type Hit%20Result%20Structure%20%28by%20ref%29))
  (Variables|Default|SetPlayerTouched OtherActor)
  (Rendering|SetVisibility (Variables|Default|GetSphere) false false)
  (bind _outactors (Actor|GetAllActorsOfClass "SwitchTest_BP_C"))
  (for _array_element _outactors
    (if (not (== _array_element self))
      (CallFunction|ResetSwitch _array_element))))

(event OnComponentEndOverlap(Capsule)
  (params (OverlappedComponent :type Primitive%20Component%20Object%20Reference) (OtherActor :type Actor%20Object%20Reference) (OtherComp :type Primitive%20Component%20Object%20Reference) (OtherBodyIndex :type Integer))
  (Variables|Default|SetPlayerTouched 0))

(event EventBeginPlay)

(event Collision|EventActorBeginOverlap
  (params (OtherActor :type Actor%20Object%20Reference)))

(event EventTick
  (params (DeltaSeconds :type Float%20%28single-precision%29)))

(fn ConstructionScript)

(fn ResetSwitch
  (Rendering|SetVisibility (Variables|Default|GetSphere) true false))