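; Small EXP orb pickup that scatters on spawn, homes to the player and grants experience on contact.
; The construction script randomizes launch speed and an upward-biased direction; after a short delay it stops, enabling homing and overlap events.
; Any attract-sphere overlap sets the player's capsule as homing target.
; Player contact with the orb calls EXPExchange with HealAmount and destroys it; otherwise a timer destroys it after a few seconds.
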(event OnComponentBeginOverlap(AttactSphere)
  (params (OverlappedComponent :type Primitive%20Component%20Object%20Reference) (OtherActor :type Actor%20Object%20Reference) (OtherComp :type Primitive%20Component%20Object%20Reference) (OtherBodyIndex :type Integer) (bFromSweep :type Boolean) (SweepResult :type Hit%20Result%20Structure%20%28by%20ref%29))
  ;[1 1 1] Trigger checks
  (Variables|Default|SetLastLocation (Transformation|GetWorldLocation (Variables|Default|GetOrb)))
  (bind _asmc_prototype_bp (Utilities|Casting|CastToMC_Prototype_BP (Game|GetPlayerCharacter 0)))
  (bind _output_get (Variables|Default|SetPlayerRef _asmc_prototype_bp))
  (Variables|/Script/Engine.ProjectileMovementComponent|SetHomingTargetComponent (Variables|Default|GetProjectileMovement) (Variables|/Script/Engine.Character|GetCapsuleComponent _output_get)))

(event OnComponentBeginOverlap(Orb)
  (params (OverlappedComponent :type Primitive%20Component%20Object%20Reference) (OtherActor :type Actor%20Object%20Reference) (OtherComp :type Primitive%20Component%20Object%20Reference) (OtherBodyIndex :type Integer) (bFromSweep :type Boolean) (SweepResult :type Hit%20Result%20Structure%20%28by%20ref%29))
  ;[1 1 1] Trigger checks
  (if (== OtherActor (Game|GetPlayerCharacter 0))
    (bind _asmc_prototype_bp (Utilities|Casting|CastToMC_Prototype_BP (Game|GetPlayerCharacter 0)))
    (Variables|Default|SetPlayerRef _asmc_prototype_bp)
    (Default|EXPExchange (Variables|Default|GetPlayerRef) (Variables|Default|GetHealAmount))
    (Actor|DestroyActor)))

(event Custom|KillMe
  ;[1 1 1] Death Event
  (Actor|DestroyActor))

(event EventBeginPlay
  (bind _projectilemovement (Variables|Default|GetProjectileMovement))
  (Utilities|Time|SetTimerbyFunctionName 0 "KillMe" 5.0)
  (Utilities|FlowControl|Delay 0.7)
  ;[1 1 1] Turns on the homing stuff
  (Variables|/Script/Engine.ProjectileMovementComponent|SetMaxSpeed _projectilemovement 0.0)
  (Variables|/Script/Engine.ProjectileMovementComponent|SetInitialSpeed _projectilemovement 0.0)
  (Variables|/Script/Engine.MovementComponent|SetVelocity _projectilemovement "0, 0, 0")
  (Variables|/Script/Engine.ProjectileMovementComponent|SetbIsHomingProjectile _projectilemovement true)
  (Variables|/Script/Engine.PrimitiveComponent|SetbGenerateOverlapEvents (Variables|Default|GetAttactSphere) true)
  (Variables|/Script/Engine.PrimitiveComponent|SetbGenerateOverlapEvents (Variables|Default|GetOrb) true))

(fn ConstructionScript
  (bind _projectilemovement (Variables|Default|GetProjectileMovement))
  (Variables|/Script/Engine.ProjectileMovementComponent|SetInitialSpeed _projectilemovement (Math|Random|RandomFloatinRange 3e+02 1e+03))
  (Variables|/Script/Engine.MovementComponent|SetVelocity _projectilemovement (Math|Vector|MakeVector (Math|Random|RandomFloatinRange -1.0 1.0) (Math|Random|RandomFloatinRange -1.0 1.0) (Math|Random|RandomFloatinRange 0.0 1.0))))