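; Healing heart drop that launches in a random, non-downward direction at random speed via its projectile movement, set in the construction script.
; Overlap events switch on after a short delay, and a timer destroys uncollected hearts.
; The first overlap by any actor heals the player through DealingDamage with negative damage, plays sound and particles, then destroys the heart.
; Homing setup exists but is never executed.
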(event OnComponentBeginOverlap(Parent)
  (params (OverlappedComponent :type Primitive%20Component%20Object%20Reference) (OtherActor :type Actor%20Object%20Reference) (OtherComp :type Primitive%20Component%20Object%20Reference) (OtherBodyIndex :type Integer) (bFromSweep :type Boolean) (SweepResult :type Hit%20Result%20Structure%20%28by%20ref%29))
  ;[1 1 1] Trigger checks
  (Utilities|FlowControl|DoOnce false
    (:Completed
      (Audio|PlaySound2D "/Game/Reign_Assets/Sounds/Magic_1_Cue.Magic_1_Cue" 0.4 1.0 0.0 0 0)
      (Effects|SpawnEmitteratLocation "/Game/Reign_Assets/World_Objects/Tunnel_Object/Tunnel_Spawn_FX.Tunnel_Spawn_FX" (Transformation|GetActorLocation))
      (Default|DealingDamage (Variables|Default|GetPlayerRef) -2 0 "None")
      (Actor|DestroyActor))))

(event Custom|KillMe
  ;[1 1 1] Death Event
  (Actor|DestroyActor))

(event EventBeginPlay
  (bind _asmc_prototype_bp (Utilities|Casting|CastToMC_Prototype_BP (Game|GetPlayerCharacter 0)))
  (Variables|Default|SetPlayerRef _asmc_prototype_bp)
  (Utilities|Time|SetTimerbyFunctionName 0 "KillMe" 2e+01)
  (Utilities|FlowControl|Delay 0.7)
  (Variables|/Script/Engine.PrimitiveComponent|SetbGenerateOverlapEvents (Variables|Default|GetParent) true))

(fn ConstructionScript
  (bind _projectilemovement (Variables|Default|GetProjectileMovement))
  (Variables|/Script/Engine.ProjectileMovementComponent|SetInitialSpeed _projectilemovement (Math|Random|RandomFloatinRange 6e+02 1.5e+03))
  (Variables|/Script/Engine.MovementComponent|SetVelocity _projectilemovement (Math|Vector|MakeVector (Math|Random|RandomFloatinRange -1.0 1.0) (Math|Random|RandomFloatinRange -1.0 1.0) (Math|Random|RandomFloatinRange 0.0 1.0))))