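; Healing orb drop that homes in on the player character and applies healing on contact.
; One second after spawn its projectile movement enables homing.
; Any overlap on the attract sphere stores the player and targets their capsule.
; Any overlap on the death sphere passes HealAmount through the player's DealingDamage function, attaches a healing effect and destroys the orb.
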(event OnComponentBeginOverlap(DeathSphere)
  (params (OverlappedComponent :type Primitive%20Component%20Object%20Reference) (OtherActor :type Actor%20Object%20Reference) (OtherComp :type Primitive%20Component%20Object%20Reference) (OtherBodyIndex :type Integer) (bFromSweep :type Boolean) (SweepResult :type Hit%20Result%20Structure%20%28by%20ref%29))
  (Default|DealingDamage (Variables|Default|GetPlayerRef) (Variables|Default|GetHealAmount) self)
  (Effects|SpawnEmitterAttached "/Game/Reign_Assets/World_Objects/Drop_Objects/Healing_Active_FX.Healing_Active_FX" (Variables|/Script/Engine.Character|GetCapsuleComponent (Variables|Default|GetPlayerRef)) "Spine" "0, 0,-50.000000" "0, 0, 0" "1.000000,1.000000,1.000000" "SnapToTarget")
  (Actor|DestroyActor))

(event OnComponentBeginOverlap(AttactSphere)
  (params (OverlappedComponent :type Primitive%20Component%20Object%20Reference) (OtherActor :type Actor%20Object%20Reference) (OtherComp :type Primitive%20Component%20Object%20Reference) (OtherBodyIndex :type Integer) (bFromSweep :type Boolean) (SweepResult :type Hit%20Result%20Structure%20%28by%20ref%29))
  (bind _asmc_prototype_bp (Utilities|Casting|CastToMC_Prototype_BP (Game|GetPlayerCharacter 0)))
  (Variables|Default|SetPlayerRef _asmc_prototype_bp)
  (Variables|/Script/Engine.ProjectileMovementComponent|SetHomingTargetComponent (Variables|Default|GetProjectileMovement) (Variables|/Script/Engine.Character|GetCapsuleComponent _asmc_prototype_bp)))

(event EventBeginPlay
  (Utilities|FlowControl|Delay 1.0)
  (Variables|/Script/Engine.ProjectileMovementComponent|SetbIsHomingProjectile (Variables|Default|GetProjectileMovement) true))

(fn ConstructionScript)