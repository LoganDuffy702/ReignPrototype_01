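; Healing pickup in the world objects drop set that restores player health when its overlap fires.
; A looping timeline bobs the static mesh vertically around its starting location.
; On overlap it plays a sound and particle effect, heals the cached MC_Prototype_BP player through DealingDamage with negative "Health" damage, then destroys itself.
; The overlap does not check which actor triggered it.
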(event OnComponentBeginOverlap(Parent)
  (params (OverlappedComponent :type Primitive%20Component%20Object%20Reference) (OtherActor :type Actor%20Object%20Reference) (OtherComp :type Primitive%20Component%20Object%20Reference) (OtherBodyIndex :type Integer) (bFromSweep :type Boolean) (SweepResult :type Hit%20Result%20Structure%20%28by%20ref%29))
  (Audio|PlaySound2D "/Game/Reign_Assets/Sounds/Magic_1_Cue.Magic_1_Cue" 0.4 1.0 0.0 0 0)
  (Effects|SpawnEmitteratLocation "/Game/Reign_Assets/World_Objects/Tunnel_Object/Tunnel_Spawn_FX.Tunnel_Spawn_FX" (Transformation|GetActorLocation))
  (Default|DealingDamage (Variables|Default|GetPlayerRef) -1 0 "Health")
  (Actor|DestroyActor))

(event Custom|Hover
  (bind _newtrack_0 (Timeline|Timeline_0 PlayFromStart)
    (:Update
      (Transformation|SetWorldLocation (Variables|Default|GetStaticMesh) (+ (Variables|Default|GetOriginLoc) (Math|Vector|MakeVector 0.0 0.0 (* _newtrack_0 1e+02))) false false))
    (:Finished
      (CallFunction|Hover))))

(event EventBeginPlay
  (Variables|Default|SetOriginLoc (Transformation|GetWorldLocation (Variables|Default|GetStaticMesh)))
  (CallFunction|Hover)
  (bind _asmc_prototype_bp (Utilities|Casting|CastToMC_Prototype_BP (Game|GetPlayerCharacter 0)))
  (Variables|Default|SetPlayerRef _asmc_prototype_bp))

(fn ConstructionScript)