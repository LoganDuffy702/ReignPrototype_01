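; Ground pressure switch that signals linked Walls when an actor steps onto or is placed on it.
; Overlapping the T1 component sets Active, lowers the Button and calls CanIOpen, which sends SwitchInterface(true) to Walls.
; Ending the overlap clears Active and raises the Button but sends nothing to Walls.
; Any actor triggers it, as the check involving PushAndPull_1_BP is disconnected.
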(event OnComponentEndOverlap(T1)
  (params (OverlappedComponent :type Primitive%20Component%20Object%20Reference) (OtherActor :type Actor%20Object%20Reference) (OtherComp :type Primitive%20Component%20Object%20Reference) (OtherBodyIndex :type Integer))
  (Variables|Default|SetActive? false)
  (Transformation|SetRelativeLocation (Variables|Default|GetButton) "0, 0, 0" false false))

(event OnComponentBeginOverlap(T1)
  (params (OverlappedComponent :type Primitive%20Component%20Object%20Reference) (OtherActor :type Actor%20Object%20Reference) (OtherComp :type Primitive%20Component%20Object%20Reference) (OtherBodyIndex :type Integer) (bFromSweep :type Boolean) (SweepResult :type Hit%20Result%20Structure%20%28by%20ref%29))
  (Variables|Default|SetActive? true)
  (Transformation|SetRelativeLocation (Variables|Default|GetButton) "0, 0,-10.000000" false false)
  (CallFunction|CanIOpen?))

(event Custom|Can%20I%20Open?
  (Default|SwitchInterface (Variables|Default|GetWalls) true))

(event EventBeginPlay)

(fn ConstructionScript)