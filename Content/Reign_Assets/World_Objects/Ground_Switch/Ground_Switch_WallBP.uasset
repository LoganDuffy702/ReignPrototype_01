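; Ground switch wall Blueprint that opens when all of its linked ground switches are active.
; On each SwitchInterface event it loops through the GroundSwitches array, stopping at the first inactive switch.
; If all are active it hides the Cube and disables the Box collision; otherwise it shows the Cube and restores query and physics collision.
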(event EventBeginPlay)

(event Collision|EventActorBeginOverlap
  (params (OtherActor :type Actor%20Object%20Reference)))

(event EventTick
  (params (DeltaSeconds :type Float%20%28single-precision%29)))

(event EventSwitchInterface
  (params (Activate%20Switch? :type Boolean))
  (bind _cube (Variables|Default|GetCube))
  (bind _box (Variables|Default|GetBox))
  (Variables|Default|SetAll%20True? true)
  (bind _array_element (Utilities|Array|ForEachLoopwithBreak (Variables|Default|GetGroundSwitches) :!label _label)
    (:LoopBody
      (if (not (Variables|/Game/Reign_Assets/World_Objects/Ground_Switch/GroundSwitch_BP.GroundSwitch_BP_C|GetActive? _array_element))
        (Variables|Default|SetAll%20True? false)
        (goto _label Break)))
    (:Completed
      (if (Variables|Default|GetAll%20True?)
        (Rendering|SetVisibility _cube false false)
        (Collision|SetCollisionEnabled _box "NoCollision")
        (else
          (Rendering|SetVisibility _cube true false)
          (Collision|SetCollisionEnabled _box "QueryAndPhysics"))))))

(fn ConstructionScript)