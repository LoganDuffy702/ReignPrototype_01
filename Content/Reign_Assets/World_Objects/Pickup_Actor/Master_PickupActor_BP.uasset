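; Base-style pickup actor that spins its mesh in the world and offers a weapon to the player character.
; A self-restarting timeline drives a continuous yaw rotation from BeginPlay.
; Overlapping the collision shows the pickup widget for any actor, then sets AttachedWeapon on MC_Prototype_BP to ItemToAdd.
; Ending overlap hides the widget and clears that reference; the pickup action itself is not handled here.
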(event OnComponentBeginOverlap(Collision)
  (params (OverlappedComponent :type Primitive%20Component%20Object%20Reference) (OtherActor :type Actor%20Object%20Reference) (OtherComp :type Primitive%20Component%20Object%20Reference) (OtherBodyIndex :type Integer) (bFromSweep :type Boolean) (SweepResult :type Hit%20Result%20Structure%20%28by%20ref%29))
  ;[1 1 1] Setting text visibilty, and sending the Attached weapon class value to the main char.
  (Rendering|SetVisibility (Variables|Default|GetPickupWidget) true false)
  (bind _asmc_prototype_bp (Utilities|Casting|CastToMC_Prototype_BP OtherActor))
  (Variables|/Game/Reign_Assets/Player_Character/Blueprints/MC_Prototype_BP.MC_Prototype_BP_C|SetAttachedWeapon _asmc_prototype_bp (Variables|Default|GetItemToAdd)))

(event OnComponentEndOverlap(Collision)
  (params (OverlappedComponent :type Primitive%20Component%20Object%20Reference) (OtherActor :type Actor%20Object%20Reference) (OtherComp :type Primitive%20Component%20Object%20Reference) (OtherBodyIndex :type Integer))
  ;[1 1 1] Same as top but if they leave the area there is nothing to pick up
  (Rendering|SetVisibility (Variables|Default|GetPickupWidget) false false)
  (bind _asmc_prototype_bp (Utilities|Casting|CastToMC_Prototype_BP OtherActor))
  (Variables|/Game/Reign_Assets/Player_Character/Blueprints/MC_Prototype_BP.MC_Prototype_BP_C|SetAttachedWeapon _asmc_prototype_bp 0))

(event Custom|Hover
  (bind _newtrack_0 (Timeline|Timeline_0 PlayFromStart)
    (:Update
      (Transformation|SetRelativeRotation (Variables|Default|GetStaticMesh) (Math|Rotator|MakeRotator 0.0 0.0 (* _newtrack_0 3.6e+02)) false false))
    (:Finished
      (CallFunction|Hover))))

(event EventBeginPlay
  (CallFunction|Hover))

(fn ConstructionScript)