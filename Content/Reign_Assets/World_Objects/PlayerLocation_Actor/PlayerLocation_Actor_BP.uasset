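; World helper actor that tracks the player each Tick and handles fall-off deaths.
; It writes player capsule and camera locations to a material parameter collection for shaders and keeps a spinning companion pivot on the player.
; Falling to a fixed low Z moves the player to the last clicked checkpoint in CheckPoints list order, or reloads the level if none is clicked.
; The aiming arrow event is empty, its logic left disconnected.
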(event Custom|FalloffDeath
  ;[1 1 1] Death Event
  (if (not (Variables|Default|GetIsFallOffFuncCalled))
    (if (<= (.z (Transformation|GetActorLocation (Variables|Default|GetPlayerRef))) -6e+02)
      (Variables|Default|SetIsFallOffFuncCalled true)
      (CallFunction|FindNewestCheckpoint))))

(event Custom|Set%20Companion%20Event
  (bind _companionrotactor (Variables|Default|GetCompanionRotActor))
  ;[1 1 1] Companion
  (Transformation|SetWorldLocation _companionrotactor (Transformation|GetActorLocation (Variables|Default|GetPlayerRef)) false false)
  (Transformation|AddWorldRotation _companionrotactor (Math|Rotator|MakeRotator 0.0 0.0 (* (Variables|Default|GetDelta%20Time) (Variables|Default|GetRotationRate))) false false))

(event Custom|Set%20Aiming%20Arrow%20Event
  ;[1 1 1] Aiming Arrow
)

(event Custom|Material%20Param%20Event
  ;[1 1 1] Material Event
  (bind _asmc_prototype_bp (Utilities|Casting|CastToMC_Prototype_BP (Game|GetPlayerCharacter 0)))
  (bind _output_get (Variables|Default|SetPlayerRef _asmc_prototype_bp))
  (Rendering|Material|SetVectorParameterValue "/Game/Reign_Assets/Materials/Landscape_Mats/PlayerLocation_Param.PlayerLocation_Param" "PlayerLocation" (Math|Conversions|ToLinearColor(Vector) (Transformation|GetWorldLocation (Variables|/Script/Engine.Character|GetCapsuleComponent _output_get))) :!class /Script/Engine.KismetMaterialLibrary)
  (Rendering|Material|SetVectorParameterValue "/Game/Reign_Assets/Materials/Landscape_Mats/PlayerLocation_Param.PlayerLocation_Param" "CameraLocation" (Math|Conversions|ToLinearColor(Vector) (Transformation|GetWorldLocation (Variables|/Game/Reign_Assets/Player_Character/Blueprints/MC_Prototype_BP.MC_Prototype_BP_C|GetCamera (Variables|Default|GetPlayerRef)))) :!class /Script/Engine.KismetMaterialLibrary))

(event Custom|FindNewestCheckpoint
  (Variables|Default|SetFoundCheckPoint false)
  (for _array_element (Utilities|Struct|BreakArrayOfActor (Variables|Default|GetCheckPoints))
    (bind _ascheckpoint (Utilities|Casting|CastToCheckpoint _array_element)
      (:then
        (if (Variables|/Game/Reign_Assets/World_Objects/Checkpoints/Checkpoint.Checkpoint_C|GetWasClicked _ascheckpoint)
          (Variables|Default|SetNearestCheckpoint _ascheckpoint)
          (Variables|Default|SetFoundCheckPoint true)))
      (:CastFailed
        (Development|PrintString "CAST FAILED ARRAY CONTAINS OBJECT THAT IS NOT A CHECKPOINT BP AT Index:"))))
  (if (Variables|Default|GetFoundCheckPoint)
    (bind _asmc_prototype_bp (Utilities|Casting|CastToMC_Prototype_BP (Game|GetPlayerCharacter 0)))
    (Transformation|SetActorLocation _asmc_prototype_bp (Transformation|GetActorLocation (Variables|Default|GetNearestCheckpoint)) false false)
    (Variables|Default|SetIsFallOffFuncCalled false)
    (else
      (bind _returnvalue (Game|GetCurrentLevelName true))
      (Game|OpenLevel(byName) (Utilities|String|StringToName _returnvalue)))))

(event EventTick
  (params (DeltaSeconds :type Float%20%28single-precision%29))
  (Variables|Default|SetDelta%20Time DeltaSeconds)
  (CallFunction|MaterialParamEvent)
  (CallFunction|SetCompanionEvent)
  (CallFunction|SetAimingArrowEvent)
  (CallFunction|FalloffDeath))

(fn ConstructionScript)