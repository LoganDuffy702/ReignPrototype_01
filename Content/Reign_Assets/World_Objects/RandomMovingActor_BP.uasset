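; Prototype actor apparently meant to reposition randomly around the player, but its movement logic is disconnected.
; BeginPlay stores the spawn location after a delay, and Tick only caches delta time.
; RandLoc debug-traces from the player capsule toward a random XY offset and sets itself on a looping timer.
; Nothing live calls RandLoc or sets PlayerRef; the player cast, interpolated drift and teleport chains never run.
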(event Custom|RandLoc
  (bind _returnvalue (Math|Random|RandomFloatinRange -1.0 1.0))
  (bind _player_ref (Variables|Default|GetPlayer%20Ref))
  (bind _returnvalue_2 (Math|Float|Round _returnvalue))
  (bind _capsulecomponent (Variables|/Script/Engine.Character|GetCapsuleComponent _player_ref))
  (bind _returnvalue_3 (Transformation|GetWorldLocation _capsulecomponent))
  (bind (_x _y _z) (Math|Vector|BreakVector _returnvalue_3))
  (Collision|LineTraceByChannel (Transformation|GetWorldLocation (Variables|/Script/Engine.Character|GetCapsuleComponent (Variables|Default|GetPlayer%20Ref))) (Math|Vector|MakeVector (+ _x (* _returnvalue_2 (Math|Random|RandomFloatinRange 3e+02 5e+02))) (+ _y (* _returnvalue_2 (Math|Random|RandomFloatinRange 3e+02 5e+02))) _z) "TraceTypeQuery1" false 0 "ForDuration" true "(R=0.000000,G=1.000000,B=0.172497,A=1.000000)" "(R=0.000000,G=0.953292,B=1.000000,A=1.000000)")
  (Utilities|Time|SetTimerbyFunctionName 0 "RandLoc" 0.2 true))

(event EventBeginPlay
  (Utilities|FlowControl|Delay 1.0)
  (Variables|Default|SetOrigin%20Location (Transformation|GetActorLocation)))

(event Collision|EventActorBeginOverlap
  (params (OtherActor :type Actor%20Object%20Reference)))

(event EventTick
  (params (DeltaSeconds :type Float%20%28single-precision%29))
  (Variables|Default|SetDelta%20time DeltaSeconds))

(fn ConstructionScript)