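; Tower world object that the player blows apart by spending collected enemy souls.
; Overlapping its sphere flags the player as near, without checking which actor entered, and calls ExplodeMe.
; If the cached MC_Prototype_BP player holds at least three souls, it zeroes and refreshes the soul count, fires a radial force impulse, then destroys the tower after a delay.
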(event OnComponentBeginOverlap(Sphere)
  (params (OverlappedComponent :type Primitive%20Component%20Object%20Reference) (OtherActor :type Actor%20Object%20Reference) (OtherComp :type Primitive%20Component%20Object%20Reference) (OtherBodyIndex :type Integer) (bFromSweep :type Boolean) (SweepResult :type Hit%20Result%20Structure%20%28by%20ref%29))
  (Variables|Default|SetPlayerNear? true)
  (CallFunction|ExplodeMe))

(event OnComponentEndOverlap(Sphere)
  (params (OverlappedComponent :type Primitive%20Component%20Object%20Reference) (OtherActor :type Actor%20Object%20Reference) (OtherComp :type Primitive%20Component%20Object%20Reference) (OtherBodyIndex :type Integer))
  (Variables|Default|SetPlayerNear? false))

(event Custom|Explode%20Me
  (bind _playerref (Variables|Default|GetPlayerRef))
  (if (and (Variables|Default|GetPlayerNear?) (>= (Variables|/Game/Reign_Assets/Player_Character/Blueprints/MC_Prototype_BP.MC_Prototype_BP_C|GetEnemySouls (Variables|Default|GetPlayerRef)) 3))
    (Variables|/Game/Reign_Assets/Player_Character/Blueprints/MC_Prototype_BP.MC_Prototype_BP_C|SetEnemySouls _playerref 0)
    (Default|UpdateSouls _playerref)
    (Class|RadialForceComponent|FireImpulse (Variables|Default|GetRadialForce))
    (Variables|Default|SetPlayerNear? false)
    (Utilities|FlowControl|Delay 7.0)
    (Actor|DestroyActor)))

(event EventBeginPlay
  (bind _asmc_prototype_bp (Utilities|Casting|CastToMC_Prototype_BP (Game|GetPlayerCharacter 0)))
  (Variables|Default|SetPlayerRef _asmc_prototype_bp))

(event Collision|EventActorBeginOverlap
  (params (OtherActor :type Actor%20Object%20Reference)))

(fn ConstructionScript)