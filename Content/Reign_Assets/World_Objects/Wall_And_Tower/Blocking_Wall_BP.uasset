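; Blocking wall actor that rises and lowers on command, starting with its plane hidden and collision off.
; RaiseWallEvent uses a timeline to lerp its Z to GrowHeight, then shows the plane, enables collision and spawns a beam linking it to PowerTower's lock-on marker.
; DeactivateEvent hides the plane, destroys the beam and lerps down to negative GrowHeight, disabling collision when finished.
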(event Custom|RaiseWall%20Event
  (Variables|Default|SetOriginLocation (Transformation|GetActorLocation))
  (bind _newtrack_0 (Timeline|UP%20Timeline PlayFromStart)
    (:Update
      (Transformation|SetActorLocation (Math|Vector|Lerp(Vector) (Variables|Default|GetOriginLocation) (Math|Vector|MakeVector (.x (Variables|Default|GetOriginLocation)) (.y (Variables|Default|GetOriginLocation)) (Variables|Default|GetGrowHeight)) _newtrack_0) false false))
    (:Finished
      (Rendering|SetVisibility (Variables|Default|GetPlane) true false)
      (bind _returnvalue (Effects|SpawnEmitteratLocation "/Game/Reign_Assets/FX/Gun/CableBased/Towers/LinkIndecator_FX.LinkIndecator_FX" "0, 0, 0"))
      (Class|ParticleSystemComponent|SetBeamSourcePoint _returnvalue 0 (Transformation|GetWorldLocation (Variables|Default|GetLinkLocation)))
      (Class|ParticleSystemComponent|SetBeamEndPoint _returnvalue 0 (Transformation|GetWorldLocation (Variables|/Game/Reign_Assets/EnemyObjects/Master_LockOn_BP/Master_LockOn_Object_BP.Master_LockOn_Object_BP_C|GetLockOnMarker (Variables|Default|GetPowerTower))))
      (Collision|SetCollisionEnabled (Variables|Default|GetCollisionWall) "QueryAndPhysics"))))

(event Custom|Deactivate%20Event
  (Rendering|SetVisibility (Variables|Default|GetPlane) false false)
  (Variables|Default|SetOriginLocation (Transformation|GetActorLocation))
  (Components|DestroyComponent (stale Custom|RaiseWall%20Event _returnvalue))
  (bind _newtrack_0 (Timeline|Down%20Timeline PlayFromStart)
    (:Update
      (Transformation|SetActorLocation (Math|Vector|Lerp(Vector) (Variables|Default|GetOriginLocation) (Math|Vector|MakeVector (.x (Variables|Default|GetOriginLocation)) (.y (Variables|Default|GetOriginLocation)) (* (Variables|Default|GetGrowHeight) -1.0)) _newtrack_0) false false))
    (:Finished
      (Collision|SetCollisionEnabled (Variables|Default|GetCollisionWall) "NoCollision"))))

(event EventBeginPlay
  (Rendering|SetVisibility (Variables|Default|GetPlane) false false)
  (Collision|SetCollisionEnabled (Variables|Default|GetCollisionWall) "NoCollision"))

(event Collision|EventActorBeginOverlap
  (params (OtherActor :type Actor%20Object%20Reference)))

(event EventTick
  (params (DeltaSeconds :type Float%20%28single-precision%29)))

(fn ConstructionScript)