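; Zone tower that locks down an encounter: on first aggro overlap it raises linked walls and spawns enemies around its choke point at intervals.
; After spawning, a looping timer keeps capsule collision off until all enemies are gone, then makes the tower hittable.
; Hits remove fixed health; at zero it signals the walls and hides its fire.
; The damage-type switch leading to the timeline-driven player grapple is disconnected.
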(event OnComponentBeginOverlap(AgroCollision)
  (params (OverlappedComponent :type Primitive%20Component%20Object%20Reference) (OtherActor :type Actor%20Object%20Reference) (OtherComp :type Primitive%20Component%20Object%20Reference) (OtherBodyIndex :type Integer) (bFromSweep :type Boolean) (SweepResult :type Hit%20Result%20Structure%20%28by%20ref%29))
  ;[1 1 1] Agro
  (Utilities|FlowControl|DoOnce false
    (:Completed
      (Development|PrintString "Hello")
      (for _array_element (Variables|Default|GetWall%20Objects)
        (Default|RaiseWallEvent _array_element))
      (bind _counter (Utilities|FlowControl|DoN (Variables|Default|GetNumber%20of%20Enemies%20Spawned) :!label _label)
        (:Exit
          (CallFunction|SpawnEnemies)
          (if (>= _counter (Variables|Default|GetNumber%20of%20Enemies%20Spawned))
            (CallFunction|CheckAliveEnemies)
            (Utilities|Time|SetTimerbyFunctionName 0 "CheckAliveEnemies" 0.1 true)
            (else
              (Utilities|FlowControl|Delay (Variables|Default|GetSpawnInterval))
              (goto _label))))))))

(event Custom|Activate%20Walls%20Event
  ;[1 1 1] Send Switch
  (Variables|Default|SetIsDestroyed? true)
  (for _array_element (Variables|Default|GetWall%20Objects)
    (Default|SwitchInterface _array_element true))
  (Rendering|SetVisibility (Variables|Default|GetFire) false false))

(event Custom|Grapple%20Event
  (bind _playerref (Variables|Default|GetPlayerRef))
  ;[1 1 1] Grapple
  (Variables|Default|SetPlayersLastLoc (Transformation|GetWorldLocation (Variables|/Script/Engine.Character|GetCapsuleComponent _playerref)))
  (Variables|/Script/Engine.CharacterMovementComponent|SetGravityScale (Variables|/Script/Engine.Character|GetCharacterMovement _playerref) 0.0)
  (bind _newtrack_0 (Timeline|GraplleTimeline PlayFromStart)
    (:Update
      (Transformation|SetWorldLocation (Variables|/Script/Engine.Character|GetCapsuleComponent (Variables|Default|GetPlayerRef)) (Math|Vector|Lerp(Vector) (Variables|Default|GetPlayersLastLoc) (+ (* (+ (Transformation|GetWorldLocation (Variables|Default|GetChokePoint)) "0, 0,150.000000") (/ 3.0 4.0)) (* (Variables|Default|GetPlayersLastLoc) (/ 1.0 4.0))) _newtrack_0) false false))
    (:Finished
      (Default|WeaponReset (Variables|/Game/Reign_Assets/Player_Character/Blueprints/MC_Prototype_BP.MC_Prototype_BP_C|GetEquippedWeapon (Variables|Default|GetPlayerRef)))
      (Variables|/Script/Engine.CharacterMovementComponent|SetGravityScale (Variables|/Script/Engine.Character|GetCharacterMovement (Variables|Default|GetPlayerRef)) 2.0))))

(event Custom|HealthCheck
  ;[1 1 1] HealthCheck
  (CallFunction|ShowHealthbar)
  (Variables|Default|SetCurrentHealth (- (Variables|Default|GetCurrentHealth) 10))
  (CallFunction|UpdateHealth)
  (if (<= (Variables|Default|GetCurrentHealth) 0)
    (CallFunction|ActivateWallsEvent)))

(event EventBeginPlay
  (|CallParentFunction)
  (Variables|Default|SetIsDestroyed? false)
  (Collision|SetCollisionEnabled (Variables|Default|GetCapsuleComponent) "NoCollision"))

(event EventDealingDamage
  (params (Sent%20Damage :type Integer) (Sender :type Actor%20Object%20Reference) (DamageType :type Name :default "None"))
  ;[1 1 1] Damage Solver
  (CallFunction|HealthCheck))

(fn ConstructionScript
  (|CallParentFunction))

(fn SpawnEnemies
  (bind _capsulecomponent (Variables|Default|GetCapsuleComponent))
  (bind _returnvalue (Transformation|GetWorldLocation _capsulecomponent))
  (Variables|Default|SetSpawnStart (Math|Random|RandomPointinBoundingBox (Transformation|GetWorldLocation (Variables|Default|GetChokePoint)) (Math|Vector|MakeVector 5e+02 5e+02 0.0)))
  (Utilities|FlowControl|MultiGate true true -1
    (:Out%200
      (Audio|PlaySoundatLocation "/Game/Reign_Assets/Sounds/Teleport_Sound1.Teleport_Sound1" _returnvalue "0, 0, 0" 0.5 1.0 0.0 0 0 0))
    (:Out%201
      (Audio|PlaySoundatLocation "/Game/Reign_Assets/Sounds/Teleport_Sound2.Teleport_Sound2" _returnvalue "0, 0, 0" 0.5 1.0 0.0 0 0 0))
    (:Out%202
      (Audio|PlaySoundatLocation "/Game/Reign_Assets/Sounds/Teleport_Sound3.Teleport_Sound3" _returnvalue "0, 0, 0" 0.5 1.0 0.0 0 0 0)))
  (Effects|SpawnEmitteratLocation "/Game/Reign_Assets/World_Objects/Tunnel_Object/Tunnel_Spawn_FX.Tunnel_Spawn_FX" (Variables|Default|GetSpawnStart) "0, 0, 0" "2.000000,2.000000,2.000000")
  (bind _returnvalue_2 (Game|SpawnActorfromClass (Variables|Default|GetEnemy%20To%20Spawn) (Math|Transform|MakeTransform (Variables|Default|GetSpawnStart) "0, 0, 0" "2.000000,2.000000,2.000000") "Undefined" 0 0))
  (Utilities|Array|Add (Variables|Default|GetActiveEnemies) _returnvalue_2))

(fn CheckAliveEnemies
  (Variables|Default|SetAll%20Alive? false)
  (bind _array_element (Utilities|Array|ForEachLoopwithBreak (Variables|Default|GetActiveEnemies))
    (:LoopBody
      (Utilities|IsValid _array_element
        (:Is%20Valid
          (Variables|Default|SetAll%20Alive? true))))
    (:Completed
      (if (Variables|Default|GetAll%20Alive?)
        (Collision|SetCollisionEnabled (Variables|Default|GetCapsuleComponent) "NoCollision")
        (Variables|Default|SetCanTakeDmg? false)
        (else
          (Collision|SetCollisionEnabled (Variables|Default|GetCapsuleComponent) "QueryAndPhysics")
          (Class|KismetSystemLibrary|PauseTimer 0 "CheckAliveEnemies")
          (Variables|Default|SetCanTakeDmg? true))))))