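; Key_BP is a collectible key pickup that spins and bobs until something overlaps its sphere.
; Tick rotates the mesh and offsets it by HoverValue, whose vertical direction HoverTimer flips on a repeating timer.
; The first overlap, with no actor filter, hides the mesh, decal and particles via DoOnce, then after a short delay calls AddKey on the Inventory actor found at BeginPlay.
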(event OnComponentBeginOverlap(Sphere)
  (params (OverlappedComponent :type Primitive%20Component%20Object%20Reference) (OtherActor :type Actor%20Object%20Reference) (OtherComp :type Primitive%20Component%20Object%20Reference) (OtherBodyIndex :type Integer) (bFromSweep :type Boolean) (SweepResult :type Hit%20Result%20Structure%20%28by%20ref%29))
  (Utilities|FlowControl|DoOnce false
    (:Completed
      (Rendering|SetVisibility (Variables|Default|GetKeyMesh) false false)
      (Utilities|FlowControl|Delay 0.5)
      (Default|AddKey (Variables|Default|GetInventoryRef)))))

(event Custom|HoverTimer
  (Utilities|FlowControl|FlipFlop
    (:A
      (Variables|Default|SetHoverValue "0, 0,1.000000"))
    (:B
      (Variables|Default|SetHoverValue "0, 0,-1.000000")))
  (Utilities|Time|SetTimerbyEvent (delegate Custom|HoverTimer) 2.0 true))

(event EventBeginPlay
  (bind _asmc_prototype_bp (Utilities|Casting|CastToMC_Prototype_BP (Game|GetPlayerCharacter 0)))
  (Variables|Default|SetPlayer%20Ref _asmc_prototype_bp)
  (bind _outactors (Actor|GetAllActorsOfClass "/Game/Wrath_Content/ChrisBossStuff/KeyAndLockSystem/Inventory.Inventory_C"))
  (Variables|Default|SetInventoryRef (Utilities|Array|Get(acopy) _outactors))
  (CallFunction|HoverTimer))

(event EventTick
  (params (DeltaSeconds :type Float%20%28single-precision%29))
  (Transformation|AddLocalRotation (Variables|Default|GetKeyMesh) "0,1.000000, 0" false false)
  (Transformation|AddWorldOffset (Variables|Default|GetKeyMesh) (Variables|Default|GetHoverValue) false false))

(fn ConstructionScript)