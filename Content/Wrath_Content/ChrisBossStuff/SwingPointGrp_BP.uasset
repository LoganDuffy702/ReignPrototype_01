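; SwingPointGrp_BP is a boss-content Blueprint that acts as a switch, relocating another actor when its DealingDamage event fires.
; The event calls MoveObject, which sets the ToMove actor to TargetLocation in one step without sweep and prints a "Switch activated" message.
; The default BeginPlay, overlap and Tick events are disabled, so DealingDamage is the only active trigger in the event graph.
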(event EventBeginPlay
  (|CallParentFunction) ; This node is disabled and will not be called.\nDrag off pins to build functionality.
)

(event Collision|EventActorBeginOverlap
  (params (OtherActor :type Actor%20Object%20Reference)))

(event EventTick
  (params (DeltaSeconds :type Float%20%28single-precision%29))
  (|CallParentFunction DeltaSeconds) ; This node is disabled and will not be called.\nDrag off pins to build functionality.
)

(event EventDealingDamage
  (params (Sent%20Damage :type Integer) (Sender :type Actor%20Object%20Reference) (DamageType :type Name :default "None"))
  (CallFunction|MoveObject))

(fn ConstructionScript
  (|CallParentFunction))

(fn MoveObject
  (Transformation|SetActorLocation (Variables|Default|GetToMove) (Variables|Default|GetTargetLocation) false false)
  (Development|PrintString "Switch activated"))