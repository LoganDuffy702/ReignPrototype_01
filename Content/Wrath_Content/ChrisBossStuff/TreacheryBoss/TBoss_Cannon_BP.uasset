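; Cannon actor for the Treachery boss that reacts to the type of damage it receives.
; Melee, Special and AIR hits rotate it by a fixed step, while a "Pull to" hit spawns a cannonball from its capsule's transform.
; A Grapple hit runs a timeline that lerps the player three quarters of the way toward a point above the cannon, updating the weapon's chain beam endpoint to the ChokePoint.
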(event Custom|PullPlayerEvent
  (bind _capsulecomponent (Variables|Default|GetCapsuleComponent))
  (bind _returnvalue (Transformation|GetWorldLocation _capsulecomponent))
  (Development|PrintString "Grapple")
  (Variables|Default|SetPlayerLastLoc (Transformation|GetActorLocation (Variables|Default|GetPlayerRef)))
  (bind _newtrack_0 (Timeline|Timeline_0 PlayFromStart)
    (:Update
      (Class|ParticleSystemComponent|SetBeamEndPoint (Variables|/Game/Reign_Assets/Weapon_BP/Master_Weapon_BP.Master_Weapon_BP_C|GetChainParticle (Variables|/Game/Reign_Assets/Player_Character/Blueprints/MC_Prototype_BP.MC_Prototype_BP_C|GetEquippedWeapon (Variables|Default|GetPlayerRef))) 0 (Transformation|GetWorldLocation (Variables|Default|GetChokePoint)))
      (Transformation|SetActorLocation (Variables|Default|GetPlayerRef) (Math|Vector|Lerp(Vector) (Math|Vector|MakeVector (.X (Math|Vector|BreakVector (Variables|Default|GetPlayerLastLoc))) (.Y (Math|Vector|BreakVector (Variables|Default|GetPlayerLastLoc))) (.Z (Math|Vector|BreakVector (Variables|Default|GetPlayerLastLoc)))) (+ (* (Math|Vector|MakeVector (.x _returnvalue) (.y _returnvalue) (+ (.z _returnvalue) 1.5e+02)) (/ 3.0 4.0)) (* (Math|Vector|MakeVector (.X (Math|Vector|BreakVector (Variables|Default|GetPlayerLastLoc))) (.Y (Math|Vector|BreakVector (Variables|Default|GetPlayerLastLoc))) (.Z (Math|Vector|BreakVector (Variables|Default|GetPlayerLastLoc)))) (/ 1.0 4.0))) _newtrack_0) false false))))

(event EventBeginPlay
  (|CallParentFunction) ; This node is disabled and will not be called.\nDrag off pins to build functionality.
)

(event Collision|EventActorBeginOverlap
  (params (OtherActor :type Actor%20Object%20Reference)))

(event EventTick
  (params (DeltaSeconds :type Float%20%28single-precision%29))
  (|CallParentFunction DeltaSeconds) ; This node is disabled and will not be called.\nDrag off pins to build functionality.
)

(event EventDealingDamage
  (params (Sent%20Damage :type Integer) (Sender :type Actor%20Object%20Reference) (DamageType :type Name :default "None"))
  (bind _capsulecomponent (Variables|Default|GetCapsuleComponent))
  (switch name DamageType
    (:Melee
      (Class|Actor|AddActorWorldRotation "0,45.000000, 0" :!label _label))
    (:Special
      (goto _label))
    (:AIR
      (goto _label))
    (:Grapple
      (CallFunction|PullPlayerEvent))
    (:PullTo
      (Development|PrintString "Fire")
      (Game|SpawnActorfromClass "/Game/Wrath_Content/ChrisBossStuff/TreacheryBoss/TBoss_CannonBall_BP.TBoss_CannonBall_BP_C" (Math|Transform|MakeTransform (Transformation|GetWorldLocation _capsulecomponent) (Transformation|GetWorldRotation _capsulecomponent) "1,1,1") "Undefined" 0 0))))

(fn ConstructionScript
  (|CallParentFunction))