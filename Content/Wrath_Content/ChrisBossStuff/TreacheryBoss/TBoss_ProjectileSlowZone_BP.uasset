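; Projectile slow zone actor for the Treachery boss that can be switched on and off.
; Activate and deactivate events toggle the Sphere's collision between query-and-physics and none, and show or hide the Visual component to match.
; On BeginPlay it deactivates itself unless StartActivated is set.
; The graph holds no slowing logic, only this toggle.
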(event Custom|EventActivate
  (Collision|SetCollisionEnabled (Variables|Default|GetSphere) "QueryAndPhysics")
  (Development|SetHiddeninGame (Variables|Default|GetVisual) false false))

(event Custom|EventDeactivate
  (Collision|SetCollisionEnabled (Variables|Default|GetSphere) "NoCollision")
  (Development|SetHiddeninGame (Variables|Default|GetVisual) true false))

(event EventBeginPlay
  (if (not (Variables|Default|GetStartActivated))
    (CallFunction|EventDeactivate)))

(event Collision|EventActorBeginOverlap
  (params (OtherActor :type Actor%20Object%20Reference)))

(event EventTick
  (params (DeltaSeconds :type Float%20%28single-precision%29)))

(fn ConstructionScript)