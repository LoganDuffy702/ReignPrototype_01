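; A Treachery boss shotgun ball projectile that slows inside projectile slow zones and explodes on overlapping anything else.
; Sphere overlap with a TBoss_ProjectileSlowZone_BP sets local forward velocity to SlowSpeed, and leaving restores the max speed cached at BeginPlay.
; Any other overlap spawns an explosion effect and destroys the actor, while blocking hits only spawn an impact effect.
; Velocity is debug-printed at spawn and on each speed change.
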(event OnComponentEndOverlap(Sphere)
  (params (OverlappedComponent :type Primitive%20Component%20Object%20Reference) (OtherActor :type Actor%20Object%20Reference) (OtherComp :type Primitive%20Component%20Object%20Reference) (OtherBodyIndex :type Integer))
  (Utilities|Casting|CastToTBoss_ProjectileSlowZone_BP OtherActor)
  (CallFunction|EventSpeedUp))

(event OnComponentBeginOverlap(Sphere)
  (params (OverlappedComponent :type Primitive%20Component%20Object%20Reference) (OtherActor :type Actor%20Object%20Reference) (OtherComp :type Primitive%20Component%20Object%20Reference) (OtherBodyIndex :type Integer) (bFromSweep :type Boolean) (SweepResult :type Hit%20Result%20Structure%20%28by%20ref%29))
  (Utilities|Casting|CastToTBoss_ProjectileSlowZone_BP OtherActor
    (:then
      (CallFunction|EventSlowDown))
    (:CastFailed
      (Effects|SpawnEmitteratLocation "/Game/StarterContent/Particles/P_Explosion.P_Explosion" (Transformation|GetWorldLocation (Variables|Default|GetSphere)) "0, 0, 0" "10.000000,10.000000,10.000000")
      (Actor|DestroyActor))))

(event OnComponentHit(Sphere)
  (params (HitComponent :type Primitive%20Component%20Object%20Reference) (OtherActor :type Actor%20Object%20Reference) (OtherComp :type Primitive%20Component%20Object%20Reference) (NormalImpulse :type Vector :default "0, 0, 0") (Hit :type Hit%20Result%20Structure%20%28by%20ref%29))
  (Effects|SpawnEmitteratLocation "/Game/Reign_Assets/EnemyObjects/Jump_Enemy/Jump_FX/JumpStart_Enemy_LeapFX1.JumpStart_Enemy_LeapFX1" (.impactpoint Hit) "0, 0, 0" "5.000000,5.000000,5.000000"))

(event Custom|EventSlowDown
  (Game|Components|ProjectileMovement|SetVelocityinLocalSpace (Variables|Default|GetProjectileMovement) (Math|Vector|MakeVector (Variables|Default|GetSlowSpeed) 0.0 0.0))
  (Development|PrintString (Utilities|String|ToString(Vector) (Variables|/Script/Engine.MovementComponent|GetVelocity (Variables|Default|GetProjectileMovement)))))

(event Custom|EventSpeedUp
  (Game|Components|ProjectileMovement|SetVelocityinLocalSpace (Variables|Default|GetProjectileMovement) (Math|Vector|MakeVector (Variables|Default|GetOG_MaxSpeed) 0.0 0.0))
  (Development|PrintString (Utilities|String|ToString(Vector) (Variables|/Script/Engine.MovementComponent|GetVelocity (Variables|Default|GetProjectileMovement)))))

(event EventBeginPlay
  (Variables|Default|SetOG_MaxSpeed (Class|MovementComponent|GetMaxSpeed (Variables|Default|GetProjectileMovement)))
  (Development|PrintString (Utilities|String|ToString(Vector) (Variables|/Script/Engine.MovementComponent|GetVelocity (Variables|Default|GetProjectileMovement)))))

(event Collision|EventActorBeginOverlap
  (params (OtherActor :type Actor%20Object%20Reference)))

(event EventTick
  (params (DeltaSeconds :type Float%20%28single-precision%29)))

(fn ConstructionScript)