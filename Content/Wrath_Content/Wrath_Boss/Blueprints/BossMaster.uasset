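; BossMaster is the Wrath boss actor, holding its health, player-facing rotation, melee hit detection and a toggleable head damage point.
; BeginPlay caches the player, FireBreath and PhaseHandler, hides the mesh, disables the head collider and unhides the grapples after a delay.
; A flag-gated Tick yaws the mesh toward the player.
; Arm and bicep overlaps share one damage path, gated by an attack flag and a short re-hit cooldown.
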(event OnComponentBeginOverlap(RightArm)
  (params (OverlappedComponent :type Primitive%20Component%20Object%20Reference) (OtherActor :type Actor%20Object%20Reference) (OtherComp :type Primitive%20Component%20Object%20Reference) (OtherBodyIndex :type Integer) (bFromSweep :type Boolean) (SweepResult :type Hit%20Result%20Structure%20%28by%20ref%29))
  (if (Math|Boolean|ANDBoolean (Math|Boolean|ORBoolean (== OtherActor (Variables|Default|GetPlayer)) (== (stale OnComponentBeginOverlap(LeftArm) OtherActor) (Variables|Default|GetPlayer)) (== (stale OnComponentBeginOverlap(LeftBicep) OtherActor) (Variables|Default|GetPlayer)) (== (stale OnComponentBeginOverlap(RightBicep) OtherActor) (Variables|Default|GetPlayer))) (not (Variables|Default|GetHitPlayerWithMelee)) (Variables|Default|GetCanHitPlayerWithMelee))
    (CallFunction|DelayUntilPlayerCanGetHitbyMelee)
    (Class|HealthDamageInterface|DealingDamage(Message) (Variables|Default|GetPlayer) 30 0 "None")))

(event OnComponentBeginOverlap(LeftArm)
  (params (OverlappedComponent :type Primitive%20Component%20Object%20Reference) (OtherActor :type Actor%20Object%20Reference) (OtherComp :type Primitive%20Component%20Object%20Reference) (OtherBodyIndex :type Integer) (bFromSweep :type Boolean) (SweepResult :type Hit%20Result%20Structure%20%28by%20ref%29))
  (if (Math|Boolean|ANDBoolean (Math|Boolean|ORBoolean (== (stale OnComponentBeginOverlap(RightArm) OtherActor) (Variables|Default|GetPlayer)) (== OtherActor (Variables|Default|GetPlayer)) (== (stale OnComponentBeginOverlap(LeftBicep) OtherActor) (Variables|Default|GetPlayer)) (== (stale OnComponentBeginOverlap(RightBicep) OtherActor) (Variables|Default|GetPlayer))) (not (Variables|Default|GetHitPlayerWithMelee)) (Variables|Default|GetCanHitPlayerWithMelee))
    (CallFunction|DelayUntilPlayerCanGetHitbyMelee)
    (Class|HealthDamageInterface|DealingDamage(Message) (Variables|Default|GetPlayer) 30 0 "None")))

(event OnComponentBeginOverlap(LeftBicep)
  (params (OverlappedComponent :type Primitive%20Component%20Object%20Reference) (OtherActor :type Actor%20Object%20Reference) (OtherComp :type Primitive%20Component%20Object%20Reference) (OtherBodyIndex :type Integer) (bFromSweep :type Boolean) (SweepResult :type Hit%20Result%20Structure%20%28by%20ref%29))
  (if (Math|Boolean|ANDBoolean (Math|Boolean|ORBoolean (== (stale OnComponentBeginOverlap(RightArm) OtherActor) (Variables|Default|GetPlayer)) (== (stale OnComponentBeginOverlap(LeftArm) OtherActor) (Variables|Default|GetPlayer)) (== OtherActor (Variables|Default|GetPlayer)) (== (stale OnComponentBeginOverlap(RightBicep) OtherActor) (Variables|Default|GetPlayer))) (not (Variables|Default|GetHitPlayerWithMelee)) (Variables|Default|GetCanHitPlayerWithMelee))
    (CallFunction|DelayUntilPlayerCanGetHitbyMelee)
    (Class|HealthDamageInterface|DealingDamage(Message) (Variables|Default|GetPlayer) 30 0 "None")))

(event OnComponentBeginOverlap(RightBicep)
  (params (OverlappedComponent :type Primitive%20Component%20Object%20Reference) (OtherActor :type Actor%20Object%20Reference) (OtherComp :type Primitive%20Component%20Object%20Reference) (OtherBodyIndex :type Integer) (bFromSweep :type Boolean) (SweepResult :type Hit%20Result%20Structure%20%28by%20ref%29))
  (if (Math|Boolean|ANDBoolean (Math|Boolean|ORBoolean (== (stale OnComponentBeginOverlap(RightArm) OtherActor) (Variables|Default|GetPlayer)) (== (stale OnComponentBeginOverlap(LeftArm) OtherActor) (Variables|Default|GetPlayer)) (== (stale OnComponentBeginOverlap(LeftBicep) OtherActor) (Variables|Default|GetPlayer)) (== OtherActor (Variables|Default|GetPlayer))) (not (Variables|Default|GetHitPlayerWithMelee)) (Variables|Default|GetCanHitPlayerWithMelee))
    (CallFunction|DelayUntilPlayerCanGetHitbyMelee)
    (Class|HealthDamageInterface|DealingDamage(Message) (Variables|Default|GetPlayer) 30 0 "None")))

(event Custom|DelayUntilPlayerCanGetHitByMelee
  (Variables|Default|SetHitPlayerWithMelee true)
  (Utilities|FlowControl|Delay 1.0)
  (Variables|Default|SetHitPlayerWithMelee false))

(event Custom|TempLookAt
  (Transformation|SetWorldRotation (Variables|Default|GetSkeletalMesh1) (Math|Rotator|MakeRotator 0.0 0.0 (- (.yaw (Math|Rotator|FindLookatRotation (Transformation|GetWorldLocation (Variables|Default|GetSkeletalMesh1)) (Transformation|GetActorLocation (Variables|Default|GetTempPlayerRef)))) 9e+01)) false false))

(event Custom|EventDisableHeadCollider
  (bind _asboss_head_damage_pt (Utilities|Casting|CastToBossHeadDamagePt (Variables|/Script/Engine.ChildActorComponent|GetChildActor (Variables|Default|GetBossHeadDamagePt))))
  (Default|EventDisable _asboss_head_damage_pt))

(event Custom|EventEnableHeadCollider
  (bind _asboss_head_damage_pt (Utilities|Casting|CastToBossHeadDamagePt (Variables|/Script/Engine.ChildActorComponent|GetChildActor (Variables|Default|GetBossHeadDamagePt))))
  (Default|EventEnable _asboss_head_damage_pt))

(event EventBeginPlay
  (Variables|Default|SetPlayer (Game|GetPlayerCharacter 0))
  (bind _outactors (Actor|GetAllActorsOfClass "/Game/Wrath_Content/ChrisBossStuff/FlameBreathStuff/FireBreath.FireBreath_C"))
  (Variables|Default|SetFireBreathRef (Utilities|Array|Get(acopy) _outactors))
  (Variables|Default|SetHealth (Variables|Default|GetMaxHealth))
  (Rendering|SetVisibility (Variables|Default|GetSkeletalMesh1) false false)
  (bind _asmc_prototype_bp (Utilities|Casting|CastToMC_Prototype_BP (Game|GetPlayerCharacter 0)))
  (Variables|Default|SetTempPlayerRef _asmc_prototype_bp)
  (bind _outactors_2 (Actor|GetAllActorsOfClass "/Game/Wrath_Content/Wrath_Boss/Blueprints/PhaseHandler.PhaseHandler_C"))
  (Variables|Default|SetPhaseHandlerRef (Utilities|Array|Get(acopy) _outactors_2))
  (CallFunction|EventDisableHeadCollider)
  (Utilities|FlowControl|Delay 2.0)
  (for _array_element (Variables|Default|GetGrapples)
    (Rendering|SetActorHiddenInGame _array_element false)))

(event Collision|EventActorBeginOverlap
  (params (OtherActor :type Actor%20Object%20Reference)))

(event EventTick
  (params (DeltaSeconds :type Float%20%28single-precision%29))
  (if (Variables|Default|GetTempLookAt?)
    (CallFunction|TempLookat)))

(fn ConstructionScript)

(fn GetDistancetoPlayer
  (return (Math|Float|Absolute(Float) (Math|Vector|VectorLength (- (Transformation|GetActorLocation) (Transformation|GetActorLocation (Variables|Default|GetPlayer)))))))