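; Boss-fight handler that spawns enemies in timed waves through the level's BossEnemySpawner actors, cached on BeginPlay with the player.
; SpawnEnemies starts a looping timer that spawns one enemy per tick via FindSmallestSpawner, meant to pick the spawner nearest the player, though its distance checks show no target.
; The timer ends and sets IsFinished when the never-reset spawn count equals the requested number or StopSpawningEvent flags a phase 2 halt.
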(event Custom|SpawnEnemies
  (params (NumOfEnemies :type Integer) (Spawn%20Rate :type Float%20%28single-precision%29))
  (Variables|Default|SetNumOfEnemies NumOfEnemies)
  (Variables|Default|SetIsFinished false)
  (bind _returnvalue (Utilities|Time|SetTimerbyEvent (delegate Custom|StartToSpawnEnemy) Spawn%20Rate true))
  (Variables|Default|SetTimer%20Hamdler _returnvalue))

(event Custom|StartToSpawnEnemy
  ;[1 1 1] Spawns in an enemy
  (if (or (== (Variables|Default|GetNumOfEnemies) (Variables|Default|GetEnemiesSpawned)) (Variables|Default|GetStopSpawning))
    (Variables|Default|SetStopSpawning false)
    (Variables|Default|SetIsFinished true)
    (Utilities|Time|ClearandInvalidateTimerbyHandle (Variables|Default|GetTimer%20Hamdler))
    (else
      (bind _smallest_spawner (CallFunction|FindSmallestSpawner))
      (Math|Integer|IncrementInt (Variables|Default|GetEnemiesSpawned)
        (:%20%20
          (Default|SpawnEnemy _smallest_spawner))))))

(event Custom|StopSpawningEvent
  ;[1 1 1] For Behavior tree when player enters phase 2
  (Variables|Default|SetStopSpawning true))

(event EventBeginPlay
  (bind _outactors (Actor|GetAllActorsOfClass "/Game/Wrath_Content/Wrath_Boss/Blueprints/BossEnemySpawner.BossEnemySpawner_C"))
  (Variables|Default|SetSpawners _outactors)
  (bind _outactors_2 (Actor|GetAllActorsOfClass "/Game/Reign_Assets/Player_Character/Blueprints/MC_Prototype_BP.MC_Prototype_BP_C"))
  (bind _asmc_prototype_bp (Utilities|Casting|CastToMC_Prototype_BP (Utilities|Array|Get(acopy) _outactors_2)))
  (Variables|Default|SetPlayer _asmc_prototype_bp))

(fn ConstructionScript)

(fn FindSmallestSpawner
  (bind _player (Variables|Default|GetPlayer))
  (bind _returnvalue (Transformation|GetDistanceTo _player 0))
  (Variables|Default|SetSmallestSpawner (Utilities|Array|Get(acopy) (Variables|Default|GetSpawners)))
  (Variables|Default|SetSmallestDistance (Transformation|GetDistanceTo (Variables|Default|GetPlayer) 0))
  (for _array_element (Variables|Default|GetSpawners)
    (if (> (Variables|Default|GetSmallestDistance) _returnvalue)
      (Variables|Default|SetSmallestSpawner _array_element)
      (Variables|Default|SetSmallestDistance _returnvalue)))
  (Development|PrintString (Utilities|GetDisplayName (Variables|Default|GetSmallestSpawner)))
  (return (Variables|Default|GetSmallestSpawner)))