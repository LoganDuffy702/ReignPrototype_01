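; Wrath boss fireball projectile that launches at a set angle and velocity, then steers toward the player and spreads into fire.
; Each tick, while the height gap to the player meets both homing thresholds, it zeroes gravity and resets local-space velocity from the player offset.
; CircleCollider overlap runs a timeline that widens and flattens FireCollision, then destroys the actor after a delay.
; FireCollision damages only the player's capsule component.
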(event OnComponentBeginOverlap(CircleCollider)
  (params (OverlappedComponent :type Primitive%20Component%20Object%20Reference) (OtherActor :type Actor%20Object%20Reference) (OtherComp :type Primitive%20Component%20Object%20Reference) (OtherBodyIndex :type Integer) (bFromSweep :type Boolean) (SweepResult :type Hit%20Result%20Structure%20%28by%20ref%29))
  (CallFunction|SpreadFire))

(event OnComponentBeginOverlap(FireCollision)
  (params (OverlappedComponent :type Primitive%20Component%20Object%20Reference) (OtherActor :type Actor%20Object%20Reference) (OtherComp :type Primitive%20Component%20Object%20Reference) (OtherBodyIndex :type Integer) (bFromSweep :type Boolean) (SweepResult :type Hit%20Result%20Structure%20%28by%20ref%29))
  ;[1 1 1] If Collider Hits Player Do Damage
  (bind _asmc_prototype_bp (Utilities|Casting|CastToMC_Prototype_BP (Game|GetPlayerCharacter 0)))
  (if (== OtherComp (Actor|GetComponentbyClass _asmc_prototype_bp "/Script/Engine.CapsuleComponent"))
    (Default|DealingDamage _asmc_prototype_bp 10 0 "None")))

(event Custom|Spread%20Fire
  ;[1 1 1] SpreadsFire
  (Variables|Default|SetOriginalFireVectorScale (.scale (Transformation|GetRelativeTransform (Variables|Default|GetFireCollision))))
  (bind _newtrack_0 (Timeline|FireSpreadTimeline Play)
    (:Update
      (Transformation|SetRelativeScale3D (Variables|Default|GetFireCollision) (Math|Vector|MakeVector (.X (Math|Vector|BreakVector (Math|Vector|Lerp(Vector) (Variables|Default|GetOriginalFireVectorScale) (Variables|Default|GetFinalFireVectorScale) _newtrack_0))) (.Y (Math|Vector|BreakVector (Math|Vector|Lerp(Vector) (Variables|Default|GetOriginalFireVectorScale) (Variables|Default|GetFinalFireVectorScale) _newtrack_0))) 0.1)))
    (:Finished
      (Utilities|FlowControl|Delay 2.0)
      (Actor|DestroyActor))))

(event Custom|CheckWhenToStartHoming
  ;[1 1 1] Check When To Start Homing Called in Event TICK
  (if (>= (Math|Float|Absolute(Float) (- (.z (.location (Transformation|GetActorTransform (Variables|Default|GetPlayer)))) (.z (.Location (Math|Transform|BreakTransform (Transformation|GetActorTransform)))))) (Variables|Default|GetDistanceToStartHoming))
    (CallFunction|ChecktoStopHoming)))

(event Custom|CheckToStopHoming
  ;[1 1 1] Check when to stop homing called in event CheckWhenToStartHoming
  (if (not (< (Math|Float|Absolute(Float) (- (.z (.location (Transformation|GetActorTransform (Variables|Default|GetPlayer)))) (.z (.Location (Math|Transform|BreakTransform (Transformation|GetActorTransform)))))) (Variables|Default|GetDistanceTilStopHoming)))
    (CallFunction|HometoPlayer)))

(event Custom|HomeToPlayer
  ;[1 1 1] Start Homing to the player called in event: "Check When to stop homing"
  (Variables|/Script/Engine.ProjectileMovementComponent|SetProjectileGravityScale (Variables|Default|GetProjectileMovement) 0.0)
  (bind _outactors (Actor|GetAllActorsOfClass "/Game/Reign_Assets/Player_Character/Blueprints/MC_Prototype_BP.MC_Prototype_BP_C"))
  (Game|Components|ProjectileMovement|SetVelocityinLocalSpace (Variables|Default|GetProjectileMovement) (* (- (.location (Transformation|GetActorTransform (Utilities|Array|Get(acopy) _outactors))) (.Location (Math|Transform|BreakTransform (Transformation|GetActorTransform)))) 1.5)))

(event EventBeginPlay
  ;[1 1 1] Initialize Rotation and Launch Speed
  (Transformation|SetActorRelativeRotation (Variables|Default|GetFireballAngle))
  (Game|Components|ProjectileMovement|SetVelocityinLocalSpace (Variables|Default|GetProjectileMovement) (Variables|Default|GetVelocity))
  (bind _outactors (Actor|GetAllActorsOfClass "/Game/Reign_Assets/Player_Character/Blueprints/MC_Prototype_BP.MC_Prototype_BP_C"))
  (Variables|Default|SetPlayer (Utilities|Array|Get(acopy) _outactors)))

(event EventTick
  (params (DeltaSeconds :type Float%20%28single-precision%29))
  (CallFunction|CheckwhentoStartHoming))

(fn ConstructionScript)