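; Boss-fight handler actor that fires timed waves of fireballs from the FireballSpawner actors in the level.
; SpawnFireballs starts a looping timer that triggers the spawner nearest the player until the requested count is reached, then flags IsFinished.
; StopSpawningEvent, meant for the phase 2 behavior tree, makes the next tick destroy live fireballs and end the wave.
; A random-spawner variant exists but is never wired to the timer.
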(event Custom|SpawnClosestToPlayer
  (bind _fireballs_spawned (Variables|Default|GetFireballs%20Spawned))
  ;[1 1 1] Spawn Fireball in the Spawner that is Closest to the player
  (Development|PrintString (Utilities|String|ToString(Integer) _fireballs_spawned))
  (if (== (Variables|Default|GetNumOfFireballs) _fireballs_spawned)
    (Variables|Default|SetStopSpawning false :!label _label)
    (Variables|Default|SetIsFinished true)
    (Utilities|Time|ClearandInvalidateTimerbyHandle (Variables|Default|GetTimer%20Hamdler))
    (elif (Variables|Default|GetStopSpawning)
      (bind _outactors (Actor|GetAllActorsOfClass "/Game/Wrath_Content/Wrath_Boss/Blueprints/Fireball.Fireball_C"))
      (for _array_element _outactors
        (Actor|DestroyActor _array_element)
        (goto _label))
      (goto _label)
      (else
        (bind _smallest_spawner (CallFunction|FindSmallestSpawner))
        (Default|SpawnFireball _smallest_spawner)
        (Math|Integer|IncrementInt (Variables|Default|GetFireballs%20Spawned))))))

(event Custom|SpawnRandomly
  ;[1 1 1] Spawns Fireballs Randomly
  (if (== (Variables|Default|GetNumOfFireballs) (Variables|Default|GetFireballs%20Spawned))
    (Variables|Default|SetIsFinished true)
    (Utilities|Time|ClearandInvalidateTimerbyHandle (Variables|Default|GetTimer%20Hamdler))
    (else
      (bind _result (Math|Integer|DecrementInt (Utilities|Array|Length (Variables|Default|GetSpawners)))
        (:%20%20
          (Development|PrintString (Utilities|String|ToString(Integer) (Math|Random|RandomIntegerinRange 0 _result)))
          (Default|SpawnFireball (Utilities|Array|Get(acopy) (Variables|Default|GetSpawners) (Math|Random|RandomIntegerinRange 0 _result)))
          (Math|Integer|IncrementInt (Variables|Default|GetFireballs%20Spawned)))))))

(event Custom|SpawnFireballs
  (params (SpawnRate :type Float%20%28single-precision%29) (NumOfFireballs :type Integer) (RandomSpawn :type Boolean))
  (Variables|Default|SetFireballs%20Spawned 0)
  (Variables|Default|SetNumOfFireballs NumOfFireballs)
  (Variables|Default|SetIsFinished false)
  (bind _returnvalue (Utilities|Time|SetTimerbyEvent (delegate Custom|SpawnClosestToPlayer) SpawnRate true))
  (Variables|Default|SetTimer%20Hamdler _returnvalue))

(event Custom|StopSpawningEvent
  ;[1 1 1] For Behavior tree when player enters phase 2
  (Variables|Default|SetStopSpawning true)
  (Variables|Default|SetFireballs%20Spawned 0))

(event EventBeginPlay
  (bind _outactors (Actor|GetAllActorsOfClass "/Game/Wrath_Content/Wrath_Boss/Blueprints/FireballSpawner.FireballSpawner_C"))
  (Variables|Default|SetSpawners _outactors)
  (bind _outactors_2 (Actor|GetAllActorsOfClass "/Game/Reign_Assets/Player_Character/Blueprints/MC_Prototype_BP.MC_Prototype_BP_C"))
  (bind _asmc_prototype_bp (Utilities|Casting|CastToMC_Prototype_BP (Utilities|Array|Get(acopy) _outactors_2)))
  (Variables|Default|SetPlayer _asmc_prototype_bp))

(fn ConstructionScript)

(fn FindSmallestSpawner
  (bind _spawners (Variables|Default|GetSpawners))
  (bind _output (Utilities|Array|Get(acopy) _spawners))
  (Variables|Default|SetSmallestSpawner _output)
  (Variables|Default|SetSmallestDistance (Transformation|GetDistanceTo (Variables|Default|GetPlayer) _output))
  (for _array_element (Variables|Default|GetSpawners)
    (if (> (Variables|Default|GetSmallestDistance) (Transformation|GetDistanceTo (Variables|Default|GetPlayer) _array_element))
      (Variables|Default|SetSmallestSpawner _array_element)
      (Variables|Default|SetSmallestDistance (Transformation|GetDistanceTo (Variables|Default|GetPlayer) _array_element))))
  (return (Variables|Default|GetSmallestSpawner)))