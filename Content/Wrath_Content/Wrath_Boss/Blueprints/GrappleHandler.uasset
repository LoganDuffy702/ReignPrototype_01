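; GrappleHandler toggles the visibility of grapple switch actors in pairs, as part of the Wrath boss content.
; On BeginPlay it copies the actor list from its Grapples reference.
; DisableSwitches hides the two actors at the current Index, and EnableSwitches shows them again, then advances Index by two, wrapping to zero at the list's end.
; Only hidden-in-game state changes; collision and tick are untouched.
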(event Custom|EnableSwitches
  (bind _grapplelist (Variables|Default|GetGrappleList))
  (Rendering|SetActorHiddenInGame (Utilities|Array|Get(acopy) _grapplelist (Variables|Default|GetIndex)) false)
  (Rendering|SetActorHiddenInGame (Utilities|Array|Get(acopy) _grapplelist (+ (Variables|Default|GetIndex) 1)) false)
  (if (>= (+ (Variables|Default|GetIndex) 2) (Utilities|Array|Length (Variables|Default|GetGrappleList)))
    (Variables|Default|SetIndex 0)
    (else
      (Variables|Default|SetIndex (+ (Variables|Default|GetIndex) 2)))))

(event Custom|DisableSwitches
  (bind _grapplelist (Variables|Default|GetGrappleList))
  (bind _index (Variables|Default|GetIndex))
  (Rendering|SetActorHiddenInGame (Utilities|Array|Get(acopy) _grapplelist _index) true)
  (Rendering|SetActorHiddenInGame (Utilities|Array|Get(acopy) _grapplelist (+ _index 1)) true))

(event EventBeginPlay
  (Variables|Default|SetGrappleList (Utilities|Struct|BreakArrayOfActor (Variables|Default|GetGrapples))))

(fn ConstructionScript)