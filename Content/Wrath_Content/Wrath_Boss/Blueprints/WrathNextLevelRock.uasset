(event Custom|RiseFromGround
  (params (HowFarUp :type Float%20%28single-precision%29))
  (bind _defaultsceneroot (Variables|Default|GetDefaultSceneRoot))
  (bind _returnvalue (Transformation|GetWorldLocation _defaultsceneroot))
  (bind _moveuptrack (Timeline|Timeline_0 PlayFromStart)
    (:Update
      (Transformation|SetWorldLocation _defaultsceneroot (Math|Vector|MakeVector (.x _returnvalue) (.y _returnvalue) (+ (Variables|Default|GetOriginalZLocation) (* HowFarUp _moveuptrack))) false false))
    (:Finished
      (Variables|Default|SetOriginalZLocation (.z (Transformation|GetWorldLocation (Variables|Default|GetDefaultSceneRoot))))
      (Utilities|FlowControl|MultiGate false false -1
        (:Out%201
          (Utilities|FlowControl|Delay 1.0)
          (bind _returnvalue_2 (UserInterface|CreateWidget "/Game/Reign_Assets/Reign_UI/Thankyou_Widget.Thankyou_Widget_C"))
          (UserInterface|Viewport|AddtoViewport _returnvalue_2 0))))))

(event EventBeginPlay
  (Variables|Default|SetOriginalZLocation (.z (Transformation|GetWorldLocation (Variables|Default|GetDefaultSceneRoot))))
  (bind _outactors (Actor|GetAllActorsOfClass "/Game/Wrath_Content/Wrath_Boss/Blueprints/BossMaster.BossMaster_C"))
  (Variables|Default|SetBoss (Utilities|Array|Get(acopy) _outactors))
  (Actor|GetAllActorsOfClass "/Game/Camera/CameraManager.CameraManager_C")
  (Utilities|FlowControl|Delay 1.0)
  (Default|UnlockPortal (Variables|/Game/Wrath_Content/Wrath_Boss/Blueprints/BossMaster.BossMaster_C|GetActivatePortal_Component (Variables|Default|GetBoss))))

(event Collision|EventActorBeginOverlap
  (params (OtherActor :type Actor%20Object%20Reference)))

(event EventTick
  (params (DeltaSeconds :type Float%20%28single-precision%29)))

(fn ConstructionScript)